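; BP_TileBlockCreator is a construction-script actor that builds a rectangular block of floor tiles from width and height values.
; It fills a tile struct array with static mesh components on a 100-unit grid, then adds one box collision sized to the whole block.
; Each tile mesh is vertex-painted red as a test fill for grass placement, whose random index pass is switched off.
; A neighbour line-trace pass for reassigning meshes is unfinished and never runs.
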(fn `UserConstructionScript`
  (locals (aTiles :type "Array of /Game/HenryWorkFolder/Blueprints/Strut_Occom_TileAssign Structure") (cRow :type Integer :default 1) (TypeSelf :type "Array of EObjectTypeQuery Enum") (lineCheck :type Integer) (iGrass :type "Array of /Game/HenryWorkFolder/Blueprints/BP_GrassBlade Object Reference") (indexGrass :type "/Game/HenryWorkFolder/Blueprints/BP_GrassBlade Object Reference"))
  (bind _igrass (`local.iGrass`))
  (bind _returnvalue (* (`self.tHeight`) 50.0))
  (bind _returnvalue_2 (* (`self.tWidth`) 50.0))
  ;[1 1 1] Prep array size
  (`KismetArrayLibrary.Array_Resize` (`local.aTiles`) (* (`self.tWidth`) (`self.tHeight`)))
  ;[1 1 1] Create mesh
  (for (_ _array_index) (`local.aTiles`)
    (if (> (+ _array_index 1) (* (`self.tHeight`) (`local.cRow`))) :!label _label
      (bind _result (`/Engine/EditorBlueprintResources/StandardMacros.IncrementInt` (`local.cRow`))
        (:`  `
          (bind _output_get (set `local.cRow` _result))
          (goto _label)))
      (else
        (bind _returnvalue_3 (`AddComponent|NODE_AddStaticMeshComponent-0` :`RelativeTransform` (`KismetMathLibrary.MakeTransform` (`KismetMathLibrary.MakeVector` (+ (* (mod _array_index (`self.tHeight`)) 100.0) 50.0) (- (* _output_get 100.0) 50.0)))))
        (bind _output_get_2 (set `self.structTileAssign` (make `/Game/HenryWorkFolder/Blueprints/Strut_Occom_TileAssign` false "NewEnumerator8" _returnvalue_3)))
        (`KismetArrayLibrary.Array_Set` (`local.aTiles`) _array_index _output_get_2))))
  ;[1 1 1] Create Collision
  (set `local.cRow` 1)
  (`AddComponent|NODE_AddBoxComponent-0` :`RelativeTransform` (`KismetMathLibrary.MakeTransform` (`KismetMathLibrary.MakeVector` (* _returnvalue 1.0) (* _returnvalue_2 1.0)) (struct) (`KismetMathLibrary.MakeVector` _returnvalue _returnvalue_2 1.0)))
  ;[1 1 1] Place Grass on red verte colors
  (for (_array_element _array_index_2) (`local.aTiles`)
    ;;[1 1 1] AutoFill for Testing
    (`MeshVertexPainterKismetLibrary.PaintVerticesSingleColor` (`.CorrelatedMesh_9_C90531DD475CA495E681549C75CD32CF` (break `/Game/HenryWorkFolder/Blueprints/Strut_Occom_TileAssign` _array_element)) (`KismetMathLibrary.LinearColor_Red`))
    (if (and false (> (`KismetMathLibrary.RandomIntegerInRange` 0 100) 80))
      (bind _returnvalue_4 (`KismetArrayLibrary.Array_Add` _igrass))
      (`KismetArrayLibrary.Array_Set` _igrass _returnvalue_4 (`local.indexGrass`)))))