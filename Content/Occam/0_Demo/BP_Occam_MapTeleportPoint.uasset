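; Map teleport trigger for the Occam demo that sends the world player character to another map and spawn point when it overlaps the box.
; The destination comes from a DT_Occam_Map_Data row picked by LocalMapDataName and MapDataIndex.
; On overlap it updates the area name through the player controller's SaveManager component, then calls ChangeMap.
; The construction script labels two text renders with source and destination names and orients them to world north.
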(event `self.Box.OnComponentBeginOverlap`
  (params (OverlappedComponent :type "PrimitiveComponent Object Reference") (OtherActor :type "Actor Object Reference") (OtherComp :type "PrimitiveComponent Object Reference") (OtherBodyIndex :type Integer) (bFromSweep :type Boolean) (SweepResult :type "HitResult Structure (by ref)"))
  (bind _mapdataindex (`self.MapDataIndex`))
  (cast `/Game/Occam/2_Blueprints/5_GameBaseActors/BP_Occam_Character_Player_World` OtherActor)
  (bind _returnvalue (`|GetDataTableRow` "/Game/Occam/2_Blueprints/1_Datatables/DT_Occam_Map_Data.DT_Occam_Map_Data" (`self.LocalMapDataName`))
    (:`then`
      (bind (_maphardcodedname _mapdisplayname _originspawnpoint _destinationmaphardcodedname _desinationmapdisplayname _destinationspawnpoint) (break `/Game/Occam/2_Blueprints/2_Structures/Strut_Occam_MapData` _returnvalue))
      (`/Game/Occam/2_Blueprints/0_Components/AC_Occam_SaveManager.ChangeAreaName` (`self.GetComponentByClass` (`GameplayStatics.GetPlayerController` 0) "/Game/Occam/2_Blueprints/0_Components/AC_Occam_SaveManager.AC_Occam_SaveManager_C") (`KismetTextLibrary.Conv_StringToText` (`|GetArrayItem` _desinationmapdisplayname _mapdataindex)))
      (`/Game/Occam/2_Blueprints/FL_Occam_CustomFunctionsLibrary.ChangeMap` (`KismetStringLibrary.Conv_StringToName` (`|GetArrayItem` _destinationmaphardcodedname _mapdataindex)) (`KismetStringLibrary.Conv_StringToName` (`|GetArrayItem` _destinationspawnpoint _mapdataindex))))))

(fn `UserConstructionScript`
  (bind _returnvalue (`|GetDataTableRow` "/Game/Occam/2_Blueprints/1_Datatables/DT_Occam_Map_Data.DT_Occam_Map_Data" (`self.LocalMapDataName`))
    (:`then`
      (bind (_maphardcodedname _mapdisplayname _originspawnpoint _destinationmaphardcodedname _desinationmapdisplayname) (break `/Game/Occam/2_Blueprints/2_Structures/Strut_Occam_MapData` _returnvalue))
      (`TextRenderComponent.K2_SetText` (`self.TextRender`) (`|FormatText` "{0} - {1}" _mapdisplayname (`self.MapDataIndex`)))
      (`TextRenderComponent.K2_SetText` (`self.TextRender1`) (`KismetTextLibrary.Conv_StringToText` (`|GetArrayItem` _desinationmapdisplayname (`self.MapDataIndex`))))
      (`/Game/Occam/2_Blueprints/FL_Occam_CustomFunctionsLibrary.SetToWorldNorth` (`self.TextRender`) (`self.Scene`))
      (`/Game/Occam/2_Blueprints/FL_Occam_CustomFunctionsLibrary.SetToWorldNorth` (`self.TextRender1`) (`self.Scene`)))))