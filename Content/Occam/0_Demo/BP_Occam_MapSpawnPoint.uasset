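; BP_Occam_MapSpawnPoint is a spawn point marker for Occam maps, serving as either a save point or an origin spawn point.
; Its construction script uses SaveSpawn to choose the save point or map data table, then labels TextRender with the entry at MapDataIndex in the LocalMapDataName row.
; When the row is found, it aligns both text renders relative to world north.
; GetSpawnTransfrom returns the Arrow's world transform.
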(fn `GetSpawnTransfrom`
  (returns (SpawnTransform :type "Transform Structure"))
  (return (`SceneComponent.K2_GetComponentToWorld` (`self.Arrow`))))

(fn `UserConstructionScript`
  (locals (Local_W :type "Float (double-precision)" :default 180.0))
  (bind _localmapdataname (`self.LocalMapDataName`))
  (if (`self.SaveSpawn?`)
    (bind _returnvalue (`|GetDataTableRow` "/Game/Occam/2_Blueprints/1_Datatables/DT_Occam_SavePointData.DT_Occam_SavePointData" _localmapdataname)
      (:`then`
        (`TextRenderComponent.K2_SetText` (`self.TextRender`) (`KismetTextLibrary.Conv_StringToText` (`|GetArrayItem` (`.SavePointHardcodedName_7_D632BBF9447B033CE88B6A8152829E6A` (break `/Game/Occam/2_Blueprints/2_Structures/Strut_Occam_SavePointData` _returnvalue)) (`self.MapDataIndex`))))))
    (else
      (bind _returnvalue_2 (`|GetDataTableRow` "/Game/Occam/2_Blueprints/1_Datatables/DT_Occam_Map_Data.DT_Occam_Map_Data" _localmapdataname)
        (:`then`
          (`TextRenderComponent.K2_SetText` (`self.TextRender`) (`KismetTextLibrary.Conv_StringToText` (`|GetArrayItem` (`.OriginSpawnPoint_15_A0CE083E42694BAF0022C6867E85D3DD` (break `/Game/Occam/2_Blueprints/2_Structures/Strut_Occam_MapData` _returnvalue_2)) (`self.MapDataIndex`))))))))
  (`/Game/Occam/2_Blueprints/FL_Occam_CustomFunctionsLibrary.SetToWorldNorth` (`self.TextRender`) (`self.Scene`))
  (`/Game/Occam/2_Blueprints/FL_Occam_CustomFunctionsLibrary.SetToWorldNorth` (`self.TextRender1`) (`self.Scene`)))