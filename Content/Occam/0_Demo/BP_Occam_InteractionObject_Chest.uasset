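; Interactable loot chest that grants the items in ItemsInChest to the player's inventory.
; Interaction requires an unlooted, non-empty chest and a passed skill check, then adds items via the inventory manager and fills the loot menu with one info bar per item.
; Looting plays the open animation, sets the interaction state and disables interaction.
; An empty chest on BeginPlay, or a loaded looted state, plays the AM_Occam_Chest_Close animation.
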(event `self.ReceiveBeginPlay`
  (`parent.ReceiveBeginPlay`)
  (if (not (> (`BlueprintSetLibrary.Set_Length` (`self.ItemsInChest`)) 0))
    (`SkeletalMeshComponent.PlayAnimation` (`self.SkeletalMesh`) "/Game/Occam/5_Props/Chest/AM_Occam_Chest_Close.AM_Occam_Chest_Close" false :!label _label)))

(event `self.OnObjectInteractionStateLoaded`
  (params (InteractionState :type Boolean))
  (if InteractionState
    (goto _label)))

(event `self.ReceiveTick`
  (params (DeltaSeconds :type "Float (single-precision)"))
  (`parent.ReceiveTick` DeltaSeconds))

(event `self.OnInteractionRequested`
  (params (PlayerWorldCharacter :type "/Game/Occam/2_Blueprints/5_GameBaseActors/BP_Occam_Character_Player_World Object Reference"))
  (bind _playercontroller (`/Game/Occam/2_Blueprints/5_GameBaseActors/BP_Occam_Character_Player_World.PlayerController` PlayerWorldCharacter))
  (bind _world_interface (`/Game/Occam/2_Blueprints/BP_Occam_PController_World.World Interface` _playercontroller))
  (`KismetSystemLibrary.PrintString` "Hello")
  (`/Engine/EditorBlueprintResources/StandardMacros.IsValid` PlayerWorldCharacter
    (:`Is Valid`
      (if (`self.GetObjectInteractionState`)
        _
        (elif (> (`BlueprintSetLibrary.Set_Length` (`self.ItemsInChest`)) 0)
          (bind _skillchecksuccessful_ (`self.Interaction Skill Check`))
          (if _skillchecksuccessful_
            ;[1 1 1] Adding and Displaying Items
            (`self.AddItemsFromChestToInventory` (`/Game/Occam/2_Blueprints/BP_Occam_PController_World.AC_Occam_InventoryManager` _playercontroller))
            (`self.ConstructInteractionPopUpText` _world_interface)
            (`/Game/Occam/6_UI/2_Main_Widgets/WBP_WorldInterface.WorldInterface_LootMenu` _world_interface)
            (`self.SetObjectInteractionState` true)
            (`SkeletalMeshComponent.PlayAnimation` (`self.SkeletalMesh`) "/Game/Occam/5_Props/Chest/AM_Occam_Chest_Open.AM_Occam_Chest_Open" false)
            (`self.OnInteractionDisabled`))
          (else
            (`KismetSystemLibrary.PrintString` "No Items in Chest")))))
    (:`Is Not Valid`
      (`KismetSystemLibrary.PrintString` "player not vaild"))))

(fn `AddItemsFromChestToInventory`
  (params (InventoryManager :type "/Game/Occam/2_Blueprints/0_Components/AC_Occam_InventoryManager Object Reference"))
  (bind _result (`BlueprintSetLibrary.Set_ToArray` (`self.ItemsInChest`)))
  (for _array_element _result
    (bind (_itemhardcodedname _itemtype _stacksamount) (break `/Game/Occam/2_Blueprints/2_Structures/Items/Strut_Occam_Loot_Data` _array_element))
    (`/Game/Occam/2_Blueprints/0_Components/AC_Occam_InventoryManager.AddItemToInventory` InventoryManager _itemhardcodedname _itemtype _stacksamount)))

(fn `ConstructInteractionPopUpText`
  (params (WorldInterface :type "/Game/Occam/6_UI/2_Main_Widgets/WBP_WorldInterface Object Reference"))
  (bind _result (`BlueprintSetLibrary.Set_ToArray` (`self.ItemsInChest`)))
  (for _array_element _result
    (bind (_itemhardcodedname _itemtype _stacksamount) (break `/Game/Occam/2_Blueprints/2_Structures/Items/Strut_Occam_Loot_Data` _array_element))
    (bind (_hardcodedname _iteminventorydata) (`/Game/Occam/2_Blueprints/FL_Occam_CustomFunctionsLibrary.ItemTypeData_To_ItemInventoryData` _itemhardcodedname _itemtype))
    (bind _returnvalue (`|CreateWidget` "/Game/Occam/6_UI/0_Templates/WBP_Occam_Loot_InfoBar.WBP_Occam_Loot_InfoBar_C"))
    (`/Game/Occam/6_UI/0_Templates/WBP_Occam_Loot_InfoBar.SetLootInfo` _returnvalue (`KismetTextLibrary.Conv_NameToText` (`.DisplayName_26_6CBA5E024366E45830160E87514802B2` (break `/Game/Occam/2_Blueprints/2_Structures/Items/Strut_Occam_Item_Inventory_Data` _iteminventorydata))) _stacksamount)
    (`VerticalBox.AddChildToVerticalBox` (`/Game/Occam/6_UI/1_PopUp_Widgets/WBP_LootMenu.VB_Item_InfoBars` (`/Game/Occam/6_UI/2_Main_Widgets/WBP_WorldInterface.WBP_LootMenu` WorldInterface)) _returnvalue))
  (return))

(fn `UserConstructionScript`
  (`parent.UserConstructionScript`))