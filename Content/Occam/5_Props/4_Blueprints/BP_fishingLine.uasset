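; Fishing line prop that stretches a line mesh between its lure source's LineStart and its own location.
; The construction script aims and scales the mesh by distance, then adds foam particles and a ripple mesh if InWater, otherwise a Paper2D hook sprite.
; On Tick, dry lines play a wind timeline that sways the actor along Y and re-aims the mesh.
; In water, Tick plays WaterTime, which drives nothing.
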(event `self.ReceiveTick`
  (params (DeltaSeconds :type "Float (single-precision)"))
  (bind (_returnvalue_x _returnvalue_y _returnvalue_z) (`KismetMathLibrary.BreakVector` (`self.K2_GetActorLocation`)))
  (bind _returnvalue (`self.K2_GetActorLocation`))
  (bind _returnvalue_2 (`SceneComponent.K2_GetComponentLocation` (`/Game/Occam/5_Props/4_Blueprints/BP_prop_fishinPole_wLine.LineStart` (`self.LureSource`))))
  (if (`self.inWater?`)
    (bind (_direction _sin) (`Timeline|waterTime`))
    (else
      (bind (_direction_2 _sin_2) (`Timeline|windTime`)
        (:`Update`
          (`self.K2_SetActorLocation` (`KismetMathLibrary.MakeVector` _returnvalue_x (+ (* _sin_2 0.25) _returnvalue_y) _returnvalue_z))
          (`SceneComponent.K2_SetRelativeTransform` (`self.sm_line`) (`KismetMathLibrary.MakeTransform` (0.0 0.0 0.0) (`KismetMathLibrary.FindLookAtRotation` _returnvalue_2 _returnvalue) (`KismetMathLibrary.MakeVector` (/ (`KismetMathLibrary.Vector_Distance` _returnvalue_2 _returnvalue) -2.5) 1.0 1.0)) false false))))))

(fn `UserConstructionScript`
  (locals (BP_Ripple :type "/Game/Occam/3_Environment/0_LevelBlueprints/CartoonWaterBlueprints/BP_WaterRipple_River Object Reference"))
  (bind _returnvalue (`self.K2_GetActorLocation`))
  (bind _returnvalue_2 (`SceneComponent.K2_GetComponentLocation` (`/Game/Occam/5_Props/4_Blueprints/BP_prop_fishinPole_wLine.LineStart` (`self.LureSource`))))
  (bind _returnvalue_3 (`AddComponent|NODE_AddStaticMeshComponent-0` :`RelativeTransform` (`KismetMathLibrary.MakeTransform` (0.0 0.0 0.0) (`KismetMathLibrary.FindLookAtRotation` _returnvalue_2 _returnvalue) (`KismetMathLibrary.MakeVector` (/ (`KismetMathLibrary.Vector_Distance` _returnvalue_2 _returnvalue) -2.5) 1.0 1.0))))
  (set `self.sm_line` _returnvalue_3)
  (if (`self.inWater?`)
    (bind _returnvalue_4 (`AddComponent|NODE_AddParticleSystemComponent-0`))
    (set `self.part_foam` _returnvalue_4)
    (bind _returnvalue_5 (`AddComponent|NODE_AddStaticMeshComponent-2`))
    (set `self.sm_ripple` _returnvalue_5)
    (else
      (bind _returnvalue_6 (`AddComponent|NODE_AddPaperSpriteComponent-1` :`RelativeTransform` (`KismetMathLibrary.MakeTransform` (0.0 0.0 -20.0) (struct :`Yaw` 90.0) (2.5 2.5 2.5))))
      (set `self.p_Hook` _returnvalue_6))))