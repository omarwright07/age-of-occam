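; Base Blueprint for Occam interaction objects that tests the player's skill grade against a requirement when interaction is requested.
; With SkillCheck enabled, it converts the first SkillRequirement entry and the matching GameInstance PlayerSkills grade to integers, passing on equal or higher.
; It prints a colored success or failure message and returns a bool, which the interaction event currently leaves unused.
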(event `/Game/Occam/2_Blueprints/4_Interfaces/BPI_Occam_Interaction.OnInteractionRequested`
  (params (PlayerWorldCharacter :type "/Game/Occam/2_Blueprints/5_GameBaseActors/BP_Occam_Character_Player_World Object Reference"))
  (`/Engine/EditorBlueprintResources/StandardMacros.IsValid` PlayerWorldCharacter
    (:`Is Valid`
      (`self.Interaction Skill Check`))))

(fn `Interaction Skill Check`
  (returns (`SkillCheckSuccessful?` :type Boolean))
  (bind _skillrequirement (`self.SkillRequirement`))
  (if (`self.SkillCheck?`)
    (bind _asbp_occam_gi_general (cast `/Game/Occam/2_Blueprints/BP_Occam_GI_General` (`GameplayStatics.GetGameInstance`)))
    (bind _keys (`BlueprintMapLibrary.Map_Keys` _skillrequirement))
    (bind _output (`|GetArrayItem` _keys))
    (bind _value (`BlueprintMapLibrary.Map_Find` (`/Game/Occam/2_Blueprints/BP_Occam_GI_General.PlayerSkills` _asbp_occam_gi_general) _output))
    (bind _value_2 (`BlueprintMapLibrary.Map_Find` _skillrequirement _output))
    (`/Engine/EditorBlueprintResources/StandardMacros.CompareInt` (`/Game/Occam/2_Blueprints/FL_Occam_CustomFunctionsLibrary.SkillsGradeToInteger` _value) (`/Game/Occam/2_Blueprints/FL_Occam_CustomFunctionsLibrary.SkillsGradeToInteger` _value_2)
      (:`>`
        _)
      (:`==`
        _)
      (:`<`
        (bind _text (`/Game/Occam/2_Blueprints/FL_Occam_CustomFunctionsLibrary.SkillsToText` _output))
        (bind _text_2 (`/Game/Occam/2_Blueprints/FL_Occam_CustomFunctionsLibrary.SkillsGradeToText` _value_2))
        (bind _text_3 (`/Game/Occam/2_Blueprints/FL_Occam_CustomFunctionsLibrary.SkillsGradeToText` _value))
        (`KismetSystemLibrary.PrintString` (`KismetTextLibrary.Conv_TextToString` (`|FormatText` "FAILED | Skill Check for \"{0}\" - Requires {1} - Player's Skill {2}" _text _text_2 _text_3)) true true (struct :`R` 1.0 :`B` 0.226903 :`A` 1.0) 20.0)
        (return false)))
    (`KismetSystemLibrary.PrintString` (`KismetTextLibrary.Conv_TextToString` (`|FormatText` "SUCCESS | Skill Check for \"{0}\" - Requires {1} - Player's Skill {2}" _text _text_2 _text_3)) true true (struct :`R` 0.135668 :`G` 1.0 :`B` 0.415117 :`A` 1.0) 20.0)
    (return true)
    (else
      (return false))))

(fn `UserConstructionScript`
  (`parent.UserConstructionScript`))