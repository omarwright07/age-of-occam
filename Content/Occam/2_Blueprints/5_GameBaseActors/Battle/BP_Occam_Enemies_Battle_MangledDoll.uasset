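; Battle enemy Blueprint for the Mangled Doll, defining its AI turn as a basic attack on a random player character.
; PerformActionbyAI shows an attack tooltip and ends the character's turn through the battle manager, then applies damage after a short delay.
; Damage and crit values come from the doll's battle stats component, with crit rate and power reading the same stat.
; After a second delay, it resumes the battle.
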(event `self.PerformActionByAI`
  (bind _battlemanagerreference (`self.BattleManagerReference`))
  (bind _playercharacters (`/Game/Occam/2_Blueprints/0_Components/AC_Occam_BattleManager.PlayerCharacters` (`self.BattleManagerReference`)))
  (bind _characterstats (`/Game/Occam/2_Blueprints/0_Components/AC_Occam_CharacterBattleStats.CharacterStats` (`self.AC_Occam_CharacterBattleStats`)))
  (bind _value (`BlueprintMapLibrary.Map_Find` _characterstats "NewEnumerator6"))
  (`/Game/Occam/2_Blueprints/0_Components/AC_Occam_BattleManager.ShowBattleTooltip` _battlemanagerreference (`|FormatText` "{0} Attacks" (`KismetTextLibrary.Conv_StringToText` (`/Game/Occam/2_Blueprints/0_Components/AC_Occam_CharacterBattleStats.CharacterDisplayName` (`self.AC_Occam_CharacterBattleStats`)))))
  (`/Game/Occam/2_Blueprints/0_Components/AC_Occam_BattleManager.EndCharacterTurn` _battlemanagerreference)
  (`KismetSystemLibrary.Delay` 0.3)
  (bind _output_get (set `self.Targeted` (`|GetArrayItem` _playercharacters (`KismetMathLibrary.RandomIntegerInRange` 0 (- (`KismetArrayLibrary.Array_Length` _playercharacters) 1)))))
  (`/Game/Occam/2_Blueprints/0_Components/AC_Occam_CharacterBattleStats.ReceiveDamage` (`/Game/Occam/2_Blueprints/5_GameBaseActors/Battle/BP_Occam_Character_Battle_Base.AC_Occam_CharacterBattleStats` _output_get) (`BlueprintMapLibrary.Map_Find` _characterstats "NewEnumerator1") _value _value "NewEnumerator0")
  (`KismetSystemLibrary.Delay` 0.5)
  ;[1 1 1] Add all the battle stuff before this
  (`/Game/Occam/2_Blueprints/0_Components/AC_Occam_BattleManager.ResumeBattle` _battlemanagerreference))

(fn `UserConstructionScript`
  (`parent.UserConstructionScript`))