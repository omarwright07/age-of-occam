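; Base Blueprint for player characters in Occam battles, handling combat events and action costs.
; On death it sets the dead flag, clears defending and notifies the battle manager; damage and resurrection pass through to the parent, with damage meant for child overrides.
; Attacks apply their effect and restore SP.
; Magic and skill actions only deduct MP, SP and HP costs looked up from the player controller's actions manager component.
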(event `/Game/Occam/2_Blueprints/4_Interfaces/BPI_Occam_BattleCommunication.OnDeath`
  (set `self.Dead?` true)
  (set `/Game/Occam/2_Blueprints/0_Components/AC_Occam_CharacterBattleStats.Defending` false (`self.AC_Occam_CharacterBattleStats`))
  (bind _battlemanagerreference (`self.BattleManagerReference`)
    (:`then`
      (`/Game/Occam/2_Blueprints/0_Components/AC_Occam_BattleManager.OnPlayerCharacterKilled` _battlemanagerreference self))
    (:`else`)))

(event `/Game/Occam/2_Blueprints/4_Interfaces/BPI_Occam_BattleCommunication.OnDamageReceived`
  (params (Damage :type Integer) (`Critical?` :type Boolean))
  ;[1 1 1] Made to be call in children
  (`parent.OnDamageReceived` Damage `Critical?`))

(event `/Game/Occam/2_Blueprints/4_Interfaces/BPI_Occam_BattleCommunication.OnResurrected`
  (params (HealAmount :type Integer))
  ;[1 1 1] Made to be call in children
  (`parent.OnResurrected` HealAmount))

(event `self.ExecuteAttackAction`
  (`self.ApplyAttackEffect`)
  (`/Game/Occam/2_Blueprints/0_Components/AC_Occam_CharacterBattleStats.RecoverSP` (`self.AC_Occam_CharacterBattleStats`) 25))

(event `self.ExecuteMagicAction`
  (params (MagicName :type Name))
  (bind _ac_occam_characterbattlestats (`self.AC_Occam_CharacterBattleStats`))
  (bind (_cost_mp _cost_sp _cost_hp) (`/Game/Occam/2_Blueprints/0_Components/AC_Occam_ActionsManager.GetActionCost` (`self.GetComponentByClass` (`GameplayStatics.GetPlayerController` 0) "/Game/Occam/2_Blueprints/0_Components/AC_Occam_ActionsManager.AC_Occam_ActionsManager_C") MagicName))
  (`/Game/Occam/2_Blueprints/0_Components/AC_Occam_CharacterBattleStats.ReduceMP` _ac_occam_characterbattlestats _cost_mp)
  (`/Game/Occam/2_Blueprints/0_Components/AC_Occam_CharacterBattleStats.ReduceSP` _ac_occam_characterbattlestats _cost_sp)
  (`/Game/Occam/2_Blueprints/0_Components/AC_Occam_CharacterBattleStats.ReduceHP` _ac_occam_characterbattlestats _cost_hp))

(event `self.ExecuteSkillsAction`
  (params (SkillsName :type Name))
  (bind _ac_occam_characterbattlestats (`self.AC_Occam_CharacterBattleStats`))
  (bind (_cost_mp _cost_sp _cost_hp) (`/Game/Occam/2_Blueprints/0_Components/AC_Occam_ActionsManager.GetActionCost` (`self.GetComponentByClass` (`GameplayStatics.GetPlayerController` 0) "/Game/Occam/2_Blueprints/0_Components/AC_Occam_ActionsManager.AC_Occam_ActionsManager_C") SkillsName))
  (`/Game/Occam/2_Blueprints/0_Components/AC_Occam_CharacterBattleStats.ReduceMP` _ac_occam_characterbattlestats _cost_mp)
  (`/Game/Occam/2_Blueprints/0_Components/AC_Occam_CharacterBattleStats.ReduceSP` _ac_occam_characterbattlestats _cost_sp)
  (`/Game/Occam/2_Blueprints/0_Components/AC_Occam_CharacterBattleStats.ReduceHP` _ac_occam_characterbattlestats _cost_hp))

(fn `UserConstructionScript`
  (`parent.UserConstructionScript`))