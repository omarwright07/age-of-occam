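; Base battle character for Occam's turn-based combat, handling cursor targeting, action dispatch and combat feedback.
; Capsule hover drives the TargetingManager and flipbook pointer; clicking a targeted character requests execution from the BattleManager.
; ExecuteAction routes action types to empty events, interface events spawn damage/heal pop-ups or flag death, and turn-number checks track temporary inactivity.
; ApplyAttackEffect only prints debug text; its damage loop is disconnected.
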(event `self.ReceiveBeginPlay`
  (`PaperFlipbookComponent.SetLooping` (`self.FB_Pointer`) false))

(event `self.TargetingCapsule.OnBeginCursorOver`
  (params (TouchedComponent :type "PrimitiveComponent Object Reference"))
  ;[1 1 1] During battle, if targeting is enabled, it will show or hide TargetPointer over targeted characters
  (bind _targetingmanagerreference (`self.TargetingManagerReference`)
    (:`then`
      (if (`/Game/Occam/2_Blueprints/0_Components/AC_Occam_TargetingManager.TargetingEnabled?` _targetingmanagerreference)
        (`/Game/Occam/2_Blueprints/0_Components/AC_Occam_TargetingManager.ShowTargets` _targetingmanagerreference self)))
    (:`else`)))

(event `self.TargetingCapsule.OnEndCursorOver`
  (params (TouchedComponent :type "PrimitiveComponent Object Reference"))
  (bind _fb_pointer (`self.FB_Pointer`))
  ;[1 1 1] During battle, if targeting is enabled, it will show or hide TargetPointer over targeted characters
  (bind _targetingmanagerreference (`self.TargetingManagerReference`)
    (:`then`
      (if (`/Game/Occam/2_Blueprints/0_Components/AC_Occam_TargetingManager.TargetingEnabled?` _targetingmanagerreference)
        (`/Game/Occam/2_Blueprints/0_Components/AC_Occam_TargetingManager.HideTargets` _targetingmanagerreference)
        (`PaperFlipbookComponent.ReverseFromEnd` _fb_pointer)
        (`KismetSystemLibrary.Delay` (`PaperFlipbookComponent.GetFlipbookLength` _fb_pointer))
        (`SceneComponent.SetVisibility` _fb_pointer false false)))
    (:`else`)))

(event `self.TargetingCapsule.OnClicked`
  (params (TouchedComponent :type "PrimitiveComponent Object Reference") (ButtonPressed :type "Key Structure"))
  (bind _fb_pointer (`self.FB_Pointer`))
  (bind _targetingmanagerreference (`self.TargetingManagerReference`)
    (:`then`
      (if (`/Game/Occam/2_Blueprints/0_Components/AC_Occam_TargetingManager.TargetingEnabled?` _targetingmanagerreference)
        (`PaperFlipbookComponent.ReverseFromEnd` _fb_pointer)
        (`KismetSystemLibrary.Delay` (`PaperFlipbookComponent.GetFlipbookLength` _fb_pointer))
        (`SceneComponent.SetVisibility` _fb_pointer false false)
        (bind _targetedcharacters (`/Game/Occam/2_Blueprints/0_Components/AC_Occam_TargetingManager.TargetedCharacters` _targetingmanagerreference))
        (if (`KismetArrayLibrary.Array_Contains` _targetedcharacters self)
          (bind _battlemanagerreference (`self.BattleManagerReference`)
            (:`then`
              (`/Game/Occam/2_Blueprints/0_Components/AC_Occam_BattleManager.RequestActionExecution` _battlemanagerreference _targetedcharacters))
            (:`else`)))))
    (:`else`)))

(event `/Game/Occam/2_Blueprints/4_Interfaces/BPI_Occam_BattleCommunication.OnDamageReceived`
  (params (Damage :type Integer) (`Critical?` :type Boolean))
  (`|SpawnActorFromClass` "/Game/Occam/2_Blueprints/5_GameBaseActors/BP_Occam_DamagePopUp.BP_Occam_DamagePopUp_C" (`KismetMathLibrary.MakeTransform` (`SceneComponent.K2_GetComponentLocation` (`self.FB_Pointer`))) "Undefined" "OverrideRootScale" null Damage `Critical?` false false null))

(event `/Game/Occam/2_Blueprints/4_Interfaces/BPI_Occam_BattleCommunication.OnHealed`
  (params (HealAmount :type Integer) (`RestoredMP?` :type Boolean))
  (`|SpawnActorFromClass` "/Game/Occam/2_Blueprints/5_GameBaseActors/BP_Occam_DamagePopUp.BP_Occam_DamagePopUp_C" (`self.GetTransform`) "Undefined" "OverrideRootScale" null HealAmount false true `RestoredMP?` null))

(event `/Game/Occam/2_Blueprints/4_Interfaces/BPI_Occam_BattleCommunication.OnDeath`
  (set `self.Dead?` true)
  (set `/Game/Occam/2_Blueprints/0_Components/AC_Occam_CharacterBattleStats.Defending` false (`self.AC_Occam_CharacterBattleStats`)))

(event `/Game/Occam/2_Blueprints/4_Interfaces/BPI_Occam_BattleCommunication.OnResurrected`
  (params (HealAmount :type Integer))
  (`|SpawnActorFromClass` "/Game/Occam/2_Blueprints/5_GameBaseActors/BP_Occam_DamagePopUp.BP_Occam_DamagePopUp_C" (`KismetMathLibrary.MakeTransform` (`SceneComponent.K2_GetComponentLocation` (`self.FB_Pointer`))) "Undefined" "OverrideRootScale" null HealAmount false true false null))

(event `ExecuteAttackAction`)

(event `ExecuteAction`
  (params (`Action Type` :type "/Game/Occam/2_Blueprints/3_Enumerations/Other/Enum_Occam_ActionType Enum" :default "NewEnumerator0") (`Secondary Action Name` :type Name))
  (switch `/Game/Occam/2_Blueprints/3_Enumerations/Other/Enum_Occam_ActionType` `Action Type`
    (:`NewEnumerator1`
      (`self.ExecuteAttackAction`))
    (:`NewEnumerator9`
      (`self.ExecuteDefendAction`))
    (:`NewEnumerator2`
      (`self.ExecuteMagicAction` `Secondary Action Name`))
    (:`NewEnumerator3`
      (`self.ExecuteSkillsAction` `Secondary Action Name`))
    (:`NewEnumerator4`
      (`self.ExecuteItemAction` `Secondary Action Name`))
    (:`NewEnumerator5`
      (`self.ExecuteSwitchAction`))
    (:`NewEnumerator6`
      (`self.ExecuteRunAction`))))

(event `ExecuteDefendAction`)

(event `ExecuteMagicAction`
  (params (MagicName :type Name)))

(event `ExecuteSkillsAction`
  (params (SkillsName :type Name)))

(event `ExecuteItemAction`
  (params (ItemName :type Name)))

(event `ExecuteSwitchAction`)

(event `ExecuteRunAction`)

(fn `ActionMan - ActionEffect`
  (`/Game/Occam/2_Blueprints/0_Components/AC_Occam_ActionsManager.ActivateActionEffect` (`/Game/Occam/2_Blueprints/7_Controllers/BP_Occam_PController_Battle.AC_Occam_ActionsManager` (cast `/Game/Occam/2_Blueprints/7_Controllers/BP_Occam_PController_Battle` (`GameplayStatics.GetPlayerController` 0) :!pure true))))

(fn `ApplyAttackEffect`
  (`KismetSystemLibrary.PrintString` "Apply Attack Effect" true true (struct :`R` 0.797505 :`G` 1.0 :`A` 1.0) 15.0))

(fn `CheckForActiveTurn`
  (returns (`CanAct?` :type Boolean))
  (`KismetSystemLibrary.PrintString` "Check For Active Turn")
  (`/Engine/EditorBlueprintResources/StandardMacros.CompareInt` (`self.ActiveTurn#`)
    (:`>`
      (`/Engine/EditorBlueprintResources/StandardMacros.CompareInt` (`self.ActiveTurn#`) (`/Game/Occam/2_Blueprints/0_Components/AC_Occam_BattleManager.TurnNumber` (`self.BattleManagerReference`))
        (:`>`
          (return false))
        (:`==`
          _)
        (:`<`
          _))
      (set `self.ActiveTurn#` 0 :!label _label))
    (:`==`
      _)
    (:`<`
      (goto _label)))
  (return true))

(fn `PerformActionByAI`)

(fn `SetInactiveTurns`
  (bind _output_get (set `self.ActiveTurn#` (+ (`/Game/Occam/2_Blueprints/0_Components/AC_Occam_BattleManager.TurnNumber` (`self.BattleManagerReference`)) 2)))
  (`KismetSystemLibrary.PrintString` (`KismetTextLibrary.Conv_TextToString` (`|FormatText` "Disabled Tile Turn {0}" _output_get)) true true (struct :`R` 1.0 :`B` 0.381948 :`A` 1.0) 20.0))

(fn `ShowTargetPointer`
  (bind _fb_pointer (`self.FB_Pointer`))
  (`SceneComponent.SetVisibility` _fb_pointer true false)
  (`PaperFlipbookComponent.PlayFromStart` _fb_pointer))

(fn `UserConstructionScript`)