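; BP_Occam_Character_Player_World is a player character Blueprint, apparently for world play, that picks which nearby actor to interact with.
; GetNearestActorInInteractionRange scans ActorsInInteractionRange, tracking the shortest distance to the character in local variables.
; It stores the result in ActorToInteract and returns it, or returns without setting it when the array is empty.
; The construction script is empty, and the graphs shown do not populate the array.
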(fn `GetNearestActorInInteractionRange`
  (returns (`Nearest Actor` :type "Actor Object Reference"))
  (locals (Local_DistanceToNearestActorLocal :type "Float (double-precision)") (Local_NearestActor :type "Actor Object Reference"))
  (if (> (`KismetArrayLibrary.Array_Length` (`self.ActorsInInteractionRange`)) 0)
    (for _array_element (`self.ActorsInInteractionRange`)
      (bind _returnvalue (`self.GetDistanceTo` _array_element self))
      (if (< _returnvalue (`local.Local_DistanceToNearestActorLocal`))
        (set `local.Local_DistanceToNearestActorLocal` _returnvalue)
        (set `local.Local_NearestActor` _array_element)))
    (bind _output_get (set `self.ActorToInteract` (`local.Local_NearestActor`)))
    (return _output_get)
    (else
      (return null))))

(fn `UserConstructionScript`)