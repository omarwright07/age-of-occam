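; Player controller for Occam battles that bootstraps the encounter and handles battle input.
; Its construction script has the battle manager component create the battle interface.
; On BeginPlay it sets game-and-UI input with mouse cursor and events off when gamepad controls are enabled, then after a short delay spawns player characters and enemies, resumes battle and activates gamepad battle controls.
; Right mouse cancels targeting through the targeting manager.
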(event `self.ReceiveBeginPlay`
  (`WidgetBlueprintLibrary.SetInputMode_GameAndUIEx` self null "DoNotLock" false)
  (bind _output_get (set `self.bShowMouseCursor` (not (`/Game/Occam/2_Blueprints/0_Components/AC_Occam_GamepadControls.GamepadControlsEnabled?` (`self.AC_Occam_GamepadControls`)))))
  (bind _output_get_2 (set `self.bEnableMouseOverEvents` _output_get))
  (set `self.bEnableClickEvents` _output_get_2)
  (`KismetSystemLibrary.Delay` 0.2)
  (`|ExecutionSequence`
    (:`then_0`
      (`|ExecutionSequence`
        (:`then_0`
          (`/Game/Occam/2_Blueprints/0_Components/AC_Occam_BattleManager.SpawnPlayerCharacters` (`self.AC_Occam_BattleManager`)))
        (:`then_1`
          (`/Game/Occam/2_Blueprints/0_Components/AC_Occam_BattleManager.SpawnEnemies` (`self.AC_Occam_BattleManager`)))
        (:`then_2`
          (`/Game/Occam/2_Blueprints/0_Components/AC_Occam_BattleManager.ResumeBattle` (`self.AC_Occam_BattleManager`)))))
    (:`then_1`
      (`/Game/Occam/2_Blueprints/0_Components/AC_Occam_GamepadControls.ActivateGamepadControls_Battle` (`self.AC_Occam_GamepadControls`)))))

(event `Key|RightMouseButton`
  (params (Key :type "Key Structure"))
  (:`Pressed`
    (`/Game/Occam/2_Blueprints/0_Components/AC_Occam_TargetingManager.CancelTargeting` (`self.AC_Occam_TargetingManager`))))

(event `InputAction|D-PadUp` :paused true
  (params (Key :type "Key Structure")))

(event `InputAction|D-PadDown` :paused true
  (params (Key :type "Key Structure")))

(event `InputAction|D-PadRight` :paused true
  (params (Key :type "Key Structure")))

(event `InputAction|D-PadLeft` :paused true
  (params (Key :type "Key Structure")))

(event `InputAction|AcceptButton` :paused true
  (params (Key :type "Key Structure")))

(event `InputAction|CancelButton` :paused true
  (params (Key :type "Key Structure")))

(event `InputAction|SelectButton` :paused true
  (params (Key :type "Key Structure")))

(event `InputAction|DiscardButton` :paused true
  (params (Key :type "Key Structure")))

(event `InputAction|ShoulderRight` :paused true
  (params (Key :type "Key Structure")))

(event `InputAction|TriggerRight` :paused true
  (params (Key :type "Key Structure")))

(event `InputAction|ShoulderLeft`
  (params (Key :type "Key Structure")))

(event `InputAction|TriggerLeft`
  (params (Key :type "Key Structure")))

(fn `UserConstructionScript`
  (`/Game/Occam/2_Blueprints/0_Components/AC_Occam_BattleManager.CreateBattleInterface` (`self.AC_Occam_BattleManager`)))