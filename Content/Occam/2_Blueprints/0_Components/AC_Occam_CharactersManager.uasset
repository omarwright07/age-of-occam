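; Actor component that manages Occam's RPG characters: roster, party membership and formation, XP and levels, stats, abilities and HP/MP recovery.
; All data lives in the game instance, cached on BeginPlay with a retry, and each edit writes the modified character or party struct back.
; XP gains loop through level-ups that apply per-level stats, also adjusting matching battle characters through the owner's BattleManager.
; Ability upgrades are capped by the actions DataTable.
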(event `self.ReceiveBeginPlay`
  (bind _asbp_occam_gi_general (cast `/Game/Occam/2_Blueprints/BP_Occam_GI_General` (`GameplayStatics.GetGameInstance`) :!label _label)
    (:`then`
      (set `self.GameInstanceReference` _asbp_occam_gi_general))
    (:`CastFailed`
      (`KismetSystemLibrary.Delay` 0.1)
      (goto _label))))

(fn `AddCharacterToParty`
  (params (CharacterHardcodedName :type Name))
  (if (< (`KismetArrayLibrary.Array_Length` (`/Game/Occam/2_Blueprints/BP_Occam_GI_General.CurrentParty` (`self.GameInstanceReference`))) (`self.MaxCharactersAmountInParty`))
    (if (not (`self.CheckIfThereIsCharacterInParty` CharacterHardcodedName))
      (`KismetArrayLibrary.Array_Add` (`/Game/Occam/2_Blueprints/BP_Occam_GI_General.CurrentParty` (`self.GameInstanceReference`)) (make `/Game/Occam/2_Blueprints/2_Structures/Strut_Occam_PartySlots` CharacterHardcodedName)))))

(fn `AddExperienceToCharacter`
  (params (Amount :type Integer) (CharacterHardcodedName :type Name))
  (locals (Local_GainedXP :type Integer) (Local_CharacterName :type Name) (Local_CharacterExperience :type Integer))
  (bind _characterscollection (`/Game/Occam/2_Blueprints/BP_Occam_GI_General.CharactersCollection` (`self.GameInstanceReference`)))
  (bind (_hardcodedname _displayname _charactericon _characteractorclass _currentlevel _currentxp) (break `/Game/Occam/2_Blueprints/2_Structures/Strut_Occam_CharacterSheet` (`BlueprintMapLibrary.Map_Find` (`/Game/Occam/2_Blueprints/BP_Occam_GI_General.CharactersCollection` (`self.GameInstanceReference`)) (`local.Local_CharacterName`))))
  (bind _xptonextlevel (`/Game/Occam/2_Blueprints/FL_Occam_CustomFunctionsLibrary.GetExperienceNeededToNextLevel` _currentlevel _currentxp))
  (set `local.Local_GainedXP` Amount)
  (set `local.Local_CharacterName` CharacterHardcodedName)
  (while (>= (`local.Local_GainedXP`) _xptonextlevel)
    (set `local.Local_GainedXP` (- (`local.Local_GainedXP`) _xptonextlevel))
    (`self.LevelUpCharacter` (`local.Local_CharacterName`)))
  (set `local.Local_CharacterExperience` (+ (`local.Local_GainedXP`) (`.CurrentXP_29_EC2BCCC24D76316C6AF1B898BBEC599A` (break `/Game/Occam/2_Blueprints/2_Structures/Strut_Occam_CharacterSheet` (`BlueprintMapLibrary.Map_Find` (`/Game/Occam/2_Blueprints/BP_Occam_GI_General.CharactersCollection` (`self.GameInstanceReference`)) (`local.Local_CharacterName`))))))
  ;[1 1 1] Push back update character data to Game Instance
  (bind _structout (setmembers `/Game/Occam/2_Blueprints/2_Structures/Strut_Occam_CharacterSheet` :`StructRef` (`BlueprintMapLibrary.Map_Find` _characterscollection (`local.Local_CharacterName`)) :`CurrentXP` (`local.Local_CharacterExperience`)))
  (`BlueprintMapLibrary.Map_Add` _characterscollection (`local.Local_CharacterName`) _structout))

(fn `AddNewCharacterToCollection`
  (params (CharacterSheet :type "/Game/Occam/2_Blueprints/2_Structures/Strut_Occam_CharacterSheet Structure"))
  (locals (Local_CharacterStruct :type "/Game/Occam/2_Blueprints/2_Structures/Strut_Occam_CharacterSheet Structure") (Local_CharacterEquipment :type "Map of /Game/Occam/2_Blueprints/3_Enumerations/Items/Enum_Occam_ItemSubtype Enum to /Game/Occam/2_Blueprints/2_Structures/Items/Strut_Occam_Equipment_StaticData Structure"))
  (bind _returnvalue (`KismetStringLibrary.Conv_StringToName` (`.HardcodedName_18_4AF2431E4AEBF3342AA55497D2301794` (break `/Game/Occam/2_Blueprints/2_Structures/Strut_Occam_CharacterSheet` (`local.Local_CharacterStruct`)))))
  (set `local.Local_CharacterStruct` CharacterSheet)
  (if (< (`BlueprintMapLibrary.Map_Length` (`/Game/Occam/2_Blueprints/BP_Occam_GI_General.CharactersCollection` (`self.GameInstanceReference`))) (`self.MaxCharactersAmountInCollection`))
    ;[1 1 1] Initially add character to game instance
    (`BlueprintMapLibrary.Map_Add` (`/Game/Occam/2_Blueprints/BP_Occam_GI_General.CharactersCollection` (`self.GameInstanceReference`)) (`KismetStringLibrary.Conv_StringToName` (`.HardcodedName_18_4AF2431E4AEBF3342AA55497D2301794` (break `/Game/Occam/2_Blueprints/2_Structures/Strut_Occam_CharacterSheet` (`local.Local_CharacterStruct`)))) (`local.Local_CharacterStruct`))
    ;[1 1 1] Read character equipment from data table and equip to character.
    (bind _output_get (set `local.Local_CharacterEquipment` (`.CharacterEquipment_61_0E814BA140B4B1C22FD97582B2DA4708` (break `/Game/Occam/2_Blueprints/2_Structures/Strut_Occam_CharacterSheet` (`local.Local_CharacterStruct`)))))
    (bind _keys (`BlueprintMapLibrary.Map_Keys` _output_get))
    (for _array_element _keys
      (`self.IncreaseCharacterStats` (`KismetStringLibrary.Conv_StringToName` (`.HardcodedName_18_4AF2431E4AEBF3342AA55497D2301794` (break `/Game/Occam/2_Blueprints/2_Structures/Strut_Occam_CharacterSheet` (`local.Local_CharacterStruct`)))) (`.Attributes_44_FE64B69F473E0BC189F57494D4ED8A5B` (break `/Game/Occam/2_Blueprints/2_Structures/Items/Strut_Occam_Equipment_StaticData` (`BlueprintMapLibrary.Map_Find` (`local.Local_CharacterEquipment`) _array_element)))))
    (`|ExecutionSequence`
      (:`then_0`
        ;[1 1 1] Update character equipment and overwrite character data in game instance.
        (bind _structout (setmembers `/Game/Occam/2_Blueprints/2_Structures/Strut_Occam_CharacterSheet` :`StructRef` (`BlueprintMapLibrary.Map_Find` (`/Game/Occam/2_Blueprints/BP_Occam_GI_General.CharactersCollection` (`self.GameInstanceReference`)) _returnvalue) :`CharacterEquipment` (`local.Local_CharacterEquipment`)))
        (`BlueprintMapLibrary.Map_Add` (`/Game/Occam/2_Blueprints/BP_Occam_GI_General.CharactersCollection` (`self.GameInstanceReference`)) _returnvalue _structout)))))

(fn `ChangeCharacterFormation`
  (params (CharacterHardcodedName :type Name))
  (for (_array_element _array_index) (`/Game/Occam/2_Blueprints/BP_Occam_GI_General.CurrentParty` (`self.GameInstanceReference`))
    (bind (_characterhardcodedname _position) (break `/Game/Occam/2_Blueprints/2_Structures/Strut_Occam_PartySlots` _array_element))
    (if (== _characterhardcodedname CharacterHardcodedName)
      ;[1 1 1] needs a custom system
      (bind _structout (setmembers `/Game/Occam/2_Blueprints/2_Structures/Strut_Occam_PartySlots` :`StructRef` _array_element :`Position` (select `/Game/Occam/2_Blueprints/3_Enumerations/Enum_Occam_FormationType` _position :`NewEnumerator0` "NewEnumerator1" :`NewEnumerator1` "NewEnumerator1" :!type "/Game/Occam/2_Blueprints/3_Enumerations/Enum_Occam_FormationType Enum")))
      (`KismetArrayLibrary.Array_Set` (`/Game/Occam/2_Blueprints/BP_Occam_GI_General.CurrentParty` (`self.GameInstanceReference`)) _array_index _structout)
      (break))))

(fn `CheckIfThereIsCharacterInParty`
  (params (CharacterHardcodedName :type Name))
  (returns (`Success?` :type Boolean) (SlotIndex :type Integer))
  (locals (`Local_Success?` :type Boolean) (Local_SlotIndex :type Integer))
  ;[1 1 1] Loop through all party members and check if there is one with desired name.
  (for (_array_element _array_index) (`/Game/Occam/2_Blueprints/BP_Occam_GI_General.CurrentParty` (`self.GameInstanceReference`))
    (if (== (`.CharacterHardCodedName_2_0AF74C8041E930247F05C38D59AB0B65` (break `/Game/Occam/2_Blueprints/2_Structures/Strut_Occam_PartySlots` _array_element)) CharacterHardcodedName)
      (set `local.Local_Success?` true)
      (set `local.Local_SlotIndex` _array_index)
      (break)))
  (return (`local.Local_Success?`) (`local.Local_SlotIndex`)))

(fn `DecreaseCharacterStats`
  (params (CharacterHardcodedName :type Name) (StatsChangeAmount :type "Map of /Game/Occam/2_Blueprints/3_Enumerations/Character/Enum_Occam_Attributes Enum to Integer"))
  (locals (Local_CharacterName :type Name) (Local_StatsChanges :type "Map of /Game/Occam/2_Blueprints/3_Enumerations/Character/Enum_Occam_Attributes Enum to Integer") (Local_CharacterStats :type "Map of /Game/Occam/2_Blueprints/3_Enumerations/Character/Enum_Occam_Attributes Enum to Integer"))
  (bind _local_characterstats (`local.Local_CharacterStats`))
  (set `local.Local_CharacterName` CharacterHardcodedName)
  (set `local.Local_StatsChanges` StatsChangeAmount)
  (set `local.Local_CharacterStats` (`.CharacterStats_40_04DF2AA248CFB5ADD971E896CCDD0228` (break `/Game/Occam/2_Blueprints/2_Structures/Strut_Occam_CharacterSheet` (`BlueprintMapLibrary.Map_Find` (`/Game/Occam/2_Blueprints/BP_Occam_GI_General.CharactersCollection` (`self.GameInstanceReference`)) (`local.Local_CharacterName`)))))
  (bind _keys (`BlueprintMapLibrary.Map_Keys` (`local.Local_StatsChanges`)))
  (for _array_element _keys
    (`BlueprintMapLibrary.Map_Add` _local_characterstats _array_element (- (`BlueprintMapLibrary.Map_Find` _local_characterstats _array_element) (`BlueprintMapLibrary.Map_Find` (`local.Local_StatsChanges`) _array_element))))
  ;[1 1 1] Push updated character struct back to Game Instance
  (bind _structout (setmembers `/Game/Occam/2_Blueprints/2_Structures/Strut_Occam_CharacterSheet` :`StructRef` (`BlueprintMapLibrary.Map_Find` (`/Game/Occam/2_Blueprints/BP_Occam_GI_General.CharactersCollection` (`self.GameInstanceReference`)) (`local.Local_CharacterName`)) :`CharacterStats` (`local.Local_CharacterStats`)))
  (`BlueprintMapLibrary.Map_Add` (`/Game/Occam/2_Blueprints/BP_Occam_GI_General.CharactersCollection` (`self.GameInstanceReference`)) (`local.Local_CharacterName`) _structout))

(fn `DegradeAbility`
  (params (CharacterName :type Name) (AbilityName :type Name))
  (locals (Local_CharacterName :type Name) (Local_AbilityName :type Name) (Local_CharacterAbility :type "Map of Name to Integer"))
  (bind _local_charactername (`local.Local_CharacterName`))
  (bind (_value _returnvalue) (`BlueprintMapLibrary.Map_Find` (`local.Local_CharacterAbility`) (`local.Local_AbilityName`)))
  (bind _characterscollection (`/Game/Occam/2_Blueprints/BP_Occam_GI_General.CharactersCollection` (`self.GameInstanceReference`)))
  (set `local.Local_CharacterName` CharacterName)
  (set `local.Local_AbilityName` AbilityName)
  (set `local.Local_CharacterAbility` (`.CharacterAbilities_53_5D52D75246043FF26F6C4E9983ACE7FA` (break `/Game/Occam/2_Blueprints/2_Structures/Strut_Occam_CharacterSheet` (`BlueprintMapLibrary.Map_Find` (`/Game/Occam/2_Blueprints/BP_Occam_GI_General.CharactersCollection` (`self.GameInstanceReference`)) (`local.Local_CharacterName`)))))
  (if _returnvalue
    (if (> _value 1)
      ;[1 1 1] Decrease ability level by 1
      (`BlueprintMapLibrary.Map_Add` (`local.Local_CharacterAbility`) (`local.Local_AbilityName`) (- (`BlueprintMapLibrary.Map_Find` (`local.Local_CharacterAbility`) (`local.Local_AbilityName`)) 1))
      (bind _structout (setmembers `/Game/Occam/2_Blueprints/2_Structures/Strut_Occam_CharacterSheet` :`StructRef` (`BlueprintMapLibrary.Map_Find` _characterscollection _local_charactername) :`CharacterAbilities` (`local.Local_CharacterAbility`)))
      (`BlueprintMapLibrary.Map_Add` _characterscollection _local_charactername _structout)
      (`self.RefreshSelectedAbilityData`))))

(fn `ForgetAbility`
  (params (CharacterName :type Name) (AbilityName :type Name))
  (locals (Local_CharacterName :type Name) (Local_AbilityName :type Name) (Local_CharacterAbility :type "Map of Name to Integer") (Local_ActionLevel :type Integer))
  (bind _local_charactername (`local.Local_CharacterName`))
  (bind (_value _returnvalue) (`BlueprintMapLibrary.Map_Find` (`local.Local_CharacterAbility`) (`local.Local_AbilityName`)))
  (bind _characterscollection (`/Game/Occam/2_Blueprints/BP_Occam_GI_General.CharactersCollection` (`self.GameInstanceReference`)))
  (set `local.Local_CharacterName` CharacterName)
  (set `local.Local_AbilityName` AbilityName)
  (set `local.Local_CharacterAbility` (`.CharacterAbilities_53_5D52D75246043FF26F6C4E9983ACE7FA` (break `/Game/Occam/2_Blueprints/2_Structures/Strut_Occam_CharacterSheet` (`BlueprintMapLibrary.Map_Find` (`/Game/Occam/2_Blueprints/BP_Occam_GI_General.CharactersCollection` (`self.GameInstanceReference`)) (`local.Local_CharacterName`)))))
  (if _returnvalue
    (set `local.Local_ActionLevel` _value)
    (`BlueprintMapLibrary.Map_Remove` (`local.Local_CharacterAbility`) (`local.Local_AbilityName`))
    (bind _structout (setmembers `/Game/Occam/2_Blueprints/2_Structures/Strut_Occam_CharacterSheet` :`StructRef` (`BlueprintMapLibrary.Map_Find` _characterscollection _local_charactername) :`CharacterAbilities` (`local.Local_CharacterAbility`)))
    (`BlueprintMapLibrary.Map_Add` _characterscollection _local_charactername _structout)))

(fn `IncreaseCharacterStats`
  (params (CharacterHardcodedName :type Name) (StatsChangeAmount :type "Map of /Game/Occam/2_Blueprints/3_Enumerations/Character/Enum_Occam_Attributes Enum to Integer"))
  (locals (Local_CharacterName :type Name) (Local_StatsChanges :type "Map of /Game/Occam/2_Blueprints/3_Enumerations/Character/Enum_Occam_Attributes Enum to Integer") (Local_CharacterStats :type "Map of /Game/Occam/2_Blueprints/3_Enumerations/Character/Enum_Occam_Attributes Enum to Integer"))
  (bind _local_characterstats (`local.Local_CharacterStats`))
  (set `local.Local_CharacterName` CharacterHardcodedName)
  (set `local.Local_StatsChanges` StatsChangeAmount)
  (set `local.Local_CharacterStats` (`.CharacterStats_40_04DF2AA248CFB5ADD971E896CCDD0228` (break `/Game/Occam/2_Blueprints/2_Structures/Strut_Occam_CharacterSheet` (`BlueprintMapLibrary.Map_Find` (`/Game/Occam/2_Blueprints/BP_Occam_GI_General.CharactersCollection` (`self.GameInstanceReference`)) (`local.Local_CharacterName`)))))
  (bind _keys (`BlueprintMapLibrary.Map_Keys` (`local.Local_StatsChanges`)))
  (for _array_element _keys
    (`BlueprintMapLibrary.Map_Add` _local_characterstats _array_element (+ (`BlueprintMapLibrary.Map_Find` _local_characterstats _array_element) (`BlueprintMapLibrary.Map_Find` (`local.Local_StatsChanges`) _array_element)))
    (switch `/Game/Occam/2_Blueprints/3_Enumerations/Character/Enum_Occam_Attributes` _array_element
      (:`NewEnumerator7`
        ;[1 1 1] On level up increase character current HP as well.
        (for _array_element_2 (`/Game/Occam/2_Blueprints/0_Components/AC_Occam_BattleManager.PlayerCharacters` (`Actor.GetComponentByClass` (`self.GetOwner`) "/Game/Occam/2_Blueprints/0_Components/AC_Occam_BattleManager.AC_Occam_BattleManager_C"))
          (bind _ac_occam_characterbattlestats (`/Game/Occam/2_Blueprints/5_GameBaseActors/Battle/BP_Occam_Character_Battle_Base.AC_Occam_CharacterBattleStats` _array_element_2))
          (if (`KismetStringLibrary.EqualEqual_StrStr` (`/Game/Occam/2_Blueprints/0_Components/AC_Occam_CharacterBattleStats.CharacterHardcodedName` _ac_occam_characterbattlestats) (`KismetStringLibrary.Conv_NameToString` (`local.Local_CharacterName`)))
            (set `/Game/Occam/2_Blueprints/0_Components/AC_Occam_CharacterBattleStats.CurrentHP` (+ (`/Game/Occam/2_Blueprints/0_Components/AC_Occam_CharacterBattleStats.CurrentHP` _ac_occam_characterbattlestats) (`BlueprintMapLibrary.Map_Find` (`local.Local_StatsChanges`) "NewEnumerator7")) _ac_occam_characterbattlestats)
            (break))))
      (:`NewEnumerator8`
        ;[1 1 1] On level up increase character current MP as well.
        (for _array_element_3 (`/Game/Occam/2_Blueprints/0_Components/AC_Occam_BattleManager.PlayerCharacters` (`Actor.GetComponentByClass` (`self.GetOwner`) "/Game/Occam/2_Blueprints/0_Components/AC_Occam_BattleManager.AC_Occam_BattleManager_C"))
          (bind _ac_occam_characterbattlestats_2 (`/Game/Occam/2_Blueprints/5_GameBaseActors/Battle/BP_Occam_Character_Battle_Base.AC_Occam_CharacterBattleStats` _array_element_3))
          (if (`KismetStringLibrary.EqualEqual_StrStr` (`/Game/Occam/2_Blueprints/0_Components/AC_Occam_CharacterBattleStats.CharacterHardcodedName` _ac_occam_characterbattlestats_2) (`KismetStringLibrary.Conv_NameToString` (`local.Local_CharacterName`)))
            (set `/Game/Occam/2_Blueprints/0_Components/AC_Occam_CharacterBattleStats.CurrentHP` (+ (`/Game/Occam/2_Blueprints/0_Components/AC_Occam_CharacterBattleStats.CurrentHP` _ac_occam_characterbattlestats_2) (`BlueprintMapLibrary.Map_Find` (`local.Local_StatsChanges`) "NewEnumerator8")) _ac_occam_characterbattlestats_2)
            (break))))))
  ;[1 1 1] Push updated character struct back to Game Instance
  (bind _structout (setmembers `/Game/Occam/2_Blueprints/2_Structures/Strut_Occam_CharacterSheet` :`StructRef` (`BlueprintMapLibrary.Map_Find` (`/Game/Occam/2_Blueprints/BP_Occam_GI_General.CharactersCollection` (`self.GameInstanceReference`)) (`local.Local_CharacterName`)) :`CharacterStats` (`local.Local_CharacterStats`)))
  (`BlueprintMapLibrary.Map_Add` (`/Game/Occam/2_Blueprints/BP_Occam_GI_General.CharactersCollection` (`self.GameInstanceReference`)) (`local.Local_CharacterName`) _structout))

(fn `LearnNewAbility`
  (params (Character :type Name) (AbilityName :type Name) (UpgradeIfAlreadyLearned :type Boolean))
  (locals (Local_Character :type Name) (Local_AbilityName :type Name) (Local_UpgradeIfExist :type Boolean) (Local_CharacterLearnedAbility :type "Map of Name to Integer"))
  (set `local.Local_Character` Character)
  (set `local.Local_AbilityName` AbilityName)
  (set `local.Local_UpgradeIfExist` UpgradeIfAlreadyLearned)
  (set `local.Local_CharacterLearnedAbility` (`.CharacterAbilities_53_5D52D75246043FF26F6C4E9983ACE7FA` (break `/Game/Occam/2_Blueprints/2_Structures/Strut_Occam_CharacterSheet` (`BlueprintMapLibrary.Map_Find` (`/Game/Occam/2_Blueprints/BP_Occam_GI_General.CharactersCollection` (`self.GameInstanceReference`)) (`local.Local_Character`)))))
  (if (`.ReturnValue` (`BlueprintMapLibrary.Map_Find` (`local.Local_CharacterLearnedAbility`) (`local.Local_AbilityName`)))
    (if (`local.Local_UpgradeIfExist`)
      (`self.UpgradeAbility` (`local.Local_Character`) (`local.Local_AbilityName`)))
    (else
      ;[1 1 1] Adds new action to character actions and saves it to character structure in game instance.
      (`BlueprintMapLibrary.Map_Add` (`local.Local_CharacterLearnedAbility`) (`local.Local_AbilityName`) 1)
      (bind _structout (setmembers `/Game/Occam/2_Blueprints/2_Structures/Strut_Occam_CharacterSheet` :`StructRef` (`BlueprintMapLibrary.Map_Find` (`/Game/Occam/2_Blueprints/BP_Occam_GI_General.CharactersCollection` (`self.GameInstanceReference`)) (`local.Local_Character`)) :`CharacterAbilities` (`local.Local_CharacterLearnedAbility`)))
      (`BlueprintMapLibrary.Map_Add` (`/Game/Occam/2_Blueprints/BP_Occam_GI_General.CharactersCollection` (`self.GameInstanceReference`)) (`local.Local_Character`) _structout))))

(fn `LevelUpCharacter`
  (params (CharacterHardcodedName :type Name))
  (locals (Local_CharacterName :type Name))
  (bind _value (`BlueprintMapLibrary.Map_Find` (`/Game/Occam/2_Blueprints/BP_Occam_GI_General.CharactersCollection` (`self.GameInstanceReference`)) (`local.Local_CharacterName`)))
  (bind (_hardcodedname _displayname _charactericon _characteractorclass _currentlevel _currentxp _currenthp _currentmp _currentsp _characterstats _statsperlevel) (break `/Game/Occam/2_Blueprints/2_Structures/Strut_Occam_CharacterSheet` _value))
  (set `local.Local_CharacterName` CharacterHardcodedName)
  (bind _structout (setmembers `/Game/Occam/2_Blueprints/2_Structures/Strut_Occam_CharacterSheet` :`StructRef` _value :`CurrentLevel` (+ _currentlevel 1) :`CurrentXP` 0))
  (`BlueprintMapLibrary.Map_Add` (`/Game/Occam/2_Blueprints/BP_Occam_GI_General.CharactersCollection` (`self.GameInstanceReference`)) (`local.Local_CharacterName`) _structout)
  (`self.IncreaseCharacterStats` (`local.Local_CharacterName`) _statsperlevel))

(fn `RecoverAllCharactersToFull`
  (bind _characterscollection (`/Game/Occam/2_Blueprints/BP_Occam_GI_General.CharactersCollection` (`self.GameInstanceReference`)))
  (bind _keys (`BlueprintMapLibrary.Map_Keys` _characterscollection))
  (for _array_element _keys
    (bind _value (`BlueprintMapLibrary.Map_Find` _characterscollection _array_element))
    (bind (_hardcodedname _displayname _charactericon _characteractorclass _currentlevel _currentxp _currenthp _currentmp _currentsp _characterstats) (break `/Game/Occam/2_Blueprints/2_Structures/Strut_Occam_CharacterSheet` _value))
    (bind _structout (setmembers `/Game/Occam/2_Blueprints/2_Structures/Strut_Occam_CharacterSheet` :`StructRef` _value :`CurrentHP` (`BlueprintMapLibrary.Map_Find` _characterstats "NewEnumerator7") :`CurrentMP` (`BlueprintMapLibrary.Map_Find` _characterstats "NewEnumerator8")))
    (`BlueprintMapLibrary.Map_Add` (`/Game/Occam/2_Blueprints/BP_Occam_GI_General.CharactersCollection` (`self.GameInstanceReference`)) _array_element _structout)))

(fn `RefreshSelectedAbilityData`)

(fn `RemoveCharacterFromParty`
  (params (CharacterHardcodedName :type Name))
  (bind (_success_ _slotindex) (`self.CheckIfThereIsCharacterInParty` CharacterHardcodedName))
  (if (> (`KismetArrayLibrary.Array_Length` (`/Game/Occam/2_Blueprints/BP_Occam_GI_General.CurrentParty` (`self.GameInstanceReference`))) 1)
    (if (not _success_)
      (`KismetArrayLibrary.Array_Remove` (`/Game/Occam/2_Blueprints/BP_Occam_GI_General.CurrentParty` (`self.GameInstanceReference`)) _slotindex))))

(fn `RestoreHP`
  (params (CharacterHardcodedName :type Name) (`HP Amount` :type Integer))
  (bind _value (`BlueprintMapLibrary.Map_Find` (`/Game/Occam/2_Blueprints/BP_Occam_GI_General.CharactersCollection` (`self.GameInstanceReference`)) CharacterHardcodedName))
  (bind (_hardcodedname _displayname _charactericon _characteractorclass _currentlevel _currentxp _currenthp _currentmp _currentsp _characterstats) (break `/Game/Occam/2_Blueprints/2_Structures/Strut_Occam_CharacterSheet` _value))
  (bind _structout (setmembers `/Game/Occam/2_Blueprints/2_Structures/Strut_Occam_CharacterSheet` :`StructRef` _value :`CurrentHP` (`KismetMathLibrary.Clamp` (+ `HP Amount` _currenthp) 0 (`BlueprintMapLibrary.Map_Find` _characterstats "NewEnumerator7"))))
  (`BlueprintMapLibrary.Map_Add` (`/Game/Occam/2_Blueprints/BP_Occam_GI_General.CharactersCollection` (`self.GameInstanceReference`)) CharacterHardcodedName _structout))

(fn `RestoreMP`
  (params (CharacterHardcodedName :type Name) (`MP Amount` :type Integer))
  (bind _value (`BlueprintMapLibrary.Map_Find` (`/Game/Occam/2_Blueprints/BP_Occam_GI_General.CharactersCollection` (`self.GameInstanceReference`)) CharacterHardcodedName))
  (bind (_hardcodedname _displayname _charactericon _characteractorclass _currentlevel _currentxp _currenthp _currentmp _currentsp _characterstats) (break `/Game/Occam/2_Blueprints/2_Structures/Strut_Occam_CharacterSheet` _value))
  (bind _structout (setmembers `/Game/Occam/2_Blueprints/2_Structures/Strut_Occam_CharacterSheet` :`StructRef` _value :`CurrentHP` (`KismetMathLibrary.Clamp` (+ `MP Amount` _currenthp) 0 (`BlueprintMapLibrary.Map_Find` _characterstats "NewEnumerator8"))))
  (`BlueprintMapLibrary.Map_Add` (`/Game/Occam/2_Blueprints/BP_Occam_GI_General.CharactersCollection` (`self.GameInstanceReference`)) CharacterHardcodedName _structout))

(fn `UpgradeAbility`
  (params (CharacterName :type Name) (AbilityName :type Name))
  (locals (Local_CharacterName :type Name) (Local_AbilityName :type Name) (Local_CharacterAbility :type "Map of Name to Integer"))
  (bind _local_charactername (`local.Local_CharacterName`))
  (bind _value (`BlueprintMapLibrary.Map_Find` (`local.Local_CharacterAbility`) (`local.Local_AbilityName`)))
  (bind _characterscollection (`/Game/Occam/2_Blueprints/BP_Occam_GI_General.CharactersCollection` (`self.GameInstanceReference`)))
  (set `local.Local_CharacterName` CharacterName)
  (set `local.Local_AbilityName` AbilityName)
  (set `local.Local_CharacterAbility` (`.CharacterAbilities_53_5D52D75246043FF26F6C4E9983ACE7FA` (break `/Game/Occam/2_Blueprints/2_Structures/Strut_Occam_CharacterSheet` (`BlueprintMapLibrary.Map_Find` (`/Game/Occam/2_Blueprints/BP_Occam_GI_General.CharactersCollection` (`self.GameInstanceReference`)) (`local.Local_CharacterName`)))))
  (if (`.ReturnValue` (`BlueprintMapLibrary.Map_Find` (`local.Local_CharacterAbility`) (`local.Local_AbilityName`)))
    (bind _returnvalue (`|GetDataTableRow` "/Game/Occam/2_Blueprints/1_Datatables/DT_Occam_Actions.DT_Occam_Actions" (`local.Local_AbilityName`))
      (:`then`
        (if (< _value (`.MaxLevel_17_A7B31DD14459EB607B2AD381CF0DBD30` (break `/Game/Occam/2_Blueprints/2_Structures/Strut_Occam_Action` _returnvalue)))
          (`BlueprintMapLibrary.Map_Add` (`local.Local_CharacterAbility`) (`local.Local_AbilityName`) (+ _value 1))
          (bind _structout (setmembers `/Game/Occam/2_Blueprints/2_Structures/Strut_Occam_CharacterSheet` :`StructRef` (`BlueprintMapLibrary.Map_Find` _characterscollection _local_charactername) :`CharacterAbilities` (`local.Local_CharacterAbility`)))
          (`BlueprintMapLibrary.Map_Add` _characterscollection _local_charactername _structout)
          (`self.RefreshSelectedAbilityData`))))))