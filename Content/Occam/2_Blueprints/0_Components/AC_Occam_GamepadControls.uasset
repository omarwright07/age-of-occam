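; Actor component that adds gamepad navigation to Occam's UI; so far only D-pad up is implemented, for the main menu and load-game save slots.
; Activation functions cache main menu or battle interface widget references, and a macro picks the active interface by checking which reference is valid.
; D-pad up moves the selected index and tints the focused button orange through highlight helpers.
; Other button handlers and world activation are empty stubs.
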(fn `ActivateGamepadControls_Battle`
  (bind _foundwidgets (`WidgetBlueprintLibrary.GetAllWidgetsOfClass` "/Game/Occam/6_UI/6_Battle_Widgets/WBP_Occam_BattleInterface.WBP_Occam_BattleInterface_C"))
  (set `self.WindowRef_BattleInterface` (`|GetArrayItem` _foundwidgets)))

(fn `ActivateGamepadControls_MainMenu`
  (bind _foundwidgets (`WidgetBlueprintLibrary.GetAllWidgetsOfClass` "/Game/Occam/6_UI/2_Main_Widgets/WBP_Occam_MainMenu.WBP_Occam_MainMenu_C"))
  (bind _output (`|GetArrayItem` _foundwidgets))
  (set `self.WindowRef_MainMenu` _output)
  (`self.HighlightMenuButton` true (`/Game/Occam/6_UI/2_Main_Widgets/WBP_Occam_MainMenu.BTN_NewGame` _output))
  (set `self.GamepadWindowFocus` "NewEnumerator0"))

(fn `ActivateGamepadControls_World`)

(fn `D-PadDownPressed`)

(fn `D-PadLeftPressed`)

(fn `D-PadRightPressed`)

(fn `D-PadUpPressed`
  (if (not (`self.YesNoWindowActive?`))
    (`self.SwitchOnActiveInterface`
      (:`MainMenu`
        (switch `/Game/Occam/2_Blueprints/3_Enumerations/GamepadControls/Enum_Gamepad_WindowFocus` (`self.GamepadWindowFocus`)
          (:`NewEnumerator0`
            (switch `int` (`self.CurrentlySelectedMenuButton`)
              (:`0`
                (`/Engine/EditorBlueprintResources/StandardMacros.DecrementInt` (`self.CurrentlySelectedMenuButton`)
                  (:`  `
                    (`self.HighlightMenuButton` false (`/Game/Occam/6_UI/2_Main_Widgets/WBP_Occam_MainMenu.BTN_LoadGame` (`self.WindowRef_MainMenu`)))
                    (`self.HighlightMenuButton` true (`/Game/Occam/6_UI/2_Main_Widgets/WBP_Occam_MainMenu.BTN_NewGame` (`self.WindowRef_MainMenu`))))))
              (:`1`
                (`/Engine/EditorBlueprintResources/StandardMacros.DecrementInt` (`self.CurrentlySelectedMenuButton`)
                  (:`  `
                    (`self.HighlightMenuButton` false (`/Game/Occam/6_UI/2_Main_Widgets/WBP_Occam_MainMenu.BTN_Settings` (`self.WindowRef_MainMenu`)))
                    (`self.HighlightMenuButton` true (`/Game/Occam/6_UI/2_Main_Widgets/WBP_Occam_MainMenu.BTN_LoadGame` (`self.WindowRef_MainMenu`))))))
              (:`2`
                (`/Engine/EditorBlueprintResources/StandardMacros.DecrementInt` (`self.CurrentlySelectedMenuButton`)
                  (:`  `
                    (`self.HighlightMenuButton` false (`/Game/Occam/6_UI/2_Main_Widgets/WBP_Occam_MainMenu.BTN_Quit` (`self.WindowRef_MainMenu`)))
                    (`self.HighlightMenuButton` true (`/Game/Occam/6_UI/2_Main_Widgets/WBP_Occam_MainMenu.BTN_Settings` (`self.WindowRef_MainMenu`))))))))
          (:`NewEnumerator14`
            (if (`KismetMathLibrary.Conv_IntToBool` (`self.CurrentlySelectedMenuButton`))
              (bind _aswbp_occam_save_slot_1 (cast `/Game/Occam/6_UI/3_Save_Widgets/WBP_Occam_SaveSlot1` (`PanelWidget.GetChildAt` (`/Game/Occam/6_UI/3_Save_Widgets/WBP_Occam_SaveMenu1.VB_SaveSlots` (`/Game/Occam/6_UI/2_Main_Widgets/WBP_Occam_MainMenu.WBP_Occam_SaveMenu` (`self.WindowRef_MainMenu`))) (`self.CurrentlySelectedMenuButton`))))
              ;[1 1 1] Add conditions for selection based on assigned save name
              (`self.HighlightSaveSlot` false (`/Game/Occam/6_UI/3_Save_Widgets/WBP_Occam_SaveSlot1.BTN_EmptySave` _aswbp_occam_save_slot_1))
              (`/Engine/EditorBlueprintResources/StandardMacros.DecrementInt` (`self.CurrentlySelectedMenuButton`)
                (:`  `
                  (bind _aswbp_occam_save_slot_1_2 (cast `/Game/Occam/6_UI/3_Save_Widgets/WBP_Occam_SaveSlot1` (`PanelWidget.GetChildAt` (`/Game/Occam/6_UI/3_Save_Widgets/WBP_Occam_SaveMenu1.VB_SaveSlots` (`/Game/Occam/6_UI/2_Main_Widgets/WBP_Occam_MainMenu.WBP_Occam_SaveMenu` (`self.WindowRef_MainMenu`))) (`self.CurrentlySelectedMenuButton`))))
                  (`self.HighlightSaveSlot` true (`/Game/Occam/6_UI/3_Save_Widgets/WBP_Occam_SaveSlot1.BTN_EmptySave` _aswbp_occam_save_slot_1_2)))))))))))

(fn `FaceButtonBottomPressed`)

(fn `FaceButtonLeftPressed`)

(fn `FaceButtonRightPressed`)

(fn `FaceButtonTopPressed`)

(fn `HighlightActionSlotInActionsScreen`
  (params (`Highlight?` :type Boolean) (Button :type "Button Object Reference"))
  (`/Engine/EditorBlueprintResources/StandardMacros.IsValid` Button
    (:`Is Valid`
      (`Button.SetBackgroundColor` Button (`KismetMathLibrary.SelectColor` (struct :`R` 1.0 :`G` 0.624415 :`A` 1.0) (struct :`R` 1.0 :`G` 1.0 :`B` 1.0 :`A` 1.0) `Highlight?`)))))

(fn `HighlightMenuButton`
  (params (`Highlight?` :type Boolean) (Button :type "Button Object Reference"))
  (`/Engine/EditorBlueprintResources/StandardMacros.IsValid` Button
    (:`Is Valid`
      (`Button.SetBackgroundColor` Button (`KismetMathLibrary.SelectColor` (struct :`R` 1.0 :`G` 0.624415 :`A` 1.0) (struct :`R` 1.0 :`G` 1.0 :`B` 1.0 :`A` 1.0) `Highlight?`)))))

(fn `HighlightSaveSlot`
  (params (`Highlight?` :type Boolean) (Button :type "Button Object Reference"))
  (`/Engine/EditorBlueprintResources/StandardMacros.IsValid` Button
    (:`Is Valid`
      (`Button.SetBackgroundColor` Button (`KismetMathLibrary.SelectColor` (struct :`R` 1.0 :`G` 0.624415 :`A` 1.0) (struct :`R` 1.0 :`G` 1.0 :`B` 1.0 :`A` 1.0) `Highlight?`)))))

(fn `ShoulderLeftPressed`)

(fn `ShoulderRightPressed`)

(fn `TriggerLeftPressed`)

(fn `TriggerRightPressed`)