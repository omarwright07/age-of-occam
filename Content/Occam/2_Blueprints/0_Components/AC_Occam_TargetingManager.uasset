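; Targeting manager component that decides which battle characters are highlighted as targets for the selected targeting type.
; Enable, disable and cancel functions toggle targeting state, with enabling also storing the type and self-targeting rule.
; ShowTargets filters by side, current turn or self rule, reveals pointers and records single or group targets from the battle manager.
; HideTargets hides those pointers and clears the list.
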(event `self.ReceiveBeginPlay`
  (bind _asbp_occam_gi_general (cast `/Game/Occam/2_Blueprints/00_SaveContainers/BP_Occam_GI_General` (`GameplayStatics.GetGameInstance`) :!label _label)
    (:`then`
      (set `self.GameInstanceReference` _asbp_occam_gi_general))
    (:`CastFailed`
      (`KismetSystemLibrary.Delay` 0.1)
      (goto _label))))

(fn `CancelTargeting`
  (if (`self.TargetingEnabled?`)
    (set `self.TargetingEnabled?` false)))

(fn `DisableTargeting`
  (set `self.TargetingEnabled?` false))

(fn `EnableTargeting`
  (params (`CanTargetSelf?` :type Boolean) (SelectedTargetingType :type "/Game/Occam/2_Blueprints/3_Enumerations/Other/Enum_Occam_TargetingType Enum" :default "NewEnumerator0"))
  (set `self.CanTargetSelf?` `CanTargetSelf?`)
  (set `self.SelectedTargetingType` SelectedTargetingType)
  (set `self.TargetingEnabled?` true))

(fn `HideTargets`
  (for _array_element (`self.TargetedCharacters`)
    (`SceneComponent.SetHiddenInGame` (`/Game/Occam/2_Blueprints/5_GameBaseActors/Battle/BP_Occam_Character_Battle_Base.FB_Pointer` _array_element) true false))
  (`KismetArrayLibrary.Array_Clear` (`self.TargetedCharacters`)))

(fn `ShowTargets`
  (params (IndicatedCharacter :type "/Game/Occam/2_Blueprints/5_GameBaseActors/Battle/BP_Occam_Character_Battle_Base Object Reference"))
  (locals (Local_IndicatedCharacter :type "/Game/Occam/2_Blueprints/5_GameBaseActors/Battle/BP_Occam_Character_Battle_Base Object Reference"))
  (bind _local_indicatedcharacter (`local.Local_IndicatedCharacter`))
  (bind _local_indicatedcharacter_2 (`local.Local_IndicatedCharacter`))
  (bind _local_indicatedcharacter_3 (`local.Local_IndicatedCharacter`))
  (set `local.Local_IndicatedCharacter` IndicatedCharacter)
  (switch `/Game/Occam/2_Blueprints/3_Enumerations/Other/Enum_Occam_TargetingType` (`self.SelectedTargetingType`)
    (:`NewEnumerator0`
      (if (== (`/Game/Occam/2_Blueprints/0_Components/AC_Occam_BattleManager.CurrentCharacter` (`/Game/Occam/2_Blueprints/5_GameBaseActors/Battle/BP_Occam_Character_Battle_Base.BattleManagerReference` (`local.Local_IndicatedCharacter`))) (`local.Local_IndicatedCharacter`))
        (`SceneComponent.SetHiddenInGame` (`/Game/Occam/2_Blueprints/5_GameBaseActors/Battle/BP_Occam_Character_Battle_Base.FB_Pointer` _local_indicatedcharacter) false false)
        (`KismetArrayLibrary.Array_Add` (`self.TargetedCharacters`) _local_indicatedcharacter)
        (`/Game/Occam/2_Blueprints/5_GameBaseActors/Battle/BP_Occam_Character_Battle_Base.ShowTargetPointer` _local_indicatedcharacter)))
    (:`NewEnumerator1`
      (if (`/Game/Occam/2_Blueprints/5_GameBaseActors/Battle/BP_Occam_Character_Battle_Base.Enemy?` (`local.Local_IndicatedCharacter`))
        (`SceneComponent.SetHiddenInGame` (`/Game/Occam/2_Blueprints/5_GameBaseActors/Battle/BP_Occam_Character_Battle_Base.FB_Pointer` _local_indicatedcharacter_2) false false)
        (`KismetArrayLibrary.Array_Add` (`self.TargetedCharacters`) _local_indicatedcharacter_2)
        (`/Game/Occam/2_Blueprints/5_GameBaseActors/Battle/BP_Occam_Character_Battle_Base.ShowTargetPointer` _local_indicatedcharacter_2)))
    (:`NewEnumerator2`
      (if (not (`/Game/Occam/2_Blueprints/5_GameBaseActors/Battle/BP_Occam_Character_Battle_Base.Enemy?` (`local.Local_IndicatedCharacter`)))
        (if (`self.CanTargetSelf?`)
          (`SceneComponent.SetHiddenInGame` (`/Game/Occam/2_Blueprints/5_GameBaseActors/Battle/BP_Occam_Character_Battle_Base.FB_Pointer` _local_indicatedcharacter_3) false false :!label _label)
          (`KismetArrayLibrary.Array_Add` (`self.TargetedCharacters`) _local_indicatedcharacter_3)
          (`/Game/Occam/2_Blueprints/5_GameBaseActors/Battle/BP_Occam_Character_Battle_Base.ShowTargetPointer` _local_indicatedcharacter_3)
          (elif (!= (`/Game/Occam/2_Blueprints/0_Components/AC_Occam_BattleManager.CurrentCharacter` (`/Game/Occam/2_Blueprints/5_GameBaseActors/Battle/BP_Occam_Character_Battle_Base.BattleManagerReference` (`local.Local_IndicatedCharacter`))) (`local.Local_IndicatedCharacter`))
            (goto _label)))))
    (:`NewEnumerator3`
      (if (`/Game/Occam/2_Blueprints/5_GameBaseActors/Battle/BP_Occam_Character_Battle_Base.Enemy?` (`local.Local_IndicatedCharacter`))
        (for _array_element (`/Game/Occam/2_Blueprints/0_Components/AC_Occam_BattleManager.Enemies` (`/Game/Occam/2_Blueprints/5_GameBaseActors/Battle/BP_Occam_Character_Battle_Base.BattleManagerReference` (`local.Local_IndicatedCharacter`)))
          (`SceneComponent.SetHiddenInGame` (`/Game/Occam/2_Blueprints/5_GameBaseActors/Battle/BP_Occam_Character_Battle_Base.FB_Pointer` _array_element) false false)
          (`KismetArrayLibrary.Array_Add` (`self.TargetedCharacters`) _array_element)
          (`/Game/Occam/2_Blueprints/5_GameBaseActors/Battle/BP_Occam_Character_Battle_Base.ShowTargetPointer` _array_element))))
    (:`NewEnumerator4`
      (if (not (`/Game/Occam/2_Blueprints/5_GameBaseActors/Battle/BP_Occam_Character_Battle_Base.Enemy?` (`local.Local_IndicatedCharacter`)))
        (for _array_element_2 (`/Game/Occam/2_Blueprints/0_Components/AC_Occam_BattleManager.PlayerCharacters` (`/Game/Occam/2_Blueprints/5_GameBaseActors/Battle/BP_Occam_Character_Battle_Base.BattleManagerReference` (`local.Local_IndicatedCharacter`)))
          (if (`self.CanTargetSelf?`)
            (`SceneComponent.SetHiddenInGame` (`/Game/Occam/2_Blueprints/5_GameBaseActors/Battle/BP_Occam_Character_Battle_Base.FB_Pointer` _array_element_2) false false :!label _label_2)
            (`KismetArrayLibrary.Array_Add` (`self.TargetedCharacters`) _array_element_2)
            (`/Game/Occam/2_Blueprints/5_GameBaseActors/Battle/BP_Occam_Character_Battle_Base.ShowTargetPointer` _array_element_2)
            (elif (!= _array_element_2 (`local.Local_IndicatedCharacter`))
              (goto _label_2))))))))