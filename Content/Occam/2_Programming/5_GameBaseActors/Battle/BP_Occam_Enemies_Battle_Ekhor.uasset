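; Battle actor for the Ekhor enemy in Occam, defining its AI turn in turn-based combat.
; On an active turn it calls RecoverGM if guard is depleted, then eases its sprite toward a side-dependent scene marker, performs a basic attack and eases back.
; If the turn check fails, it shows a disabled tooltip instead.
; Both paths end by resuming the battle manager after a short delay.
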(event `self.PerformActionByAI`
  (bind (_relativelocation_x _relativelocation_y _relativelocation_z) (`KismetMathLibrary.BreakVector` (`SceneComponent.RelativeLocation` (`self.Sprite`))))
  (bind (_relativelocation_x_2 _relativelocation_y_2) (`KismetMathLibrary.BreakVector` (`SceneComponent.RelativeLocation` (`self.Scene_MoveFrom`))))
  (bind (_relativelocation_x_3 _relativelocation_y_3 _relativelocation_z_2) (`KismetMathLibrary.BreakVector` (`SceneComponent.RelativeLocation` (`self.Sprite`))))
  (bind (_relativelocation_x_4 _relativelocation_y_4) (`KismetMathLibrary.BreakVector` (`SceneComponent.RelativeLocation` (select `bool` (`self.Enemy?`) :`false` (`self.Scene_MoveTo_Left`) :`true` (`self.Scene_MoveTo_Right`)))))
  (bind _canact_ (`self.CheckForActiveTurn`))
  (if _canact_
    (`/Engine/EditorBlueprintResources/StandardMacros.CompareInt` (`/Game/Occam/2_Programming/0_Components/AC_Occam_CharacterBattleStats.CurrentGuard` (`self.AC_Occam_CharacterBattleStats`))
      (:`>`
        _)
      (:`==`
        (`KismetSystemLibrary.Delay` 0.3 :!label _label)
        (`/Game/Occam/2_Programming/0_Components/AC_Occam_CharacterBattleStats.RecoverGM` (`self.AC_Occam_CharacterBattleStats`)))
      (:`<`
        (goto _label)))
    (`KismetSystemLibrary.Delay` 0.3)
    (`KismetSystemLibrary.MoveComponentTo` (`self.Sprite`) (`KismetMathLibrary.MakeVector` _relativelocation_x_4 _relativelocation_y_4 _relativelocation_z) (`SceneComponent.RelativeRotation` (`self.Sprite`)) false true)
    (`/Game/Occam/2_Programming/FL_Occam_Battle.BasicAttack` (`self.AC_Occam_CharacterBattleStats`) (`self.BattleManagerReference`))
    (`KismetSystemLibrary.MoveComponentTo` (`self.Sprite`) (`KismetMathLibrary.MakeVector` _relativelocation_x_2 _relativelocation_y_2 _relativelocation_z_2) (`SceneComponent.RelativeRotation` (`self.Sprite`)) true)
    (else
      (`/Game/Occam/2_Programming/0_Components/AC_Occam_BattleManager.ShowBattleTooltip` (`self.BattleManagerReference`) (`|FormatText` "{0} Is Disabled" (`KismetTextLibrary.Conv_StringToText` (`/Game/Occam/2_Programming/0_Components/AC_Occam_CharacterBattleStats.CharacterDisplayName` (`self.AC_Occam_CharacterBattleStats`)))))))
  ;[1 1 1] Add all the battle stuff before this
  (`KismetSystemLibrary.Delay` 0.5)
  (`/Game/Occam/2_Programming/0_Components/AC_Occam_BattleManager.ResumeBattle` (`self.BattleManagerReference`)))

(fn `UserConstructionScript`
  (`parent.UserConstructionScript`))