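; Player-controlled protagonist actor for Occam battles, a child Blueprint that plays Paper2D flipbook animations for actions and reactions.
; Action events show a battle manager tooltip, switch sprite, end the turn and resume battle; only Attack waits out its animation and triggers an action effect first.
; Death and resurrection are reported to the manager, while damage briefly swaps the sprite.
; Animations come from an enum-keyed flipbook map, with each change debug-printed.
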(event `/Game/Occam/2_Programming/4_Interfaces/BPI_Occam_BattleCommunication.OnDeath`
  (`self.ChangeSpriteToAnimation` "NewEnumerator5")
  (bind _battlemanagerreference (`self.BattleManagerReference`)
    (:`then`
      (`/Game/Occam/2_Programming/0_Components/AC_Occam_BattleManager.OnPlayerCharacterKilled` _battlemanagerreference self))
    (:`else`)))

(event `/Game/Occam/2_Programming/4_Interfaces/BPI_Occam_BattleCommunication.OnDamageReceived`
  (params (Damage :type Integer) (`Critical?` :type Boolean))
  (`parent.OnDamageReceived` Damage `Critical?`)
  (`self.ChangeSpriteToAnimation` "NewEnumerator10")
  (`KismetSystemLibrary.Delay` 0.2)
  (`self.ChangeSpriteToAnimation` "NewEnumerator1"))

(event `/Game/Occam/2_Programming/4_Interfaces/BPI_Occam_BattleCommunication.OnResurrected`
  (params (HealAmount :type Integer))
  (`parent.OnResurrected` HealAmount)
  (set `self.Dead?` false)
  (bind _battlemanagerreference (`self.BattleManagerReference`)
    (:`then`
      (`/Game/Occam/2_Programming/0_Components/AC_Occam_BattleManager.OnPlayerCharacterResurrected` _battlemanagerreference self))
    (:`else`)))

(event `self.ExecuteAttackAction`
  (bind _battlemanagerreference (`self.BattleManagerReference`))
  (`parent.ExecuteAttackAction`)
  (bind _battlemanagerreference_2 (`self.BattleManagerReference`)
    (:`then`
      (`/Game/Occam/2_Programming/0_Components/AC_Occam_BattleManager.ShowBattleTooltip` _battlemanagerreference_2 (`|FormatText` "{0} Attacks" (`KismetTextLibrary.Conv_StringToText` (`/Game/Occam/2_Programming/0_Components/AC_Occam_CharacterBattleStats.CharacterDisplayName` (`self.AC_Occam_CharacterBattleStats`)))))
      (`/Game/Occam/2_Programming/0_Components/AC_Occam_BattleManager.EndCharacterTurn` _battlemanagerreference)
      (`self.ChangeSpriteToAnimation` "NewEnumerator9")
      (`KismetSystemLibrary.Delay` (`PaperFlipbook.GetTotalDuration` (`BlueprintMapLibrary.Map_Find` (`self.CharactersActionsFlipbooks`) "NewEnumerator9")))
      (`self.ActionMan - ActionEffect`)
      (`self.ChangeSpriteToAnimation` "NewEnumerator1")
      (`/Game/Occam/2_Programming/0_Components/AC_Occam_BattleManager.ResumeBattle` _battlemanagerreference))
    (:`else`)))

(event `self.ExecuteItemAction`
  (params (ItemName :type Name))
  (bind _battlemanagerreference (`self.BattleManagerReference`))
  (bind _battlemanagerreference_2 (`self.BattleManagerReference`)
    (:`then`
      (`/Game/Occam/2_Programming/0_Components/AC_Occam_BattleManager.ShowBattleTooltip` _battlemanagerreference_2 (`|FormatText` "{0} Uses {1}" (`/Game/Occam/2_Programming/0_Components/AC_Occam_CharacterBattleStats.CharacterDisplayName` (`self.AC_Occam_CharacterBattleStats`)) (`/Game/Occam/2_Programming/FL_Occam_Custom.GetDisplayName_Items` ItemName)))
      (`self.ChangeSpriteToAnimation` "NewEnumerator3")
      (`/Game/Occam/2_Programming/0_Components/AC_Occam_BattleManager.EndCharacterTurn` _battlemanagerreference)
      (`/Game/Occam/2_Programming/0_Components/AC_Occam_BattleManager.ResumeBattle` _battlemanagerreference))
    (:`else`)))

(event `self.ExecuteMagicAction`
  (params (MagicName :type Name))
  (bind _battlemanagerreference (`self.BattleManagerReference`))
  (bind _battlemanagerreference_2 (`self.BattleManagerReference`)
    (:`then`
      (`/Game/Occam/2_Programming/0_Components/AC_Occam_BattleManager.ShowBattleTooltip` _battlemanagerreference_2 (`|FormatText` "{0} Casts {1}" (`/Game/Occam/2_Programming/0_Components/AC_Occam_CharacterBattleStats.CharacterDisplayName` (`self.AC_Occam_CharacterBattleStats`)) (`/Game/Occam/2_Programming/FL_Occam_Custom.GetDisplayName_Actions` MagicName)))
      (`self.ChangeSpriteToAnimation` "NewEnumerator3")
      (`/Game/Occam/2_Programming/0_Components/AC_Occam_BattleManager.EndCharacterTurn` _battlemanagerreference)
      (`/Game/Occam/2_Programming/0_Components/AC_Occam_BattleManager.ResumeBattle` _battlemanagerreference))
    (:`else`)))

(event `self.ExecuteSkillsAction`
  (params (SkillsName :type Name))
  (bind _battlemanagerreference (`self.BattleManagerReference`))
  (bind _battlemanagerreference_2 (`self.BattleManagerReference`)
    (:`then`
      (`/Game/Occam/2_Programming/0_Components/AC_Occam_BattleManager.ShowBattleTooltip` _battlemanagerreference_2 (`|FormatText` "{0} Performs {1}" (`/Game/Occam/2_Programming/0_Components/AC_Occam_CharacterBattleStats.CharacterDisplayName` (`self.AC_Occam_CharacterBattleStats`)) (`/Game/Occam/2_Programming/FL_Occam_Custom.GetDisplayName_Actions` SkillsName)))
      (`self.ChangeSpriteToAnimation` "NewEnumerator9")
      (`/Game/Occam/2_Programming/0_Components/AC_Occam_BattleManager.EndCharacterTurn` _battlemanagerreference)
      (`/Game/Occam/2_Programming/0_Components/AC_Occam_BattleManager.ResumeBattle` _battlemanagerreference))
    (:`else`)))

(fn `ChangeSpriteToAnimation`
  (params (BattleSprite :type "/Game/Occam/2_Programming/3_Enumerations/Character/Enum_Occam_BattleSprites Enum" :default "NewEnumerator0"))
  (`KismetSystemLibrary.PrintString` (`KismetTextLibrary.Conv_TextToString` (`|FormatText` "Change Sprite to Animation -- Protag - {1}" (`|GetEnumeratorNameAsString` BattleSprite))))
  (`PaperFlipbookComponent.SetFlipbook` (`self.Sprite`) (`BlueprintMapLibrary.Map_Find` (`self.CharactersActionsFlipbooks`) BattleSprite)))

(fn `UserConstructionScript`
  (`parent.UserConstructionScript`)
  (`self.ChangeSpriteToAnimation` "NewEnumerator1"))