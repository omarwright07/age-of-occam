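; Base actor for enemies in battle, linking each one to its battle slot widget and to the battle manager.
; On BeginPlay it polls the stats component on a short delay until a slot widget reference exists, then assigns it to its EnemyBattleWidget component, whose visibility can be toggled.
; On death it flags itself dead and notifies the battle manager, while damage events pass through to the parent class.
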(event `self.ReceiveBeginPlay`
  (bind _enemybattleslotreference (`/Game/Occam/2_Programming/0_Components/AC_Occam_CharacterBattleStats.EnemyBattleSlotReference` (`self.AC_Occam_CharacterBattleStats`)))
  (if (== _enemybattleslotreference null) :!label _label
    (`KismetSystemLibrary.Delay` 0.2)
    (goto _label)
    (else
      (`WidgetComponent.SetWidget` (`self.EnemyBattleWidget`) _enemybattleslotreference))))

(event `/Game/Occam/2_Programming/4_Interfaces/BPI_Occam_BattleCommunication.OnDeath`
  (set `self.Dead?` true)
  (bind _battlemanagerreference (`self.BattleManagerReference`)
    (:`then`
      (`/Game/Occam/2_Programming/0_Components/AC_Occam_BattleManager.OnEnemyKilled` _battlemanagerreference self))
    (:`else`)))

(event `/Game/Occam/2_Programming/4_Interfaces/BPI_Occam_BattleCommunication.OnDamageReceived`
  (params (Damage :type Integer) (`Critical?` :type Boolean))
  (`parent.OnDamageReceived` Damage `Critical?`))

(fn `HideOrShowEnemyBattleWidget`
  (params (`Show?` :type Boolean))
  (`SceneComponent.SetVisibility` (`self.EnemyBattleWidget`) `Show?` false))

(fn `UserConstructionScript`
  (`parent.UserConstructionScript`))