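; BP_Occam_Character_Player_World is the world player character, with a sprite, a spring-arm camera and helpers for interaction and indoor views.
; GetNearestActorInInteractionRange scans the actors in range by distance, stores the closest as ActorToInteract and returns it.
; ChangeCamera halves spring arm length and sprite scale when Indoor is true and doubles both otherwise, relative to current values, with a leftover debug print.
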(fn `Change Camera`
  (params (`Indoor?` :type Boolean))
  (bind _springarm (`self.SpringArm`))
  (bind _sprite (`self.Sprite`))
  (bind _targetarmlength (`SpringArmComponent.TargetArmLength` _springarm))
  (bind _relativescale3d (`SceneComponent.RelativeScale3D` _sprite))
  (`KismetSystemLibrary.PrintString` "Hello")
  (set `SpringArmComponent.TargetArmLength` (select `bool` `Indoor?` :`false` (* _targetarmlength 2.0) :`true` (/ _targetarmlength 2.0)) _springarm)
  (`SceneComponent.SetRelativeScale3D` _sprite (select `bool` `Indoor?` :`false` (* _relativescale3d 2.0) :`true` (/ _relativescale3d 2.0))))

(fn `GetNearestActorInInteractionRange`
  (returns (`Nearest Actor` :type "Actor Object Reference"))
  (locals (Local_DistanceToNearestActorLocal :type "Float (double-precision)") (Local_NearestActor :type "Actor Object Reference"))
  (if (> (`KismetArrayLibrary.Array_Length` (`self.ActorsInInteractionRange`)) 0)
    (for _array_element (`self.ActorsInInteractionRange`)
      (bind _returnvalue (`self.GetDistanceTo` _array_element self))
      (if (< _returnvalue (`local.Local_DistanceToNearestActorLocal`))
        (set `local.Local_DistanceToNearestActorLocal` _returnvalue)
        (set `local.Local_NearestActor` _array_element)))
    (bind _output_get (set `self.ActorToInteract` (`local.Local_NearestActor`)))
    (return _output_get)
    (else
      (return null))))

(fn `UserConstructionScript`)