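; An interaction object placed in the world that starts a one-time enemy encounter when the player walks into range.
; The first overlap of InteractionRange by the world player character passes EncounterName and a random battle map from the game instance to the controller's battle manager.
; A DoOnce blocks repeat triggers, and the actor destroys itself when its loaded interaction state is true.
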(event `self.ReceiveBeginPlay`
  (`parent.ReceiveBeginPlay`))

(event `/Game/Occam/2_Programming/4_Interfaces/BPI_Occam_Interaction.OnObjectInteractionStateLoaded`
  (params (InteractionState :type Boolean))
  (if InteractionState
    (`self.K2_DestroyActor`)))

(event `self.ReceiveTick`
  (params (DeltaSeconds :type "Float (single-precision)"))
  (`parent.ReceiveTick` DeltaSeconds))

(event `self.InteractionRange.OnComponentBeginOverlap`
  (params (OverlappedComponent :type "PrimitiveComponent Object Reference") (OtherActor :type "Actor Object Reference") (OtherComp :type "PrimitiveComponent Object Reference") (OtherBodyIndex :type Integer) (bFromSweep :type Boolean) (SweepResult :type "HitResult Structure (by ref)"))
  (bind _possiblebattlemaps (`/Game/Occam/2_Programming/8_SaveContainers/BP_Occam_GI_General.PossibleBattleMaps` (`self.GameInstanceReference`)))
  (bind _asbp_occam_character_player_world (cast `/Game/Occam/2_Programming/5_GameBaseActors/BP_Occam_Character_Player_World` OtherActor))
  (`/Engine/EditorBlueprintResources/StandardMacros.DoOnce` false
    (:`Completed`
      (`/Game/Occam/2_Programming/0_Components/AC_Occam_BattleManager.EncounterEnemies` (`/Game/Occam/2_Programming/7_Controllers/BP_Occam_PController_World.AC_Occam_BattleManager` (`/Game/Occam/2_Programming/5_GameBaseActors/BP_Occam_Character_Player_World.PlayerController` _asbp_occam_character_player_world)) (`self.EncounterName`) (`|GetArrayItem` _possiblebattlemaps (`KismetMathLibrary.RandomIntegerInRange` 0 (- (`KismetArrayLibrary.Array_Length` _possiblebattlemaps) 1)))))))

(fn `UserConstructionScript`
  (`parent.UserConstructionScript`))