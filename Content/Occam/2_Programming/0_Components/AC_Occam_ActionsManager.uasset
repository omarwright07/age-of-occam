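; Battle component that handles the current character's action choice in turn-based combat, working through sibling BattleManager and TargetingManager components.
; SelectAction stores the choice: Attack, Magic and Skills enable targeting, while Defend and Run resolve immediately.
; ActivateActionEffect covers only Attack, Defend and Run; Attack damages targets using the character's first data-table ability.
; Magic and Skills have no activation, Items does nothing, and GetActionCost reads MP/SP/HP costs from the actions table.
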(event `self.ReceiveBeginPlay`
  (bind _asbp_occam_gi_general (cast `/Game/Occam/2_Programming/8_SaveContainers/BP_Occam_GI_General` (`GameplayStatics.GetGameInstance`) :!label _label)
    (:`then`
      (set `self.GameInstanceReference` _asbp_occam_gi_general))
    (:`CastFailed`
      (`KismetSystemLibrary.Delay` 0.2)
      (goto _label))))

(event `SelectAction`
  (params (`Action Type` :type "/Game/Occam/2_Programming/3_Enumerations/Other/Enum_Occam_ActionType Enum" :default "NewEnumerator0") (`Secondary Action Name` :type Name))
  (bind _ac_occam_characterbattlestats (`/Game/Occam/2_Programming/5_GameBaseActors/Battle/BP_Occam_Character_Battle_Base.AC_Occam_CharacterBattleStats` (`self.GetCurrentCharacter`)))
  (set `/Game/Occam/2_Programming/0_Components/AC_Occam_CharacterBattleStats.SelectedActionType` `Action Type` _ac_occam_characterbattlestats)
  (set `/Game/Occam/2_Programming/0_Components/AC_Occam_CharacterBattleStats.SelectedSecondaryActionName` `Secondary Action Name` _ac_occam_characterbattlestats)
  (switch `/Game/Occam/2_Programming/3_Enumerations/Other/Enum_Occam_ActionType` `Action Type`
    (:`NewEnumerator1`
      (`self.Select_Attack`))
    (:`NewEnumerator9`
      (`self.Select_Defend`))
    (:`NewEnumerator2`
      (`self.Select_Magic`))
    (:`NewEnumerator3`
      (`self.Select_Skills`))
    (:`NewEnumerator4`
      (switch `name` (`/Game/Occam/2_Programming/0_Components/AC_Occam_CharacterBattleStats.SelectedSecondaryActionName` (`/Game/Occam/2_Programming/5_GameBaseActors/Battle/BP_Occam_Character_Battle_Base.AC_Occam_CharacterBattleStats` (`self.GetCurrentCharacter`)))))
    (:`NewEnumerator6`
      (`self.Select_Run`))))

(event `ActivateActionEffect`
  (switch `/Game/Occam/2_Programming/3_Enumerations/Other/Enum_Occam_ActionType` (`/Game/Occam/2_Programming/0_Components/AC_Occam_CharacterBattleStats.SelectedActionType` (`/Game/Occam/2_Programming/5_GameBaseActors/Battle/BP_Occam_Character_Battle_Base.AC_Occam_CharacterBattleStats` (`self.GetCurrentCharacter`)))
    (:`NewEnumerator1`
      (`self.Activate_Attack`))
    (:`NewEnumerator9`
      (`self.Activate_Defend`))
    (:`NewEnumerator6`
      (`self.Activate_Run`))))

(fn `Activate_Attack`
  (bind _ac_occam_characterbattlestats (`/Game/Occam/2_Programming/5_GameBaseActors/Battle/BP_Occam_Character_Battle_Base.AC_Occam_CharacterBattleStats` (`self.GetCurrentCharacter`)))
  (bind _ac_occam_characterbattlestats_2 (`/Game/Occam/2_Programming/5_GameBaseActors/Battle/BP_Occam_Character_Battle_Base.AC_Occam_CharacterBattleStats` (`self.GetCurrentCharacter`)))
  (`KismetSystemLibrary.PrintString` "ActionMan - Activate Attack" true true (struct :`G` 0.66 :`B` 1.0 :`A` 1.0) 15.0)
  (bind _returnvalue (`|GetDataTableRow` "/Game/Occam/2_Programming/1_Datatables/DT_Occam_PlayerCharacters.DT_Occam_PlayerCharacters" (`KismetStringLibrary.Conv_StringToName` (`/Game/Occam/2_Programming/0_Components/AC_Occam_CharacterBattleStats.CharacterHardcodedName` _ac_occam_characterbattlestats)))
    (:`then`
      (bind _result (`BlueprintSetLibrary.Set_ToArray` (`.Abilities_65_5D52D75246043FF26F6C4E9983ACE7FA` (break `/Game/Occam/2_Programming/2_Structures/Strut_Occam_CharacterSheet` _returnvalue))))
      (for _array_element (`/Game/Occam/2_Programming/0_Components/AC_Occam_CharacterBattleStats.TargetedCharacters` _ac_occam_characterbattlestats)
        (bind _ac_occam_characterbattlestats_3 (`/Game/Occam/2_Programming/5_GameBaseActors/Battle/BP_Occam_Character_Battle_Base.AC_Occam_CharacterBattleStats` _array_element))
        (`/Game/Occam/2_Programming/0_Components/AC_Occam_CharacterBattleStats.ReceiveDamage` _ac_occam_characterbattlestats_3 (`|GetArrayItem` _result) (`/Game/Occam/2_Programming/0_Components/AC_Occam_CharacterBattleStats.CurrentLevel` _ac_occam_characterbattlestats_2) (`/Game/Occam/2_Programming/0_Components/AC_Occam_CharacterBattleStats.CharacterStats` _ac_occam_characterbattlestats_2) (`/Game/Occam/2_Programming/0_Components/AC_Occam_CharacterBattleStats.CharacterStats` _ac_occam_characterbattlestats_3) (`/Game/Occam/2_Programming/0_Components/AC_Occam_CharacterBattleStats.Weaknesses` _ac_occam_characterbattlestats_3))))))

(fn `Activate_Defend`
  (bind _battlemanager (`self.GetBattleManager`))
  (`KismetSystemLibrary.PrintString` "Activate Defend" true true (struct :`G` 0.66 :`B` 1.0 :`A` 1.0) 40.0)
  (`/Game/Occam/2_Programming/0_Components/AC_Occam_BattleManager.ShowBattleTooltip` (`self.GetBattleManager`) (`|FormatText` "{0} Defends" (`KismetTextLibrary.Conv_StringToText` (`.CharacterDisplayName` (`self.GetCurrentCharacterName`)))))
  (set `/Game/Occam/2_Programming/0_Components/AC_Occam_CharacterBattleStats.Defending` true (`/Game/Occam/2_Programming/5_GameBaseActors/Battle/BP_Occam_Character_Battle_Base.AC_Occam_CharacterBattleStats` (`self.GetCurrentCharacter`)))
  (`/Game/Occam/2_Programming/0_Components/AC_Occam_BattleManager.EndCharacterTurn` _battlemanager)
  (`/Game/Occam/2_Programming/0_Components/AC_Occam_BattleManager.ResumeBattle` _battlemanager))

(fn `Activate_Run`
  (bind _battlemanager (`self.GetBattleManager`))
  (bind _canrun_ (`/Game/Occam/2_Programming/FL_Occam_Battle.RunCal_Combat`))
  (if _canrun_
    (`/Game/Occam/2_Programming/0_Components/AC_Occam_BattleManager.GoBackToWorldMap` (`self.GetBattleManager`))
    (else
      (`/Game/Occam/2_Programming/0_Components/AC_Occam_BattleManager.EndCharacterTurn` _battlemanager)
      (`/Game/Occam/2_Programming/0_Components/AC_Occam_BattleManager.ShowBattleTooltip` _battlemanager "You failed to Run!!")
      (`/Game/Occam/2_Programming/0_Components/AC_Occam_BattleManager.ResumeBattle` _battlemanager))))

(fn `GetActionCost`
  (params (`Action Name` :type Name))
  (returns (`Cost MP` :type Integer) (`Cost SP` :type Integer) (`Cost HP` :type Integer))
  (bind _returnvalue (`|GetDataTableRow` "/Game/Occam/2_Programming/1_Datatables/DT_Occam_Actions.DT_Occam_Actions" `Action Name`)
    (:`then`
      (bind (_actiontype _issecondaryaction _hardcodedname _displayname _damagetype _description _actionpower _maxlevel _basecostmp _basecostsp _basecosthp) (break `/Game/Occam/2_Programming/2_Structures/Strut_Occam_Action` _returnvalue))
      (return _basecostmp _basecostsp _basecosthp))))

(fn `Select_Attack`
  (`KismetSystemLibrary.PrintString` "Select Attack")
  (`/Game/Occam/2_Programming/0_Components/AC_Occam_BattleManager.ShowBattleTooltip` (`self.GetBattleManager`) "Select Target")
  (`/Game/Occam/2_Programming/0_Components/AC_Occam_TargetingManager.EnableTargeting` (`self.GetTargetingManager`) false "NewEnumerator1")
  (for _array_element (`/Game/Occam/2_Programming/0_Components/AC_Occam_BattleManager.Enemies` (`self.GetBattleManager`))
    (`/Game/Occam/2_Programming/0_Components/AC_Occam_CharacterBattleStats.CollapseEnemyWeaknessIcons` (`/Game/Occam/2_Programming/5_GameBaseActors/Battle/BP_Occam_Character_Battle_Base.AC_Occam_CharacterBattleStats` _array_element) false)))

(fn `Select_Defend`
  (`/Game/Occam/2_Programming/0_Components/AC_Occam_BattleManager.DisableTargetingAndInput` (`self.GetBattleManager`))
  (`self.Activate_Defend`))

(fn `Select_Magic`
  (`KismetSystemLibrary.PrintString` "Select Magic")
  (`/Game/Occam/2_Programming/0_Components/AC_Occam_BattleManager.ShowBattleTooltip` (`self.GetBattleManager`) "Select A Spell")
  (`/Game/Occam/2_Programming/0_Components/AC_Occam_TargetingManager.EnableTargeting` (`self.GetTargetingManager`) false "NewEnumerator1")
  (for _array_element (`/Game/Occam/2_Programming/0_Components/AC_Occam_BattleManager.Enemies` (`self.GetBattleManager`))
    (`/Game/Occam/2_Programming/0_Components/AC_Occam_CharacterBattleStats.CollapseEnemyWeaknessIcons` (`/Game/Occam/2_Programming/5_GameBaseActors/Battle/BP_Occam_Character_Battle_Base.AC_Occam_CharacterBattleStats` _array_element) false)))

(fn `Select_Run`
  (`KismetSystemLibrary.PrintString` "Select Run")
  (`/Game/Occam/2_Programming/0_Components/AC_Occam_BattleManager.DisableTargetingAndInput` (`self.GetBattleManager`))
  (`self.Activate_Run`))

(fn `Select_Skills`
  (`KismetSystemLibrary.PrintString` "Select Skills")
  (`/Game/Occam/2_Programming/0_Components/AC_Occam_BattleManager.ShowBattleTooltip` (`self.GetBattleManager`) "Select A Skill")
  (`/Game/Occam/2_Programming/0_Components/AC_Occam_TargetingManager.EnableTargeting` (`self.GetTargetingManager`) false "NewEnumerator1")
  (for _array_element (`/Game/Occam/2_Programming/0_Components/AC_Occam_BattleManager.Enemies` (`self.GetBattleManager`))
    (`/Game/Occam/2_Programming/0_Components/AC_Occam_CharacterBattleStats.CollapseEnemyWeaknessIcons` (`/Game/Occam/2_Programming/5_GameBaseActors/Battle/BP_Occam_Character_Battle_Base.AC_Occam_CharacterBattleStats` _array_element) false)))