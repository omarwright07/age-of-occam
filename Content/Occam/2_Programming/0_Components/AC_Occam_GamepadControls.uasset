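; Gamepad controls component for Occam that drives D-pad navigation and highlighting in UI menus.
; Activate functions cache widget references, and those for main menu, settings and controller test also set window focus and highlight an entry.
; D-pad up/down route by active interface and focused window to scroll helpers, unless a yes/no window is active.
; D-pad left/right, face, shoulder and trigger handlers, plus world activation, are empty stubs.
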(fn `Activate Gamepad Controls Main Menu`
  (bind _foundwidgets (`WidgetBlueprintLibrary.GetAllWidgetsOfClass` "/Game/Occam/6_UI/0_WBP/2_Main/WBP_Occam_MainMenu.WBP_Occam_MainMenu_C"))
  (bind _output_get (set `self.WindowRef_MainMenu` (`|GetArrayItem` _foundwidgets)))
  (set `self.GamepadWindowFocus` "NewEnumerator0")
  (bind _output (`|GetArrayItem` (`/Game/Occam/6_UI/0_WBP/2_Main/WBP_Occam_MainMenu.Gamepad_BTNS_MainMenu` _output_get) (`self.CurrentlySelectedMenuButton`)))
  (`/Engine/EditorBlueprintResources/StandardMacros.IsValid` _output
    (:`Is Valid`
      (`/Game/Occam/2_Programming/FL_Occam_Gamepad.HighlightMenuText` (`self.GamepadControlsEnabled?`) _output)
      (`Widget.SetFocus` _output))))

(fn `Activate Gamepad Controls_Settings`
  (bind _foundwidgets (`WidgetBlueprintLibrary.GetAllWidgetsOfClass` "/Game/Occam/6_UI/0_WBP/5_Settings/WBP_Occam_SettingsMenu.WBP_Occam_SettingsMenu_C" false))
  (bind _output_get (set `self.WindowRef _Settings` (`|GetArrayItem` _foundwidgets)))
  (bind _output (`|GetArrayItem` (`/Game/Occam/6_UI/0_WBP/5_Settings/WBP_Occam_SettingsMenu.Gamepad_BTNS_Settings` _output_get)))
  (`self.HighlightMenuButton` (`self.GamepadControlsEnabled?`) _output)
  (set `self.GamepadWindowFocus` "NewEnumerator25")
  (`Widget.SetFocus` _output))

(fn `ActivateGamepadControls_Battle`
  (bind _foundwidgets (`WidgetBlueprintLibrary.GetAllWidgetsOfClass` "/Game/Occam/6_UI/0_WBP/4_Battle/WBP_Occam_BattleInterface.WBP_Occam_BattleInterface_C"))
  (set `self.WindowRef_BattleInterface` (`|GetArrayItem` _foundwidgets)))

(fn `ActivateGamepadControls_ControllerTest`
  (bind _foundwidgets (`WidgetBlueprintLibrary.GetAllWidgetsOfClass` "/Game/Occam/6_UI/0_WBP/Sims/WBP_Occam_Sim_ControllerTest.WBP_Occam_Sim_ControllerTest_C"))
  (bind _output (`|GetArrayItem` _foundwidgets))
  (set `self.WindowRef_ControllerTest` _output)
  (`/Game/Occam/2_Programming/FL_Occam_Gamepad.HighlightMenu_General` true (`|GetArrayItem` (`PanelWidget.GetAllChildren` (`/Game/Occam/6_UI/0_WBP/Sims/WBP_Occam_Sim_ControllerTest.ScrollBox_0` _output))))
  (set `self.GamepadWindowFocus` "NewEnumerator24"))

(fn `ActivateGamepadControls_World`)

(fn `D-PadDownPressed`
  (`KismetSystemLibrary.PrintString` "D-Pad Down" true true (struct :`G` 1.0 :`B` 0.408744 :`A` 1.0))
  (if (not (`self.YesNoWindowActive?`))
    (`self.SwitchOnActiveInterface`
      (:`MainMenu`
        (switch `/Game/Occam/2_Programming/3_Enumerations/GamepadControls/Enum_Gamepad_WindowFocus` (`self.GamepadWindowFocus`)
          (:`NewEnumerator0`
            (`/Game/Occam/2_Programming/FL_Occam_Gamepad.Menu Scroll Down HTX` (`self.CurrentlySelectedMenuButton`) 1 (`/Game/Occam/6_UI/0_WBP/2_Main/WBP_Occam_MainMenu.Gamepad_BTNS_MainMenu` (`self.WindowRef_MainMenu`))))
          (:`NewEnumerator19`
            (`/Game/Occam/2_Programming/FL_Occam_Gamepad.Menu Scroll Up HTX` (`self.CurrentlySelectedMenuButton`) 0 (`/Game/Occam/6_UI/0_WBP/4_Battle/WBP_Occam_GameOverMenu.Gamepad_GameOver_BTNs` (`self.WindowRef_GameOver`))))
          (:`NewEnumerator25`
            (`/Game/Occam/2_Programming/FL_Occam_Gamepad.Menu Scroll Down HBTN` (`self.CurrentlySelectedMenuButton`) 0 (`/Game/Occam/6_UI/0_WBP/5_Settings/WBP_Occam_SettingsMenu.Gamepad_BTNS_Settings` (`self.WindowRef _Settings`)))))))))

(fn `D-PadLeftPressed`)

(fn `D-PadRightPressed`)

(fn `D-PadUpPressed`
  (`KismetSystemLibrary.PrintString` "D-Pad Up" true true (struct :`G` 1.0 :`B` 0.408744 :`A` 1.0))
  (if (not (`self.YesNoWindowActive?`))
    (`self.SwitchOnActiveInterface`
      (:`MainMenu`
        (switch `/Game/Occam/2_Programming/3_Enumerations/GamepadControls/Enum_Gamepad_WindowFocus` (`self.GamepadWindowFocus`)
          (:`NewEnumerator0`
            (`/Game/Occam/2_Programming/FL_Occam_Gamepad.Menu Scroll Up HTX` (`self.CurrentlySelectedMenuButton`) 1 (`/Game/Occam/6_UI/0_WBP/2_Main/WBP_Occam_MainMenu.Gamepad_BTNS_MainMenu` (`self.WindowRef_MainMenu`))))
          (:`NewEnumerator14`
            (if (`KismetMathLibrary.Conv_IntToBool` (`self.CurrentlySelectedMenuButton`))
              (bind _aswbp_occam_save_slot (cast `/Game/Occam/6_UI/0_WBP/3_Save/WBP_Occam_SaveSlot` (`PanelWidget.GetChildAt` (`/Game/Occam/6_UI/0_WBP/3_Save/WBP_Occam_SaveMenu.VB_SaveSlots` (`/Game/Occam/6_UI/0_WBP/2_Main/WBP_Occam_MainMenu.WBP_Occam_SaveMenu` (`self.WindowRef_MainMenu`))) (`self.CurrentlySelectedMenuButton`))))
              ;[1 1 1] Add conditions for selection based on assigned save name
              (`self.HighlightSaveSlot` false (`/Game/Occam/6_UI/0_WBP/3_Save/WBP_Occam_SaveSlot.BTN_EmptySave` _aswbp_occam_save_slot))
              (`/Engine/EditorBlueprintResources/StandardMacros.DecrementInt` (`self.CurrentlySelectedMenuButton`)
                (:`  `
                  (bind _aswbp_occam_save_slot_2 (cast `/Game/Occam/6_UI/0_WBP/3_Save/WBP_Occam_SaveSlot` (`PanelWidget.GetChildAt` (`/Game/Occam/6_UI/0_WBP/3_Save/WBP_Occam_SaveMenu.VB_SaveSlots` (`/Game/Occam/6_UI/0_WBP/2_Main/WBP_Occam_MainMenu.WBP_Occam_SaveMenu` (`self.WindowRef_MainMenu`))) (`self.CurrentlySelectedMenuButton`))))
                  (`self.HighlightSaveSlot` true (`/Game/Occam/6_UI/0_WBP/3_Save/WBP_Occam_SaveSlot.BTN_EmptySave` _aswbp_occam_save_slot_2))))))
          (:`NewEnumerator19`
            (`/Game/Occam/2_Programming/FL_Occam_Gamepad.Menu Scroll Up HTX` (`self.CurrentlySelectedMenuButton`) 0 (`/Game/Occam/6_UI/0_WBP/4_Battle/WBP_Occam_GameOverMenu.Gamepad_GameOver_BTNs` (`self.WindowRef_GameOver`))))))
      (:`Invalid`
        (switch `/Game/Occam/2_Programming/3_Enumerations/GamepadControls/Enum_Gamepad_WindowFocus` (`self.GamepadWindowFocus`)
          (:`NewEnumerator24`
            (`KismetSystemLibrary.PrintString` "--Test--")
            (`/Game/Occam/2_Programming/FL_Occam_Gamepad.Menu Scroll Up General` (`self.CurrentlySelectedMenuButton`) 0 (`PanelWidget.GetAllChildren` (`/Game/Occam/6_UI/0_WBP/Sims/WBP_Occam_Sim_ControllerTest.ScrollBox_0` (`self.WindowRef_ControllerTest`))))))))))

(fn `FaceButtonBottomPressed`)

(fn `FaceButtonLeftPressed`)

(fn `FaceButtonRightPressed`)

(fn `FaceButtonTopPressed`)

(fn `HighlightActionSlotInActionsScreen`
  (params (`Highlight?` :type Boolean) (Button :type "Button Object Reference"))
  (`/Engine/EditorBlueprintResources/StandardMacros.IsValid` Button
    (:`Is Valid`
      (`Button.SetBackgroundColor` Button (`KismetMathLibrary.SelectColor` (struct :`R` 1.0 :`G` 0.624415 :`A` 1.0) (struct :`R` 1.0 :`G` 1.0 :`B` 1.0 :`A` 1.0) `Highlight?`)))))

(fn `HighlightMenuButton`
  (params (`Highlight?` :type Boolean) (Button :type "Button Object Reference"))
  (`/Engine/EditorBlueprintResources/StandardMacros.IsValid` Button
    (:`Is Valid`
      (`Button.SetBackgroundColor` Button (`KismetMathLibrary.SelectColor` (struct :`R` 1.0 :`G` 0.624415 :`A` 1.0) (struct :`R` 1.0 :`G` 1.0 :`B` 1.0 :`A` 1.0) `Highlight?`)))))

(fn `HighlightSaveSlot`
  (params (`Highlight?` :type Boolean) (Button :type "Button Object Reference"))
  (`/Engine/EditorBlueprintResources/StandardMacros.IsValid` Button
    (:`Is Valid`
      (`Button.SetBackgroundColor` Button (`KismetMathLibrary.SelectColor` (struct :`R` 1.0 :`G` 0.624415 :`A` 1.0) (struct :`R` 1.0 :`G` 1.0 :`B` 1.0 :`A` 1.0) `Highlight?`)))))

(fn `ShoulderLeftPressed`)

(fn `ShoulderRightPressed`)

(fn `TriggerLeftPressed`)

(fn `TriggerRightPressed`)