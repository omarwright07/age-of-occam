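; Quest manager component that holds the player's quest log and drives the quest log and quest trigger widgets.
; On BeginPlay it copies every DT_Occam_Quest row into the log with the first objective started, then builds quest, objective and reward entry widgets from it.
; One quest is active at a time, and a matching completion trigger advances its current objective.
; State changes are written back into the struct array by index.
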(event `self.ReceiveBeginPlay`
  (`self.BuildCurrentPlayerQuestLog`))

(fn `AddQuestToQuestLog`
  (params (RowName :type Name))
  (locals (Local_QuestStrut :type "/Game/Occam/2_Programming/2_Structures/Quest/Strut_Occam_Quest_System Structure"))
  (bind _returnvalue (`|GetDataTableRow` "/Game/Occam/2_Programming/1_Datatables/DT_Occam_Quest.DT_Occam_Quest" RowName)
    (:`then`
      (bind _output_get (set `local.Local_QuestStrut` _returnvalue))
      (`|VariableSetRef` (`.ObjectiveState_34_6897ABE2427AE1EABFD2B1903DA23EA9` (break `/Game/Occam/2_Programming/2_Structures/Quest/Strut_Occam_Objective` (`|GetArrayItem` (`.Objectives_86_350864A3445CFF95ED3D90A78BB47074` (break `/Game/Occam/2_Programming/2_Structures/Quest/Strut_Occam_Quest_System` _output_get))))) "NewEnumerator0")
      (`KismetArrayLibrary.Array_AddUnique` (`self.CurrentPlayerQuestsLog`) (`local.Local_QuestStrut`)))))

(fn `BuildCurrentPlayerQuestLog`
  (bind _outrownames (`DataTableFunctionLibrary.GetDataTableRowNames` "/Game/Occam/2_Programming/1_Datatables/DT_Occam_Quest.DT_Occam_Quest"))
  (for _array_element _outrownames
    (`self.AddQuestToQuestLog` _array_element)))

(fn `CreateQuestEntries`
  (`KismetSystemLibrary.PrintString` "Quest Man - Create Quest Entries")
  (for _array_element (`self.CurrentPlayerQuestsLog`)
    (bind (_hardcodedname _displayname _description _location _prerequisites _objectives _completeconditions _completequestrewards _queststate) (break `/Game/Occam/2_Programming/2_Structures/Quest/Strut_Occam_Quest_System` _array_element))
    (bind _returnvalue (`|CreateWidget` "/Game/Occam/6_UI/0_WBP/Sims/WBP_Sim_Quest_Entry.WBP_Sim_Quest_Entry_C" null (`KismetStringLibrary.Conv_StringToName` _displayname) _queststate (`self.WindowReference_QuestLog`) (`KismetStringLibrary.Conv_StringToName` _hardcodedname)))
    ;[1 1 1] Needs to be updated to sort between inactive and completeed quests
    (`PanelWidget.AddChild` (`/Game/Occam/6_UI/0_WBP/Sims/WBP_Sim_Quest_Log.SB_InactiveQuests` (`self.WindowReference_QuestLog`)) _returnvalue)))

(fn `FilterQuestLogForSelectedQuest`
  (params (QuestLog :type Name))
  (returns (`Found?` :type Boolean) (SelectedQuestStrut :type "/Game/Occam/2_Programming/2_Structures/Quest/Strut_Occam_Quest_System Structure") (FoundIndex :type Integer))
  (locals (Local_SelectedQuestStrut :type "/Game/Occam/2_Programming/2_Structures/Quest/Strut_Occam_Quest_System Structure") (`Local_Found?` :type Boolean :default false) (Local_FoundIndex :type Integer))
  (for (_array_element _array_index) (`self.CurrentPlayerQuestsLog`)
    (if (`KismetStringLibrary.EqualEqual_StrStr` (`.HardcodedName_18_4AF2431E4AEBF3342AA55497D2301794` (break `/Game/Occam/2_Programming/2_Structures/Quest/Strut_Occam_Quest_System` _array_element)) (`KismetStringLibrary.Conv_NameToString` QuestLog))
      (set `local.Local_SelectedQuestStrut` _array_element)
      (set `local.Local_Found?` true)
      (set `local.Local_FoundIndex` _array_index)
      (break)))
  (return (`local.Local_Found?`) (`local.Local_SelectedQuestStrut`) (`local.Local_FoundIndex`)))

(fn `FindSelectedQuestFromLog`
  (params (QuestName :type Name))
  (returns (Output :type "/Game/Occam/2_Programming/2_Structures/Quest/Strut_Occam_Quest_System Structure (by ref)"))
  (locals (Local_FoundQuestIndex :type Integer :default -1))
  (bind _local_foundquestindex (`local.Local_FoundQuestIndex`))
  (for (_array_element _array_index) (`self.CurrentPlayerQuestsLog`)
    (if (`KismetStringLibrary.EqualEqual_StrStr` (`.HardcodedName_18_4AF2431E4AEBF3342AA55497D2301794` (break `/Game/Occam/2_Programming/2_Structures/Quest/Strut_Occam_Quest_System` _array_element)) (`KismetStringLibrary.Conv_NameToString` QuestName))
      (set `local.Local_FoundQuestIndex` _array_index)
      (break)))
  (if (== _local_foundquestindex -1)
    (return)
    (else
      (return (`|GetArrayItem` (`self.CurrentPlayerQuestsLog`) _local_foundquestindex)))))

(fn `SetCurrentCondition`
  (params (QuestCondition :type "/Game/Occam/2_Programming/3_Enumerations/Quest/Enum_Occam_Quest_Conditions Enum" :default "NewEnumerator0") (CalendarDayNumber :type Integer) (SetTimeOfDay :type "/Game/Occam/2_Programming/3_Enumerations/Quest/Enum_Occam_TimePeriods Enum" :default "NewEnumerator11") (SocialRank :type "/Game/Occam/2_Programming/3_Enumerations/Enum_Occam_CharactesSocialRank Enum" :default "NewEnumerator0") (MoralityRank :type "/Game/Occam/2_Programming/3_Enumerations/Enum_Occam_CharactersMoralityRank Enum" :default "NewEnumerator17"))
  (locals (Local_CalendarDayNumber :type Integer) (Local_QuestCondition :type "/Game/Occam/2_Programming/3_Enumerations/Quest/Enum_Occam_Quest_Conditions Enum" :default "NewEnumerator0"))
  (bind _output_get (set `local.Local_QuestCondition` QuestCondition))
  (switch `/Game/Occam/2_Programming/3_Enumerations/Quest/Enum_Occam_Quest_Conditions` _output_get
    (:`NewEnumerator0`
      (bind _output_get_2 (set `local.Local_CalendarDayNumber` CalendarDayNumber))
      (`TextBlock.SetText` (`/Game/Occam/6_UI/0_WBP/Sims/WBP_Sim_Quest_Triggers.TX_CalendarDay` (`self.WindowReference_QuestTriggers`)) (`KismetTextLibrary.Conv_IntToText` _output_get_2)))
    (:`NewEnumerator1`
      (bind _output_get_3 (set `self.CurrentTimePeriod` SetTimeOfDay))
      (`TextBlock.SetText` (`/Game/Occam/6_UI/0_WBP/Sims/WBP_Sim_Quest_Triggers.TX_TimePeriod` (`self.WindowReference_QuestTriggers`)) (`KismetTextLibrary.Conv_StringToText` (`|GetEnumeratorNameAsString` _output_get_3))))
    (:`NewEnumerator3`
      (`TextBlock.SetText` (`/Game/Occam/6_UI/0_WBP/Sims/WBP_Sim_Quest_Triggers.TX_SocialRank` (`self.WindowReference_QuestTriggers`)) (`KismetTextLibrary.Conv_StringToText` (`|GetEnumeratorNameAsString` SocialRank))))
    (:`NewEnumerator5`
      (`TextBlock.SetText` (`/Game/Occam/6_UI/0_WBP/Sims/WBP_Sim_Quest_Triggers.TX_Mortality` (`self.WindowReference_QuestTriggers`)) (`KismetTextLibrary.Conv_StringToText` (`|GetEnumeratorNameAsString` MoralityRank))))))

(fn `SetCurrentObjective`
  (params (QuestLog :type Name))
  (bind (_found_ _selectedqueststrut) (`self.FilterQuestLogForSelectedQuest` QuestLog))
  (if _found_
    (for (_array_element _array_index) (`.Objectives_86_350864A3445CFF95ED3D90A78BB47074` (break `/Game/Occam/2_Programming/2_Structures/Quest/Strut_Occam_Quest_System` _selectedqueststrut))
      (if (`|EnumEquality` (`.ObjectiveState_34_6897ABE2427AE1EABFD2B1903DA23EA9` (break `/Game/Occam/2_Programming/2_Structures/Quest/Strut_Occam_Objective` _array_element)) "NewEnumerator0")
        (set `self.ActiveCurrentObjective` _array_index)
        (break)))))

(fn `SetObjectiveState`
  (params (HardcodedName :type Name) (Value :type "/Game/Occam/2_Programming/3_Enumerations/Quest/Enum_Occam_Quest_States Enum" :default "NewEnumerator0"))
  (locals (Local_QuestStrut :type "/Game/Occam/2_Programming/2_Structures/Quest/Strut_Occam_Quest_System Structure") (NewLocalVar_0 :type Name) (NewLocalVar_1 :type "/Game/Occam/2_Programming/3_Enumerations/Quest/Enum_Occam_Quest_States Enum" :default "NewEnumerator0"))
  (bind _output_get (set `local.NewLocalVar_0` HardcodedName))
  (set `local.NewLocalVar_1` Value)
  (bind (_found_ _selectedqueststrut _foundindex) (`self.FilterQuestLogForSelectedQuest` _output_get))
  (if _found_
    (bind _output_get_2 (set `local.Local_QuestStrut` _selectedqueststrut))
    (`|VariableSetRef` (`.ObjectiveState_34_6897ABE2427AE1EABFD2B1903DA23EA9` (break `/Game/Occam/2_Programming/2_Structures/Quest/Strut_Occam_Objective` (`|GetArrayItem` (`.Objectives_86_350864A3445CFF95ED3D90A78BB47074` (break `/Game/Occam/2_Programming/2_Structures/Quest/Strut_Occam_Quest_System` _output_get_2)) (`self.ActiveCurrentObjective`)))) (`local.NewLocalVar_1`))
    (`KismetArrayLibrary.Array_Set` (`self.CurrentPlayerQuestsLog`) _foundindex (`local.Local_QuestStrut`) true)
    (if (`|EnumEquality` (`local.NewLocalVar_1`) "NewEnumerator5")
      (`self.SetQuestWidgetEntry` (`local.NewLocalVar_0`) (`local.NewLocalVar_1`))
      (`self.UpdateSelectedQuestDisplayPanel` (`local.NewLocalVar_0`)))))

(fn `SetQuestAsActive`
  (bind _selectedquestlog (`self.SelectedQuestLog`))
  (bind _tx_title_activequest (`/Game/Occam/6_UI/0_WBP/Sims/WBP_Sim_Quest_Log.TX_Title_ActiveQuest` (`self.WindowReference_QuestLog`)))
  (bind _tx_activequest_objective (`/Game/Occam/6_UI/0_WBP/Sims/WBP_Sim_Quest_Log.TX_ActiveQuest_Objective` (`self.WindowReference_QuestLog`)))
  (bind (_found_ _selectedqueststrut) (`self.FilterQuestLogForSelectedQuest` (`self.SelectedQuestLog`)))
  (if (not (`|EnumEquality` (`.QuestState_101_169D9C9948440CC36E1FFDB76E2F79FE` (break `/Game/Occam/2_Programming/2_Structures/Quest/Strut_Occam_Quest_System` _selectedqueststrut)) "NewEnumerator2"))
    (for _array_element (`self.CurrentPlayerQuestsLog`)
      (bind (_hardcodedname _displayname _description _location _prerequisites _objectives _completeconditions _completequestrewards _queststate) (break `/Game/Occam/2_Programming/2_Structures/Quest/Strut_Occam_Quest_System` _array_element))
      ;[1 1 1] Checks To See If Harcoded Name = Selected Quest Log
      ; True - Sets it as Active
      ; False - Set it as Inactive
      (if (== (`KismetStringLibrary.Conv_StringToName` _hardcodedname) _selectedquestlog)
        (set `self.ActiveQuestLog` _selectedquestlog)
        (`|VariableSetRef` _queststate "NewEnumerator0")
        (`|ExecutionSequence`
          (:`then_0`
            ;[1 1 1] Set Active Title Display Text
            (`TextBlock.SetText` _tx_title_activequest (`KismetTextLibrary.Conv_StringToText` _displayname))
            (`Widget.SetVisibility` _tx_title_activequest "Visible"))
          (:`then_1`
            ;[1 1 1] Set Current Objective in Quest Man
            ; Set Active Objective Display Text
            (`self.SetCurrentObjective` (`self.ActiveQuestLog`))
            (`TextBlock.SetText` _tx_activequest_objective (`KismetTextLibrary.Conv_StringToText` (`.Description_22_7186D22448263D18F794C4B776544240` (break `/Game/Occam/2_Programming/2_Structures/Quest/Strut_Occam_Objective` (`|GetArrayItem` _objectives (`self.ActiveCurrentObjective`))))))
            (`Widget.SetVisibility` _tx_activequest_objective "Visible"))
          (:`then_2`
            ;[1 1 1] Finds the selected quest logs and set it as active
            (for _array_element_2 (`PanelWidget.GetAllChildren` (`/Game/Occam/6_UI/0_WBP/Sims/WBP_Sim_Quest_Log.SB_InactiveQuests` (`self.WindowReference_QuestLog`)))
              (bind _aswbp_sim_quest_entry (cast `/Game/Occam/6_UI/0_WBP/Sims/WBP_Sim_Quest_Entry` _array_element_2))
              (if (== (`/Game/Occam/6_UI/0_WBP/Sims/WBP_Sim_Quest_Entry.QuestHardcodedName` _aswbp_sim_quest_entry) (`self.SelectedQuestLog`))
                (set `/Game/Occam/6_UI/0_WBP/Sims/WBP_Sim_Quest_Entry.QuestState` "NewEnumerator0" _aswbp_sim_quest_entry)
                (break)))))
        (elif (not (or (`|EnumEquality` _queststate "NewEnumerator2") (`|EnumEquality` _queststate "NewEnumerator5")))
          (`|VariableSetRef` _queststate "NewEnumerator1"))))
    ;[1 1 1] Goes through all the Quest Logs and Set everyone that's not the selected quest log as inactive
    (for _array_element_3 (`PanelWidget.GetAllChildren` (`/Game/Occam/6_UI/0_WBP/Sims/WBP_Sim_Quest_Log.SB_InactiveQuests` (`self.WindowReference_QuestLog`)))
      (bind _aswbp_sim_quest_entry_2 (cast `/Game/Occam/6_UI/0_WBP/Sims/WBP_Sim_Quest_Entry` _array_element_3))
      (if (!= (`/Game/Occam/6_UI/0_WBP/Sims/WBP_Sim_Quest_Entry.QuestHardcodedName` _aswbp_sim_quest_entry_2) (`self.SelectedQuestLog`))
        (set `/Game/Occam/6_UI/0_WBP/Sims/WBP_Sim_Quest_Entry.QuestState` "NewEnumerator1" _aswbp_sim_quest_entry_2)))
    (`self.UpdateActiveQuestTriggersWidget`)))

(fn `SetQuestLogState`
  (params (HardcodedQuestName :type Name) (QuestState :type "/Game/Occam/2_Programming/3_Enumerations/Quest/Enum_Occam_Quest_States Enum" :default "NewEnumerator0"))
  (locals (Local_QuestStrut :type "/Game/Occam/2_Programming/2_Structures/Quest/Strut_Occam_Quest_System Structure"))
  (bind (_found_ _selectedqueststrut _foundindex) (`self.FilterQuestLogForSelectedQuest` HardcodedQuestName))
  (if _found_
    (bind _output_get (set `local.Local_QuestStrut` _selectedqueststrut))
    (`|VariableSetRef` (`.QuestState_101_169D9C9948440CC36E1FFDB76E2F79FE` (break `/Game/Occam/2_Programming/2_Structures/Quest/Strut_Occam_Quest_System` _output_get)) QuestState)
    (`KismetArrayLibrary.Array_Set` (`self.CurrentPlayerQuestsLog`) _foundindex (`local.Local_QuestStrut`) true)))

(fn `SetQuestRewardsPopUp`
  (params (HardcodedQuestName :type Name))
  (`KismetSystemLibrary.PrintString` "Quest Man - Set Quest Display")
  (bind (_found_ _selectedqueststrut) (`self.FilterQuestLogForSelectedQuest` HardcodedQuestName))
  (if _found_
    (`|ExecutionSequence`
      (:`then_0`
        (bind (_currency _experience _items) (break `/Game/Occam/2_Programming/2_Structures/Quest/Strut_Occam_Quest_Rewards` (`.CompleteQuestRewards_85_80DAFD654C1EDA3B3E3092A08DB0C407` (break `/Game/Occam/2_Programming/2_Structures/Quest/Strut_Occam_Quest_System` _selectedqueststrut))))
        ;[1 1 1] Builds Reward Display -- Needs Window Reference Changed
        (bind _returnvalue (`|CreateWidget` "/Game/Occam/6_UI/0_WBP/0_Templates/WBP_Occam_Loot_InfoBar.WBP_Occam_Loot_InfoBar_C" null "Bytes" _currency))
        (`PanelWidget.AddChild` (`/Game/Occam/6_UI/0_WBP/Sims/WBP_Sim_Quest_Log.VB_SelectedQuest_Reward` (`self.WindowReference_QuestLog`)) _returnvalue))
      (:`then_1`
        (bind _values (`BlueprintMapLibrary.Map_Values` _experience))
        (bind _keys (`BlueprintMapLibrary.Map_Keys` _experience))
        (for (_array_element _array_index) _keys
          (bind _returnvalue_2 (`|CreateWidget` "/Game/Occam/6_UI/0_WBP/0_Templates/WBP_Occam_Loot_InfoBar.WBP_Occam_Loot_InfoBar_C" null (`KismetTextLibrary.Conv_ByteToText` _array_element) (`|GetArrayItem` _values _array_index)))
          (`PanelWidget.AddChild` (`/Game/Occam/6_UI/0_WBP/Sims/WBP_Sim_Quest_Log.VB_SelectedQuest_Reward` (`self.WindowReference_QuestLog`)) _returnvalue_2)))
      (:`then_2`
        (bind _values_2 (`BlueprintMapLibrary.Map_Values` _items))
        (bind _keys_2 (`BlueprintMapLibrary.Map_Keys` _items))
        (for (_array_element_2 _array_index_2) _keys_2
          (bind _returnvalue_3 (`|CreateWidget` "/Game/Occam/6_UI/0_WBP/0_Templates/WBP_Occam_Loot_InfoBar.WBP_Occam_Loot_InfoBar_C" null (`KismetTextLibrary.Conv_NameToText` _array_element_2) (`|GetArrayItem` _values_2 _array_index_2)))
          (`PanelWidget.AddChild` (`/Game/Occam/6_UI/0_WBP/Sims/WBP_Sim_Quest_Log.VB_SelectedQuest_Reward` (`self.WindowReference_QuestLog`)) _returnvalue_3))))))

(fn `SetQuestWidgetEntry`
  (params (HardcodedQuestName :type Name) (QuestState :type "/Game/Occam/2_Programming/3_Enumerations/Quest/Enum_Occam_Quest_States Enum" :default "NewEnumerator0"))
  (locals (Local_QuestStrut :type "/Game/Occam/2_Programming/2_Structures/Quest/Strut_Occam_Quest_System Structure"))
  (`KismetSystemLibrary.PrintString` "Quest Man - Set Quest As Complete")
  (bind (_found_ _selectedqueststrut _foundindex) (`self.FilterQuestLogForSelectedQuest` HardcodedQuestName))
  (if _found_
    (bind _output_get (set `local.Local_QuestStrut` _selectedqueststrut))
    (`|VariableSetRef` (`.QuestState_101_169D9C9948440CC36E1FFDB76E2F79FE` (break `/Game/Occam/2_Programming/2_Structures/Quest/Strut_Occam_Quest_System` _output_get)) QuestState)
    (`KismetArrayLibrary.Array_Set` (`self.CurrentPlayerQuestsLog`) _foundindex (`local.Local_QuestStrut`) true)
    (for _array_element (`PanelWidget.GetAllChildren` (`/Game/Occam/6_UI/0_WBP/Sims/WBP_Sim_Quest_Log.SB_InactiveQuests` (`self.WindowReference_QuestLog`)))
      (bind _aswbp_sim_quest_entry (cast `/Game/Occam/6_UI/0_WBP/Sims/WBP_Sim_Quest_Entry` _array_element))
      (bind _queststate (`/Game/Occam/6_UI/0_WBP/Sims/WBP_Sim_Quest_Entry.QuestState` _aswbp_sim_quest_entry))
      (if (and (== (`/Game/Occam/6_UI/0_WBP/Sims/WBP_Sim_Quest_Entry.QuestHardcodedName` _aswbp_sim_quest_entry) (`self.SelectedQuestLog`)) (or (`|EnumInequality` _queststate "NewEnumerator2") (`|EnumInequality` _queststate "NewEnumerator5")))
        (set `/Game/Occam/6_UI/0_WBP/Sims/WBP_Sim_Quest_Entry.QuestState` QuestState _aswbp_sim_quest_entry)
        (`PanelWidget.AddChild` (`/Game/Occam/6_UI/0_WBP/Sims/WBP_Sim_Quest_Log.SB_CompletedQuests` (`self.WindowReference_QuestLog`)) _array_element)
        (break)))))

(fn `SortFinishedQuests`
  (bind _outrownames (`DataTableFunctionLibrary.GetDataTableRowNames` "/Game/Occam/2_Programming/1_Datatables/DT_Occam_Quest.DT_Occam_Quest"))
  (for _array_element _outrownames
    (`self.AddQuestToQuestLog` _array_element)))

(fn `TriggerCompleteObjective`
  (params (ObjectiveTrigger :type "/Game/Occam/2_Programming/3_Enumerations/Quest/Enum_Occam_Objective_Triggers Enum" :default "NewEnumerator0") (QuestHardcodedName :type Name))
  (bind _activequestlog (`self.ActiveQuestLog`))
  (bind _activecurrentobjective (`self.ActiveCurrentObjective`))
  (bind _activequestlog_2 (`self.ActiveQuestLog`))
  (`KismetSystemLibrary.PrintString` (`KismetTextLibrary.Conv_TextToString` (`|FormatText` "Trigger \"{0}\" == For Quest \"{1}\" - Objective \"{2}\"" (`|GetEnumeratorNameAsString` ObjectiveTrigger) _activequestlog (`self.ActiveCurrentObjective`))))
  (if (not (== _activequestlog "None"))
    (bind _output (`self.FindSelectedQuestFromLog` (`self.ActiveQuestLog`)))
    (bind (_hardcodedname _displayname _description _location _prerequisites _objectives) (break `/Game/Occam/2_Programming/2_Structures/Quest/Strut_Occam_Quest_System` _output))
    (if (>= _activecurrentobjective (`KismetArrayLibrary.Array_Length` _objectives))
      _
      (elif (`|EnumEquality` (`.CompletionTrigger_40_86F50BE54A090CA8196433B345F38B3A` (break `/Game/Occam/2_Programming/2_Structures/Quest/Strut_Occam_Objective` (`|GetArrayItem` _objectives _activecurrentobjective))) ObjectiveTrigger)
        (`KismetSystemLibrary.PrintString` "Trigger Success")
        (`self.SetObjectiveState` _activequestlog_2 "NewEnumerator2")
        (bind _result (`/Engine/EditorBlueprintResources/StandardMacros.IncrementInt` (`self.ActiveCurrentObjective`))
          (:`  `
            (if (not (>= _result (`KismetArrayLibrary.Array_Length` _objectives)))
              (`self.SetObjectiveState` _activequestlog_2))
            (`self.UpdateActiveQuestTriggersWidget`)
            (if (== (`self.SelectedQuestLog`) (`self.ActiveQuestLog`))
              (`self.UpdateSelectedQuestDisplayPanel` "None"))))
        (else
          (`KismetSystemLibrary.PrintString` "Trigger Fail"))))))

(fn `UpdateActiveQuestTriggersWidget`
  (bind (_found_ _selectedqueststrut) (`self.FilterQuestLogForSelectedQuest` (`self.ActiveQuestLog`)))
  (if _found_
    (bind (_hardcodedname _displayname _description _location _prerequisites _objectives) (break `/Game/Occam/2_Programming/2_Structures/Quest/Strut_Occam_Quest_System` _selectedqueststrut))
    (`TextBlock.SetText` (`/Game/Occam/6_UI/0_WBP/Sims/WBP_Sim_Quest_Triggers.TX_QuestTitle` (`self.WindowReference_QuestTriggers`)) (`KismetTextLibrary.Conv_StringToText` _displayname))
    (`PanelWidget.ClearChildren` (`/Game/Occam/6_UI/0_WBP/Sims/WBP_Sim_Quest_Triggers.VB_Objectives` (`self.WindowReference_QuestTriggers`)))
    (for _array_element _objectives
      (bind (_description_2 _preconditions _failconditions _completiontrigger _objectivestate) (break `/Game/Occam/2_Programming/2_Structures/Quest/Strut_Occam_Objective` _array_element))
      (bind _returnvalue (`|CreateWidget` "/Game/Occam/6_UI/0_WBP/Sims/WBP_Sim_Objective_Entry.WBP_Sim_Objective_Entry_C" null (`KismetTextLibrary.Conv_StringToText` _description_2) _objectivestate _completiontrigger))
      (`PanelWidget.AddChild` (`/Game/Occam/6_UI/0_WBP/Sims/WBP_Sim_Quest_Triggers.VB_Objectives` (`self.WindowReference_QuestTriggers`)) _returnvalue))))

(fn `UpdateSelectedQuestDisplayPanel`
  (params (RowName :type Name))
  (bind _windowreference_questlog (`self.WindowReference_QuestLog`))
  (bind _output_get (set `self.SelectedQuestLog` RowName))
  (bind (_found_ _selectedqueststrut) (`self.FilterQuestLogForSelectedQuest` _output_get))
  (`|ExecutionSequence`
    (:`then_0`
      (`PanelWidget.ClearChildren` (`/Game/Occam/6_UI/0_WBP/Sims/WBP_Sim_Quest_Log.VB_SelectedQuest_Reward` _windowreference_questlog))
      (`PanelWidget.ClearChildren` (`/Game/Occam/6_UI/0_WBP/Sims/WBP_Sim_Quest_Log.VB_SelectedQuest_Objective` _windowreference_questlog))
      (`Widget.SetVisibility` (`/Game/Occam/6_UI/0_WBP/Sims/WBP_Sim_Quest_Log.ScrollBox_2` _windowreference_questlog) "Visible"))
    (:`then_1`
      (bind (_hardcodedname _displayname _description _location _prerequisites _objectives) (break `/Game/Occam/2_Programming/2_Structures/Quest/Strut_Occam_Quest_System` _selectedqueststrut))
      ;[1 1 1] Sets Selected Title and Description
      (`TextBlock.SetText` (`/Game/Occam/6_UI/0_WBP/Sims/WBP_Sim_Quest_Log.TX_SelectedQuest_Title` (`self.WindowReference_QuestLog`)) (`KismetTextLibrary.Conv_StringToText` _displayname))
      (`TextBlock.SetText` (`/Game/Occam/6_UI/0_WBP/Sims/WBP_Sim_Quest_Log.TX_SelectedQuest_Description` (`self.WindowReference_QuestLog`)) (`KismetTextLibrary.Conv_StringToText` _description)))
    (:`then_2`
      ;[1 1 1] Builds Objective List
      (for _array_element _objectives
        (bind (_description_2 _preconditions _failconditions _completiontrigger _objectivestate) (break `/Game/Occam/2_Programming/2_Structures/Quest/Strut_Occam_Objective` _array_element))
        (bind _returnvalue (`|CreateWidget` "/Game/Occam/6_UI/0_WBP/Sims/WBP_Sim_Objective_Entry.WBP_Sim_Objective_Entry_C" null (`KismetTextLibrary.Conv_StringToText` _description_2) _objectivestate _completiontrigger))
        (`PanelWidget.AddChild` (`/Game/Occam/6_UI/0_WBP/Sims/WBP_Sim_Quest_Log.VB_SelectedQuest_Objective` (`self.WindowReference_QuestLog`)) _returnvalue)))))