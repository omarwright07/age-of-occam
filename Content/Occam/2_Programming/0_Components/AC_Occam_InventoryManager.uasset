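; Inventory and vendor component that stores items and currency in BP_Occam_GI_General, fetched on BeginPlay with a retry.
; Handles stacked adding and removal, buy/sell checks on currency, free slots, key items and sell value.
; It also drives the inventory and store menus, found by widget class search, refreshing details and currency text.
; Slot widgets are created on demand and pooled: unused ones are collapsed, released inventory slots moved to the end.
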(event `self.ReceiveBeginPlay`
  (bind _asbp_occam_gi_general (cast `/Game/Occam/2_Programming/8_SaveContainers/BP_Occam_GI_General` (`GameplayStatics.GetGameInstance`) :!label _label)
    (:`then`
      (set `self.GameInstanceReference` _asbp_occam_gi_general))
    (:`CastFailed`
      (`KismetSystemLibrary.Delay` 0.1)
      (goto _label))))

(fn `AddCurrency`
  (params (CurrenyAmount :type Integer))
  (bind _gameinstancereference (`self.GameInstanceReference`))
  (set `/Game/Occam/2_Programming/8_SaveContainers/BP_Occam_GI_General.Currency` (+ CurrenyAmount (`/Game/Occam/2_Programming/8_SaveContainers/BP_Occam_GI_General.Currency` _gameinstancereference)) _gameinstancereference)
  (`self.RefreshCurrencyAmount`))

(fn `AddItemToInventory`
  (params (ItemHardcodedName :type Name) (ItemType :type "/Game/Occam/2_Programming/3_Enumerations/Items/Enum_Occam_ItemType Enum" :default "NewEnumerator0") (Amount :type Integer))
  (locals (Local_ItemHardcodedName :type Name) (Local_AmountToAdd :type Integer) (Local_ItemStrut :type "/Game/Occam/2_Programming/2_Structures/Items/Strut_Occam_Item_Inventory_Data Structure") (Local_Surplus :type Integer))
  (bind (_itemtype _itemsubtype _hardcodedname _displayname _keyitem_ _rarity _buyvalue _sellvalue _maxstackamount) (break `/Game/Occam/2_Programming/2_Structures/Items/Strut_Occam_Item_Inventory_Data` (`local.Local_ItemStrut`)))
  (set `local.Local_ItemHardcodedName` ItemHardcodedName)
  (set `local.Local_AmountToAdd` Amount)
  ;[1 1 1] Replace with custom function
  (bind (_hardcodedname_2 _iteminventorydata) (`/Game/Occam/2_Programming/FL_Occam_Custom.ItemTypeData_To_ItemInventoryData` (`local.Local_ItemHardcodedName`) ItemType))
  (set `local.Local_ItemStrut` _iteminventorydata)
  (bind (_success_ _itemindex) (`self.CheckIfThereIsNotFullyStackedItemInInventory` (`local.Local_ItemHardcodedName`))) ; Since multiple stacking is allowed, we just need to check\nif we add item to exisiting stack or we create new one.
  (if _success_
    (bind _output (`|GetArrayItem` (`/Game/Occam/2_Programming/8_SaveContainers/BP_Occam_GI_General.Inventory` (`self.GameInstanceReference`)) _itemindex))
    (bind (_stacksamount _itemsinventorydata) (break `/Game/Occam/2_Programming/2_Structures/Items/Strut_Occam_Items_DynamicData` _output))
    (bind (_itemtype_2 _itemsubtype_2 _hardcodedname_3 _displayname_2 _keyitem__2 _rarity_2 _buyvalue_2 _sellvalue_2 _maxstackamount_2) (break `/Game/Occam/2_Programming/2_Structures/Items/Strut_Occam_Item_Inventory_Data` _itemsinventorydata))
    (set `local.Local_Surplus` (- (`local.Local_AmountToAdd`) (- _maxstackamount_2 _stacksamount)))
    (setmembers `/Game/Occam/2_Programming/2_Structures/Items/Strut_Occam_Items_DynamicData` :`StructRef` _output :`StacksAmount` (`KismetMathLibrary.Clamp` (+ (`local.Local_AmountToAdd`) _stacksamount) 1 _maxstackamount_2))
    (elif (`self.CheckIfThereIsFreeSlotInInventory`)
      (set `local.Local_Surplus` (- (`local.Local_AmountToAdd`) _maxstackamount))
      (bind _returnvalue (`KismetArrayLibrary.Array_Add` (`/Game/Occam/2_Programming/8_SaveContainers/BP_Occam_GI_General.Inventory` (`self.GameInstanceReference`)) (make `/Game/Occam/2_Programming/2_Structures/Items/Strut_Occam_Items_DynamicData` (`KismetMathLibrary.Clamp` (`local.Local_AmountToAdd`) 1 _maxstackamount) (`local.Local_ItemStrut`))))
      (`self.RefreshInventorySlot` _returnvalue) ; Update slot data with newly added item.
    )))

(fn `BuyItem`
  (params (ItemInventoryData :type "/Game/Occam/2_Programming/2_Structures/Items/Strut_Occam_Item_Inventory_Data Structure"))
  (bind (_itemtype _itemsubtype _hardcodedname _displayname _keyitem_ _rarity _buyvalue) (break `/Game/Occam/2_Programming/2_Structures/Items/Strut_Occam_Item_Inventory_Data` ItemInventoryData))
  (bind _canbebought (`self.CheckIfItemCanBeBought` ItemInventoryData))
  (if _canbebought
    (`self.AddItemToInventory` _hardcodedname _itemtype 1)
    (`self.RemoveCurrency` _buyvalue)
    (`self.RefreshStoreItemDetails` false)))

(fn `CheckAmountOfItemInInventory`
  (params (ItemHardcodedName :type Name))
  (returns (TotalAmountOwned :type Integer))
  (locals (Local_TotalAmountOwned :type Integer))
  (for _array_element (`/Game/Occam/2_Programming/8_SaveContainers/BP_Occam_GI_General.Inventory` (`self.GameInstanceReference`))
    (bind (_stacksamount _itemsinventorydata) (break `/Game/Occam/2_Programming/2_Structures/Items/Strut_Occam_Items_DynamicData` _array_element))
    (if (== (`.HardcodedName_31_372A6D92438D3B8613C5F99C2D743AB0` (break `/Game/Occam/2_Programming/2_Structures/Items/Strut_Occam_Item_Inventory_Data` _itemsinventorydata)) ItemHardcodedName)
      (set `local.Local_TotalAmountOwned` (+ _stacksamount (`local.Local_TotalAmountOwned`)))))
  (return (`local.Local_TotalAmountOwned`)))

(fn `CheckIfItemCanBeBought`
  (params (ItemInventoryData :type "/Game/Occam/2_Programming/2_Structures/Items/Strut_Occam_Item_Inventory_Data Structure"))
  (returns (CanBeBought :type Boolean))
  (bind (_itemtype _itemsubtype _hardcodedname _displayname _keyitem_ _rarity _buyvalue) (break `/Game/Occam/2_Programming/2_Structures/Items/Strut_Occam_Item_Inventory_Data` ItemInventoryData))
  (if (>= (`/Game/Occam/2_Programming/8_SaveContainers/BP_Occam_GI_General.Currency` (`self.GameInstanceReference`)) _buyvalue)
    (bind (_success_ _isitemfullystacked_) (`self.CheckIfThereIsItemInInventory` _hardcodedname))
    (if _success_
      (return (not _isitemfullystacked_))
      (else
        (return (`self.CheckIfThereIsFreeSlotInInventory`))))
    (else
      (return false))))

(fn `CheckIfItemCanBeSold`
  (params (ItemInventoryData :type "/Game/Occam/2_Programming/2_Structures/Items/Strut_Occam_Item_Inventory_Data Structure"))
  (returns (CanBeSold :type Boolean))
  (bind (_itemtype _itemsubtype _hardcodedname _displayname _keyitem_ _rarity _buyvalue _sellvalue) (break `/Game/Occam/2_Programming/2_Structures/Items/Strut_Occam_Item_Inventory_Data` ItemInventoryData))
  (return (and (not _keyitem_) (> _sellvalue 0))))

(fn `CheckIfThereIsFreeSlotInInventory`
  (returns (`Success?` :type Boolean))
  (if (== (`self.InventorySlotsAmount`) 0)
    (return true)
    (else
      (return (< (`KismetArrayLibrary.Array_Length` (`/Game/Occam/2_Programming/8_SaveContainers/BP_Occam_GI_General.Inventory` (`self.GameInstanceReference`))) (`self.InventorySlotsAmount`))))))

(fn `CheckIfThereIsItemInInventory`
  (params (ItemHardcodedName :type Name))
  (returns (`Success?` :type Boolean) (`IsItemFullyStacked?` :type Boolean) (ItemIndex :type Integer))
  (locals (`Local_Success?` :type Boolean) (`Local_IsItemFullyStacked?` :type Boolean) (Local_ItemIndex :type Integer))
  (for (_array_element _array_index) (`/Game/Occam/2_Programming/8_SaveContainers/BP_Occam_GI_General.Inventory` (`self.GameInstanceReference`))
    (bind (_stacksamount _itemsinventorydata) (break `/Game/Occam/2_Programming/2_Structures/Items/Strut_Occam_Items_DynamicData` _array_element))
    (bind (_itemtype _itemsubtype _hardcodedname _displayname _keyitem_ _rarity _buyvalue _sellvalue _maxstackamount) (break `/Game/Occam/2_Programming/2_Structures/Items/Strut_Occam_Item_Inventory_Data` _itemsinventorydata))
    (if (== _hardcodedname ItemHardcodedName)
      (set `local.Local_Success?` true)
      (set `local.Local_IsItemFullyStacked?` (== _stacksamount _maxstackamount))
      (set `local.Local_ItemIndex` _array_index)
      (break)))
  (return (`local.Local_Success?`) (`local.Local_IsItemFullyStacked?`) (`local.Local_ItemIndex`)))

(fn `CheckIfThereIsNotFullyStackedItemInInventory`
  (params (ItemHardcodedName :type Name))
  (returns (`Success?` :type Boolean) (ItemIndex :type Integer))
  (locals (`Local_Success?` :type Boolean) (Local_ItemIndex :type Integer))
  (for (_array_element _array_index) (`/Game/Occam/2_Programming/8_SaveContainers/BP_Occam_GI_General.Inventory` (`self.GameInstanceReference`))
    (bind (_stacksamount _itemsinventorydata) (break `/Game/Occam/2_Programming/2_Structures/Items/Strut_Occam_Items_DynamicData` _array_element))
    (bind (_itemtype _itemsubtype _hardcodedname _displayname _keyitem_ _rarity _buyvalue _sellvalue _maxstackamount) (break `/Game/Occam/2_Programming/2_Structures/Items/Strut_Occam_Item_Inventory_Data` _itemsinventorydata))
    (if (== _hardcodedname ItemHardcodedName)
      (if (< _stacksamount _maxstackamount)
        (set `local.Local_Success?` true)
        (set `local.Local_ItemIndex` _array_index)
        (break))))
  (return (`local.Local_Success?`) (`local.Local_ItemIndex`)))

(fn `CreateReferenceToInventoryWindow`
  ;[1 1 1] Get exisiting Inventory Screen Widget, create reference to it.
  (bind _foundwidgets (`WidgetBlueprintLibrary.GetAllWidgetsOfClass` "/Game/Occam/6_UI/0_WBP/6_Overview/WBP_Occam_InventoryMenu.WBP_Occam_InventoryMenu_C" false))
  (bind _output (`|GetArrayItem` _foundwidgets))
  (`/Engine/EditorBlueprintResources/StandardMacros.IsValid` _output
    (:`Is Valid`
      (set `/Game/Occam/6_UI/0_WBP/6_Overview/WBP_Occam_InventoryMenu.InventoryManagerReference` self _output)
      (set `self.InventoryScreenReference` _output)
      ;[1 1 1] Initially updates inventory screen data.
      (`self.RefreshItemDetails`)
      (`self.RefreshAllInventorySlots`)
      (`self.RefreshCurrencyAmount`))))

(fn `CreateReferenceToVendorWindow`
  ;[1 1 1] Get exisiting Store Menu Widget, create reference to it.
  (bind _foundwidgets (`WidgetBlueprintLibrary.GetAllWidgetsOfClass` "/Game/Occam/6_UI/0_WBP/WBP_Occam_StoreMenu.WBP_Occam_StoreMenu_C" false))
  (bind _output (`|GetArrayItem` _foundwidgets))
  (`/Engine/EditorBlueprintResources/StandardMacros.IsValid` _output
    (:`Is Valid`
      (set `self.StoreWindow` _output)
      (set `/Game/Occam/6_UI/0_WBP/WBP_Occam_StoreMenu.InventoryManagerReference` self _output))))

(fn `GetProperInventorySlotWidget`
  (params (ItemIndex :type Integer))
  (returns (InventorySlot :type "/Game/Occam/6_UI/0_WBP/WBP_InventorySlot Object Reference"))
  (bind _inventoryslotsreference (`self.InventorySlotsReference`))
  (`/Engine/EditorBlueprintResources/StandardMacros.IsValid` (`self.InventoryScreenReference`)
    (:`Is Valid`
      (if (`KismetArrayLibrary.Array_IsValidIndex` _inventoryslotsreference ItemIndex)
        (return (`|GetArrayItem` _inventoryslotsreference ItemIndex))
        (else
          (bind _returnvalue (`|CreateWidget` "/Game/Occam/6_UI/0_WBP/WBP_InventorySlot.WBP_InventorySlot_C" null self))
          (`/Engine/EditorBlueprintResources/StandardMacros.IsValid` _returnvalue
            (:`Is Valid`
              (`KismetArrayLibrary.Array_Add` (`self.InventorySlotsReference`) _returnvalue)
              (`PanelWidget.AddChild` (`/Game/Occam/6_UI/0_WBP/6_Overview/WBP_Occam_InventoryMenu.VB_ItemList` (`self.InventoryScreenReference`)) _returnvalue)
              (return _returnvalue))))))))

(fn `GetProperStoreSlot`
  (params (Index :type Integer))
  (returns (StoreItemSlot :type "/Game/Occam/6_UI/0_WBP/WBP_StoreSlot Object Reference"))
  (bind _storeitemslots (`self.StoreItemSlots`))
  (if (`KismetArrayLibrary.Array_IsValidIndex` _storeitemslots Index)
    (return (`|GetArrayItem` _storeitemslots Index))
    (else
      (bind _returnvalue (`|CreateWidget` "/Game/Occam/6_UI/0_WBP/WBP_StoreSlot.WBP_StoreSlot_C" null self))
      (`KismetArrayLibrary.Array_Add` (`self.StoreItemSlots`) _returnvalue)
      (`VerticalBox.AddChildToVerticalBox` (`/Game/Occam/6_UI/0_WBP/WBP_Occam_StoreMenu.VB_StoreItemList` (`self.StoreWindow`)) _returnvalue)
      (return _returnvalue))))

(fn `RefreshAllInventorySlots`
  ;[1 1 1 1 12] Hides all inventory slots, just in case if currently there is more slots than items in inventory.
  ; It prevents from showing slots that have no any item assigned to them.
  (for _array_element (`self.InventorySlotsReference`)
    (`Widget.SetVisibility` _array_element "Collapsed"))
  (for (_array_element_2 _array_index) (`/Game/Occam/2_Programming/8_SaveContainers/BP_Occam_GI_General.Inventory` (`self.GameInstanceReference`))
    (bind _inventoryslot (`self.GetProperInventorySlotWidget` _array_index))
    (`/Engine/EditorBlueprintResources/StandardMacros.IsValid` _inventoryslot
      (:`Is Valid`
        (bind (_stacksamount _itemsinventorydata) (break `/Game/Occam/2_Programming/2_Structures/Items/Strut_Occam_Items_DynamicData` _array_element_2))
        (`/Game/Occam/6_UI/0_WBP/WBP_InventorySlot.UpdateItemData` _inventoryslot _stacksamount _itemsinventorydata))))
  (`self.RefreshItemDetails`) ; Updates Inventory Screen data with currently selected item slot.
)

(fn `RefreshCurrencyAmount`
  (bind _foundwidgets (`WidgetBlueprintLibrary.GetAllWidgetsOfClass` "/Game/Occam/6_UI/0_WBP/2_Main/WBP_WorldInterface.WBP_WorldInterface_C" false))
  (bind _output (`|GetArrayItem` _foundwidgets))
  (`/Engine/EditorBlueprintResources/StandardMacros.IsValid` _output
    (:`Is Valid`
      (bind _foundwidgets_2 (`WidgetBlueprintLibrary.GetAllWidgetsOfClass` "/Game/Occam/6_UI/0_WBP/WBP_Occam_StoreMenu.WBP_Occam_StoreMenu_C" false))
      (`/Engine/EditorBlueprintResources/StandardMacros.IsValid` (`|GetArrayItem` _foundwidgets_2)
        (:`Is Valid`
          (`TextBlock.SetText` (`/Game/Occam/6_UI/0_WBP/WBP_Occam_StoreMenu.TX_PlayerCurrency` (`/Game/Occam/6_UI/0_WBP/2_Main/WBP_WorldInterface.WBP_Occam_StoreMenu` _output)) (`KismetTextLibrary.Conv_IntToText` (`/Game/Occam/2_Programming/8_SaveContainers/BP_Occam_GI_General.Currency` (`self.GameInstanceReference`)) false false))
          (`TextBlock.SetText` (`/Game/Occam/6_UI/0_WBP/WBP_Occam_StoreMenu.TX_PlayerCurrency` (`|GetArrayItem` _foundwidgets_2)) (`KismetTextLibrary.Conv_IntToText` (`/Game/Occam/2_Programming/8_SaveContainers/BP_Occam_GI_General.Currency` (`self.GameInstanceReference`)) false false)))))))

(fn `RefreshInventorySlot`
  (params (SlotIndex :type Integer))
  (bind (_stacksamount _itemsinventorydata) (break `/Game/Occam/2_Programming/2_Structures/Items/Strut_Occam_Items_DynamicData` (`|GetArrayItem` (`/Game/Occam/2_Programming/8_SaveContainers/BP_Occam_GI_General.Inventory` (`self.GameInstanceReference`)) SlotIndex)))
  (bind _inventoryslot (`self.GetProperInventorySlotWidget` SlotIndex))
  (`/Engine/EditorBlueprintResources/StandardMacros.IsValid` _inventoryslot
    (:`Is Valid`
      (`/Game/Occam/6_UI/0_WBP/WBP_InventorySlot.UpdateItemData` _inventoryslot _stacksamount _itemsinventorydata))))

(fn `RefreshInventorySlotAfterDiscarding`
  (params (SlotIndex :type Integer))
  (bind _returnvalue (`KismetArrayLibrary.Array_Length` (`/Game/Occam/2_Programming/8_SaveContainers/BP_Occam_GI_General.Inventory` (`self.GameInstanceReference`))))
  (if (> _returnvalue 0)
    (bind _inventoryslot (`self.GetProperInventorySlotWidget` (`KismetMathLibrary.SelectInt` SlotIndex (- _returnvalue 1) (< SlotIndex _returnvalue))))
    (`/Engine/EditorBlueprintResources/StandardMacros.IsValid` _inventoryslot
      (:`Is Valid`
        (`/Game/Occam/6_UI/0_WBP/6_Overview/WBP_Occam_InventoryMenu.HighlightNewInventoryButton` (`self.InventoryScreenReference`) (`/Game/Occam/6_UI/0_WBP/WBP_InventorySlot.BTN_InventorySlot` _inventoryslot))))))

(fn `RefreshItemDetails`
  (bind (_itemtype _itemsubtype _hardcodedname _displayname _keyitem_ _rarity _buyvalue _sellvalue _maxstackamount _description) (break `/Game/Occam/2_Programming/2_Structures/Items/Strut_Occam_Item_Inventory_Data` (`.ItemsInventoryData_20_E92CE3CC45840EE43F13188944129CE9` (break `/Game/Occam/2_Programming/2_Structures/Items/Strut_Occam_Items_DynamicData` (`|GetArrayItem` (`/Game/Occam/2_Programming/8_SaveContainers/BP_Occam_GI_General.Inventory` (`self.GameInstanceReference`)) (`self.SelectedItemSlot`))))))
  (`/Engine/EditorBlueprintResources/StandardMacros.IsValid` (`self.InventoryScreenReference`)
    (:`Is Valid`
      (if (> (`KismetArrayLibrary.Array_Length` (`/Game/Occam/2_Programming/8_SaveContainers/BP_Occam_GI_General.Inventory` (`self.GameInstanceReference`))) 0)
        (`Widget.SetVisibility` (`/Game/Occam/6_UI/0_WBP/6_Overview/WBP_Occam_InventoryMenu.VB_ItemList` (`self.InventoryScreenReference`)) "Visible")
        (`/Game/Occam/6_UI/0_WBP/6_Overview/WBP_Occam_InventoryMenu.UpdateItemDetails` (`self.InventoryScreenReference`) (`KismetTextLibrary.Conv_NameToText` _displayname) _itemsubtype _rarity (`KismetTextLibrary.Conv_StringToText` _description))
        (`Widget.SetIsEnabled` (`self.InventoryScreenReference`) false)
        (else
          (`Widget.SetVisibility` (`/Game/Occam/6_UI/0_WBP/6_Overview/WBP_Occam_InventoryMenu.VB_ItemList` (`self.InventoryScreenReference`)) "Hidden"))))))

(fn `RefreshStoreItemDetails`
  (params (ShowItemFromInventory :type Boolean))
  (bind (_stacksamount _itemsinventorydata) (break `/Game/Occam/2_Programming/2_Structures/Items/Strut_Occam_Items_DynamicData` (`|GetArrayItem` (`/Game/Occam/2_Programming/8_SaveContainers/BP_Occam_GI_General.Inventory` (`self.GameInstanceReference`)) (`self.SelectedStoreSlot`))))
  (bind (_itemtype _itemsubtype _hardcodedname _displayname _keyitem_ _rarity _buyvalue _sellvalue _maxstackamount _description) (break `/Game/Occam/2_Programming/2_Structures/Items/Strut_Occam_Item_Inventory_Data` _itemsinventorydata))
  (`/Engine/EditorBlueprintResources/StandardMacros.IsValid` (`self.StoreWindow`)
    (:`Is Valid`
      (if ShowItemFromInventory
        (if (> (`KismetArrayLibrary.Array_Length` (`/Game/Occam/2_Programming/8_SaveContainers/BP_Occam_GI_General.Inventory` (`self.GameInstanceReference`))) 0)
          (`Widget.SetVisibility` (`/Game/Occam/6_UI/0_WBP/WBP_Occam_StoreMenu.VB_ItemDetails` (`self.StoreWindow`)) "Visible")
          ;[1 1 1] Redo\
          (`/Game/Occam/6_UI/0_WBP/WBP_Occam_StoreMenu.UpdateItemDetails` (`self.StoreWindow`) (`KismetTextLibrary.Conv_NameToText` _hardcodedname) _itemsubtype _rarity (`KismetTextLibrary.Conv_StringToText` _description))
          (bind _canbesold (`self.CheckIfItemCanBeSold` _itemsinventorydata))
          (`Widget.SetIsEnabled` (`/Game/Occam/6_UI/0_WBP/WBP_Occam_StoreMenu.BTN_Sell` (`self.StoreWindow`)) _canbesold)
          (`/Game/Occam/6_UI/0_WBP/WBP_Occam_StoreMenu.HighlightNewStoreButton` (`self.StoreWindow`) (`/Game/Occam/6_UI/0_WBP/WBP_StoreSlot.BTN_StoreSlot` (`|GetArrayItem` (`self.StoreItemSlots`) (`self.SelectedStoreSlot`))))
          (else
            (`Widget.SetVisibility` (`/Game/Occam/6_UI/0_WBP/WBP_Occam_StoreMenu.VB_ItemDetails` (`self.StoreWindow`)) "Hidden")))
        (elif (> (`BlueprintSetLibrary.Set_Length` (`self.StoreItems`)) 0)
          (`Widget.SetVisibility` (`/Game/Occam/6_UI/0_WBP/WBP_Occam_StoreMenu.VB_ItemDetails` (`self.StoreWindow`)) "Visible")
          (bind _result (`BlueprintSetLibrary.Set_ToArray` (`self.StoreItems`)))
          (bind (_itemhardcodedname _itemtype_2) (break `/Game/Occam/2_Programming/2_Structures/Items/Strut_Occam_Loot_Data` (`|GetArrayItem` _result (`self.SelectedStoreSlot`))))
          (bind (_hardcodedname_2 _iteminventorydata) (`/Game/Occam/2_Programming/FL_Occam_Custom.ItemTypeData_To_ItemInventoryData` _itemhardcodedname _itemtype_2))
          (bind (_itemtype_3 _itemsubtype_2 _hardcodedname_3 _displayname_2 _keyitem__2 _rarity_2 _buyvalue_2 _sellvalue_2 _maxstackamount_2 _description_2) (break `/Game/Occam/2_Programming/2_Structures/Items/Strut_Occam_Item_Inventory_Data` _iteminventorydata))
          (`/Game/Occam/6_UI/0_WBP/WBP_Occam_StoreMenu.UpdateItemDetails` (`self.StoreWindow`) (`KismetTextLibrary.Conv_NameToText` _displayname_2) _itemsubtype_2 _rarity_2 (`KismetTextLibrary.Conv_StringToText` _description_2))
          (bind _canbebought (`self.CheckIfItemCanBeBought` _iteminventorydata))
          (`Widget.SetIsEnabled` (`/Game/Occam/6_UI/0_WBP/WBP_Occam_StoreMenu.BTN_Buy` (`self.StoreWindow`)) _canbebought)
          (`/Game/Occam/6_UI/0_WBP/WBP_Occam_StoreMenu.HighlightNewStoreButton` (`self.StoreWindow`) (`/Game/Occam/6_UI/0_WBP/WBP_StoreSlot.BTN_StoreSlot` (`|GetArrayItem` (`self.StoreItemSlots`) (`self.SelectedStoreSlot`))))
          (else
            (`Widget.SetVisibility` (`/Game/Occam/6_UI/0_WBP/WBP_Occam_StoreMenu.VB_ItemDetails` (`self.StoreWindow`)) "Hidden")))))))

(fn `ReleaseInventorySlot`
  (params (InventorySlot :type Integer))
  (locals (Local_SlotToRemove :type "/Game/Occam/6_UI/0_WBP/WBP_InventorySlot Object Reference"))
  (bind _inventoryslotsreference (`self.InventorySlotsReference`))
  (bind _output (`|GetArrayItem` (`self.InventorySlotsReference`) InventorySlot))
  (`/Engine/EditorBlueprintResources/StandardMacros.IsValid` _output
    (:`Is Valid`
      (set `local.Local_SlotToRemove` _output)
      (`Widget.SetVisibility` (`local.Local_SlotToRemove`) "Collapsed")
      ;[1 1 1] Remove slot and readd it to slots pool. This way currently not used slots will be always at the end of the array and its parent widget.
      (`KismetArrayLibrary.Array_Remove` _inventoryslotsreference InventorySlot)
      (`KismetArrayLibrary.Array_Add` _inventoryslotsreference (`local.Local_SlotToRemove`))
      (`VerticalBox.AddChildToVerticalBox` (`/Game/Occam/6_UI/0_WBP/6_Overview/WBP_Occam_InventoryMenu.VB_ItemList` (`self.InventoryScreenReference`)) (`local.Local_SlotToRemove`))
      ;[1 1 1] After removing item and hiding slot we have to make sure that Inventory Screen will be updated we new item details.
      (if (<= (`self.SelectedItemSlot`) (`KismetArrayLibrary.Array_LastIndex` (`/Game/Occam/2_Programming/8_SaveContainers/BP_Occam_GI_General.Inventory` (`self.GameInstanceReference`))))
        (`self.RefreshItemDetails`)
        (else
          (set `self.SelectedItemSlot` (`KismetArrayLibrary.Array_LastIndex` (`/Game/Occam/2_Programming/8_SaveContainers/BP_Occam_GI_General.Inventory` (`self.GameInstanceReference`))))
          (`self.RefreshItemDetails`))))))

(fn `RemoveCurrency`
  (params (BuyValue :type Integer))
  (bind _gameinstancereference (`self.GameInstanceReference`))
  (bind _currency (`/Game/Occam/2_Programming/8_SaveContainers/BP_Occam_GI_General.Currency` _gameinstancereference))
  (`/Engine/EditorBlueprintResources/StandardMacros.CompareInt` _currency BuyValue
    (:`>`
      (set `/Game/Occam/2_Programming/8_SaveContainers/BP_Occam_GI_General.Currency` (- _currency BuyValue) _gameinstancereference :!label _label)
      (`self.RefreshCurrencyAmount`)
      (`self.RefreshAllInventorySlots`))
    (:`==`
      (goto _label))
    (:`<`
      (`KismetSystemLibrary.PrintString` "Hello you're broke"))))

(fn `RemoveItemFromInventory`
  (params (ItemRowName :type Name) (Amount :type Integer))
  (locals (Local_ItemRowName :type Name) (Local_AmountToRemove :type Integer) (Local_SlotIndexToCheck :type Integer :default 0))
  (bind _local_slotindextocheck (`local.Local_SlotIndexToCheck`))
  (bind _output (`|GetArrayItem` (`/Game/Occam/2_Programming/8_SaveContainers/BP_Occam_GI_General.Inventory` (`self.GameInstanceReference`)) (`local.Local_SlotIndexToCheck`)))
  (set `local.Local_ItemRowName` ItemRowName)
  (set `local.Local_AmountToRemove` Amount)
  ;[1 1 1] Remove item from inventory, multi stacking is NOT allowed.
  (bind (_success_ _isitemfullystacked_ _itemindex) (`self.CheckIfThereIsItemInInventory` (`local.Local_ItemRowName`)))
  (if _success_
    (set `local.Local_SlotIndexToCheck` _itemindex)
    (bind _structout (setmembers `/Game/Occam/2_Programming/2_Structures/Items/Strut_Occam_Items_DynamicData` :`StructRef` _output :`StacksAmount` (- (`.StacksAmount_4_FBB4D29F4BCBB2C737E24E9E13232072` (break `/Game/Occam/2_Programming/2_Structures/Items/Strut_Occam_Items_DynamicData` _output)) (`local.Local_AmountToRemove`))))
    (if (> (`.StacksAmount_4_FBB4D29F4BCBB2C737E24E9E13232072` (break `/Game/Occam/2_Programming/2_Structures/Items/Strut_Occam_Items_DynamicData` _structout)) 0)
      (`self.RefreshInventorySlot` (`local.Local_SlotIndexToCheck`))
      (else
        (`KismetArrayLibrary.Array_Remove` (`/Game/Occam/2_Programming/8_SaveContainers/BP_Occam_GI_General.Inventory` (`self.GameInstanceReference`)) _local_slotindextocheck) ; Remove item data from inventory.
        (`self.ReleaseInventorySlot` _local_slotindextocheck)))
    (`self.RefreshInventorySlotAfterDiscarding` (`local.Local_SlotIndexToCheck`))))

(fn `SellItem`
  (params (ItemInventoryData :type "/Game/Occam/2_Programming/2_Structures/Items/Strut_Occam_Item_Inventory_Data Structure"))
  (locals (Local_ItemToSell :type Name))
  (bind (_itemtype _itemsubtype _hardcodedname _displayname _keyitem_ _rarity _buyvalue _sellvalue) (break `/Game/Occam/2_Programming/2_Structures/Items/Strut_Occam_Item_Inventory_Data` ItemInventoryData))
  (bind _selectedstoreslot (`self.SelectedStoreSlot`))
  (bind _returnvalue (- (`KismetArrayLibrary.Array_Length` (`/Game/Occam/2_Programming/8_SaveContainers/BP_Occam_GI_General.Inventory` (`self.GameInstanceReference`))) 1))
  (bind _canbesold (`self.CheckIfItemCanBeSold` ItemInventoryData))
  (if _canbesold
    (`self.RemoveItemFromInventory` _hardcodedname 1)
    (`self.AddCurrency` _sellvalue)
    (`self.ShowItemsToSell` (`KismetMathLibrary.SelectInt` _selectedstoreslot _returnvalue (< _selectedstoreslot _returnvalue)))))

(fn `ShowItemsToBuy`
  (params (SlotToFocus :type Integer))
  (set `self.SelectedStoreSlot` SlotToFocus)
  (for _array_element (`self.StoreItemSlots`)
    (`Widget.SetVisibility` _array_element "Collapsed"))
  (bind _result (`BlueprintSetLibrary.Set_ToArray` (`self.StoreItems`)))
  (for (_array_element_2 _array_index) _result
    (bind (_itemhardcodedname _itemtype) (break `/Game/Occam/2_Programming/2_Structures/Items/Strut_Occam_Loot_Data` _array_element_2))
    (bind (_hardcodedname _iteminventorydata) (`/Game/Occam/2_Programming/FL_Occam_Custom.ItemTypeData_To_ItemInventoryData` _itemhardcodedname _itemtype))
    (bind _storeitemslot (`self.GetProperStoreSlot` _array_index))
    (bind _output_get (set `/Game/Occam/6_UI/0_WBP/WBP_StoreSlot.ItemFromInventory?` false _storeitemslot))
    (`/Game/Occam/6_UI/0_WBP/WBP_StoreSlot.UpdateItemData` _storeitemslot 0 _iteminventorydata)
    (`/Game/Occam/6_UI/0_WBP/WBP_StoreSlot.UpdateItemData` _storeitemslot 0 _iteminventorydata))
  (`self.RefreshStoreItemDetails` false))

(fn `ShowItemsToSell`
  (params (SlotToFocus :type Integer))
  (set `self.SelectedStoreSlot` SlotToFocus)
  (for _array_element (`self.StoreItemSlots`)
    (`Widget.SetVisibility` _array_element "Collapsed"))
  (for (_array_element_2 _array_index) (`/Game/Occam/2_Programming/8_SaveContainers/BP_Occam_GI_General.Inventory` (`self.GameInstanceReference`))
    (bind _storeitemslot (`self.GetProperStoreSlot` _array_index))
    (set `/Game/Occam/6_UI/0_WBP/WBP_StoreSlot.ItemFromInventory?` true _storeitemslot)
    (bind (_stacksamount _itemsinventorydata) (break `/Game/Occam/2_Programming/2_Structures/Items/Strut_Occam_Items_DynamicData` _array_element_2))
    (`/Game/Occam/6_UI/0_WBP/WBP_StoreSlot.UpdateItemData` _storeitemslot _stacksamount _itemsinventorydata)
    (`/Game/Occam/6_UI/0_WBP/WBP_StoreSlot.UpdateItemData` _storeitemslot _stacksamount _itemsinventorydata))
  (`self.RefreshStoreItemDetails` true))