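; Player controller for Occam's controller test screen, which shows the sim controller-test widget with Game and UI input focused on it.
; If the gamepad controls component is enabled, it hides the cursor and activates controller-test mode; otherwise it shows the cursor.
; D-pad up/down presses forward to that component.
; MoveForward stick input triggers the same handlers through Delays set by the menu scroll speed, throttling repeats.
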(event `self.ReceiveBeginPlay`
  (bind _returnvalue (`|CreateWidget` "/Game/Occam/6_UI/0_WBP/WBP_Occam_Sim_ControllerTest.WBP_Occam_Sim_ControllerTest_C"))
  (`WidgetBlueprintLibrary.SetInputMode_GameAndUIEx` self _returnvalue "DoNotLock" false)
  (`UserWidget.AddToViewport` _returnvalue 0)
  (if (`/Game/Occam/2_Programming/0_Components/AC_Occam_GamepadControls.GamepadControlsEnabled?` (`self.AC_Occam_GamepadControls`))
    (set `self.bShowMouseCursor` false)
    (`/Game/Occam/2_Programming/0_Components/AC_Occam_GamepadControls.ActivateGamepadControls_ControllerTest` (`self.AC_Occam_GamepadControls`))
    (else
      (set `self.bShowMouseCursor` true))))

(event `InputAction|D-PadUp` :paused true
  (params (Key :type "Key Structure"))
  (:`Pressed`
    (`/Game/Occam/2_Programming/0_Components/AC_Occam_GamepadControls.D-PadUpPressed` (`self.AC_Occam_GamepadControls`) :!label _label)))

(event `InputAxis|MoveForward`
  (params (AxisValue :type "Float (single-precision)"))
  (bind _joystick_menuscroll_speed (`/Game/Occam/2_Programming/0_Components/AC_Occam_GamepadControls.Joystick_MenuScroll_Speed` (`self.AC_Occam_GamepadControls`)))
  (`/Engine/EditorBlueprintResources/StandardMacros.CompareFloat` AxisValue
    (:`>`
      (`KismetSystemLibrary.Delay` _joystick_menuscroll_speed)
      (goto _label))
    (:`<`
      (`KismetSystemLibrary.Delay` _joystick_menuscroll_speed)
      (`/Game/Occam/2_Programming/0_Components/AC_Occam_GamepadControls.D-PadDownPressed` (`self.AC_Occam_GamepadControls`) :!label _label_2))))

(event `InputAction|D-PadDown` :paused true
  (params (Key :type "Key Structure"))
  (:`Pressed`
    (goto _label_2)))

(event `InputAction|D-PadRight` :paused true
  (params (Key :type "Key Structure")))

(event `InputAction|D-PadLeft` :paused true
  (params (Key :type "Key Structure")))

(event `InputAction|AcceptButton` :paused true
  (params (Key :type "Key Structure")))

(event `InputAction|CancelButton` :paused true
  (params (Key :type "Key Structure")))

(event `InputAction|SelectButton` :paused true
  (params (Key :type "Key Structure")))

(event `InputAction|DiscardButton` :paused true
  (params (Key :type "Key Structure")))

(event `InputAction|ShoulderRight` :paused true
  (params (Key :type "Key Structure")))

(event `InputAction|TriggerRight` :paused true
  (params (Key :type "Key Structure")))

(event `InputAction|ShoulderLeft`
  (params (Key :type "Key Structure")))

(event `InputAction|TriggerLeft`
  (params (Key :type "Key Structure")))

(fn `UserConstructionScript`)