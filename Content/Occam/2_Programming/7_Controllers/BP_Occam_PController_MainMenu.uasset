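; Player controller for the Occam main menu, which creates and shows the menu when play begins.
; BeginPlay sets Game and UI input, creates the main menu widget with a reference to the save manager component, and refreshes the load slots.
; If gamepad controls are enabled, it hides the mouse cursor and activates the gamepad component's main menu controls.
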(event `self.ReceiveBeginPlay`
  (`WidgetBlueprintLibrary.SetInputMode_GameAndUIEx` self null "DoNotLock" false)
  (bind _returnvalue (`|CreateWidget` "/Game/Occam/6_UI/0_WBP/2_Main/WBP_Occam_MainMenu.WBP_Occam_MainMenu_C" null (`self.AC_Occam_SaveManager`)))
  (bind _output_get (set `self.MainMenu` _returnvalue))
  (`UserWidget.AddToViewport` _output_get 0)
  (`/Game/Occam/2_Programming/0_Components/AC_Occam_SaveManager.RefreshLoadSlots` (`self.AC_Occam_SaveManager`))
  (if (`/Game/Occam/2_Programming/0_Components/AC_Occam_GamepadControls.GamepadControlsEnabled?` (`self.AC_Occam_GamepadControls`))
    (set `self.bShowMouseCursor` false)
    (`/Game/Occam/2_Programming/0_Components/AC_Occam_GamepadControls.ActivateGamepadControls_MainMenu` (`self.AC_Occam_GamepadControls`))))

(event `InputAction|D-PadUp` :paused true
  (params (Key :type "Key Structure")))

(event `InputAction|D-PadDown` :paused true
  (params (Key :type "Key Structure")))

(event `InputAction|D-PadRight` :paused true
  (params (Key :type "Key Structure")))

(event `InputAction|D-PadLeft` :paused true
  (params (Key :type "Key Structure")))

(event `InputAction|AcceptButton` :paused true
  (params (Key :type "Key Structure")))

(event `InputAction|CancelButton` :paused true
  (params (Key :type "Key Structure")))

(event `InputAction|SelectButton` :paused true
  (params (Key :type "Key Structure")))

(event `InputAction|DiscardButton` :paused true
  (params (Key :type "Key Structure")))

(event `InputAction|ShoulderRight` :paused true
  (params (Key :type "Key Structure")))

(event `InputAction|TriggerRight` :paused true
  (params (Key :type "Key Structure")))

(event `InputAction|ShoulderLeft`
  (params (Key :type "Key Structure")))

(event `InputAction|TriggerLeft`
  (params (Key :type "Key Structure")))

(fn `UserConstructionScript`)