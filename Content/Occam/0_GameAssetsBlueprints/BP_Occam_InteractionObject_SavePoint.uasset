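; Interactable save point that opens the player's world save menu when interaction is requested.
; On construction it takes its label and global ID from the save point data table, using map name and index.
; Entering range registers it with the player controller's save manager and plays a montage; leaving clears that and plays it reversed.
; On BeginPlay or status update, it applies the active material if it matches the GameInstance's last saved point.
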(event `self.ReceiveBeginPlay`
  (`parent.ReceiveBeginPlay`)
  (bind _asbp_occam_gi_general (cast `/Game/Occam/2_Programming/8_SaveContainers/BP_Occam_GI_General` (`GameplayStatics.GetGameInstance`) :!label _label))
  (if (== (`/Game/Occam/2_Programming/8_SaveContainers/BP_Occam_GI_General.LastSavedPointName` _asbp_occam_gi_general) (`self.ObjectGlobalID`))
    (`PrimitiveComponent.SetMaterial` (`self.SkeletalMesh`) 0 "/Game/Occam/5_Props/0_Special/SavePoint/MAT_Occam_SavePoint_Base_Active.MAT_Occam_SavePoint_Base_Active")))

(event `SavePoint_UpdateActiveStatus`
  (goto _label))

(event `self.ReceiveActorBeginOverlap`
  (params (OtherActor :type "Actor Object Reference"))
  (`parent.ReceiveActorBeginOverlap` OtherActor))

(event `self.ReceiveTick`
  (params (DeltaSeconds :type "Float (single-precision)"))
  (`parent.ReceiveTick` DeltaSeconds))

(event `/Game/Occam/2_Programming/4_Interfaces/BPI_Occam_Interaction.OnInteractionRequested`
  (params (PlayerWorldCharacter :type "/Game/Occam/2_Programming/5_GameBaseActors/BP_Occam_Character_Player_World Object Reference"))
  (`/Game/Occam/6_UI/0_WBP/2_Main/WBP_WorldInterface.WorldInterface_SaveMenu` (`/Game/Occam/2_Programming/7_Controllers/BP_Occam_PController_World.World Interface` (`/Game/Occam/2_Programming/5_GameBaseActors/BP_Occam_Character_Player_World.PlayerController` PlayerWorldCharacter))))

(event `self.InteractionRange.OnComponentBeginOverlap`
  (params (OverlappedComponent :type "PrimitiveComponent Object Reference") (OtherActor :type "Actor Object Reference") (OtherComp :type "PrimitiveComponent Object Reference") (OtherBodyIndex :type Integer) (bFromSweep :type Boolean) (SweepResult :type "HitResult Structure (by ref)"))
  (if (== OtherActor (`GameplayStatics.GetPlayerCharacter` 0))
    (set `/Game/Occam/2_Programming/0_Components/AC_Occam_SaveManager.SavePointReference` self (`self.GetComponentByClass` (`GameplayStatics.GetPlayerController` 0) "/Game/Occam/2_Programming/0_Components/AC_Occam_SaveManager.AC_Occam_SaveManager_C"))
    (bind _returnvalue (`AnimInstance.Montage_Play` (`SkeletalMeshComponent.GetAnimInstance` (`self.SkeletalMesh`)) "/Game/Occam/5_Props/0_Special/SavePoint/AM_Occam_SavePoint.AM_Occam_SavePoint" 1.0 "MontageLength" 0.0 true))
    (set `self.MontageLength` _returnvalue)))

(event `self.InteractionRange.OnComponentEndOverlap`
  (params (OverlappedComponent :type "PrimitiveComponent Object Reference") (OtherActor :type "Actor Object Reference") (OtherComp :type "PrimitiveComponent Object Reference") (OtherBodyIndex :type Integer))
  (if (== OtherActor (`GameplayStatics.GetPlayerCharacter` 0))
    (set `/Game/Occam/2_Programming/0_Components/AC_Occam_SaveManager.SavePointReference` null (`self.GetComponentByClass` (`GameplayStatics.GetPlayerController` 0) "/Game/Occam/2_Programming/0_Components/AC_Occam_SaveManager.AC_Occam_SaveManager_C"))
    (bind _returnvalue (`AnimInstance.Montage_Play` (`SkeletalMeshComponent.GetAnimInstance` (`self.SkeletalMesh`)) "/Game/Occam/5_Props/0_Special/SavePoint/AM_Occam_SavePoint.AM_Occam_SavePoint" -1.0 "MontageLength" (`self.MontageLength`) true))
    (set `self.MontageLength` _returnvalue)))

(fn `UserConstructionScript`
  (`parent.UserConstructionScript`)
  (bind _returnvalue (`|GetDataTableRow` "/Game/Occam/2_Programming/1_Datatables/DT_Occam_SavePointData.DT_Occam_SavePointData" (`self.LocalMapDataName`))
    (:`then`
      (bind _output (`|GetArrayItem` (`.SavePointHardcodedName_7_D632BBF9447B033CE88B6A8152829E6A` (break `/Game/Occam/2_Programming/2_Structures/Strut_Occam_SavePointData` _returnvalue)) (`self.MapDataIndex`)))
      (`TextRenderComponent.K2_SetText` (`self.TextRender`) (`KismetTextLibrary.Conv_StringToText` _output))
      (set `self.ObjectGlobalID` (`KismetStringLibrary.Conv_StringToName` _output)))))