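; Interactable store object for the game world that acts as an item shop, weapon shop or inn depending on its StoreType.
; On an interaction request, it validates the player character and controller, then has the controller show the store window with the name, greeting, inventory and an inn flag.
; The construction script picks a minimap icon by store type and sets a test display text for inns.
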(event `/Game/Occam/2_Blueprints/4_Interfaces/BPI_Occam_Interaction.OnInteractionRequested`
  (params (PlayerWorldCharacter :type "/Game/Occam/2_Blueprints/5_GameBaseActors/BP_Occam_Character_Player_World Object Reference"))
  (`/Engine/EditorBlueprintResources/StandardMacros.IsValid` PlayerWorldCharacter
    (:`Is Valid`
      (bind _playercontroller (`/Game/Occam/2_Blueprints/5_GameBaseActors/BP_Occam_Character_Player_World.PlayerController` PlayerWorldCharacter)
        (:`then`
          (`/Game/Occam/2_Blueprints/7_Controllers/BP_Occam_PController_World.ShowStoreWindow` _playercontroller (`|EnumEquality` (`self.StoreType`) "NewEnumerator3") (`self.StoreName`) (`self.StoreGreeting`) (`self.StoreInventory`)))
        (:`else`)))))

(fn `UserConstructionScript`
  (bind _storetype (`self.StoreType`))
  (`parent.UserConstructionScript`)
  (set `/Game/Occam/2_Blueprints/0_Components/AC_POI_MiniMap.IconImage` (select `/Game/Occam/2_Blueprints/3_Enumerations/Other/Enum_Occam_StoreTypes` _storetype :`NewEnumerator0` "/Game/Occam/6_UI/8_MiniMap/MiniMap_Sprites/SpriteSheet_UI_HID_MiniMap_Icons_Sprite_4.SpriteSheet_UI_HID_MiniMap_Icons_Sprite_4" :`NewEnumerator1` "/Game/Occam/6_UI/8_MiniMap/MiniMap_Sprites/SpriteSheet_UI_HID_MiniMap_Icons_Sprite_4.SpriteSheet_UI_HID_MiniMap_Icons_Sprite_4" :`NewEnumerator2` "/Game/Occam/6_UI/8_MiniMap/MiniMap_Sprites/SpriteSheet_UI_HID_MiniMap_Icons_Sprite_5.SpriteSheet_UI_HID_MiniMap_Icons_Sprite_5" :`NewEnumerator3` "/Game/Occam/6_UI/8_MiniMap/MiniMap_Sprites/SpriteSheet_UI_HID_MiniMap_Icons_Sprite_3.SpriteSheet_UI_HID_MiniMap_Icons_Sprite_3" :!type "PaperSprite Object Reference") (`self.AC_MiniMapPOI`))
  (if (`|EnumEquality` _storetype "NewEnumerator3")
    (`TextRenderComponent.K2_SetText` (`self.TextRender2`) (`self.TestDisplayForInn`))))