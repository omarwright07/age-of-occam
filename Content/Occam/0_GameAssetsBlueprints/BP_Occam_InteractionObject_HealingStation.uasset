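; Healing station interaction object that restores all of the player's characters to full when used.
; On an interaction request with a valid world character, it calls RecoverAllCharactersToFull on the AC_Occam_CharactersManager component of player controller 0.
; It prints a message and briefly shows a text render as feedback.
; The construction script assigns a fixed ObjectGlobalID, shared by every placed station.
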(event `self.ReceiveBeginPlay`
  (`parent.ReceiveBeginPlay`))

(event `self.ReceiveActorBeginOverlap`
  (params (OtherActor :type "Actor Object Reference"))
  (`parent.ReceiveActorBeginOverlap` OtherActor))

(event `self.ReceiveTick`
  (params (DeltaSeconds :type "Float (single-precision)"))
  (`parent.ReceiveTick` DeltaSeconds))

(event `/Game/Occam/2_Programming/4_Interfaces/BPI_Occam_Interaction.OnInteractionRequested`
  (params (PlayerWorldCharacter :type "/Game/Occam/2_Programming/5_GameBaseActors/BP_Occam_Character_Player_World Object Reference"))
  (bind _returnvalue (`self.GetComponentByClass` (`GameplayStatics.GetPlayerController` 0) "/Game/Occam/2_Programming/0_Components/AC_Occam_CharactersManager.AC_Occam_CharactersManager_C"))
  (`/Engine/EditorBlueprintResources/StandardMacros.IsValid` PlayerWorldCharacter
    (:`Is Valid`
      (`/Engine/EditorBlueprintResources/StandardMacros.IsValid` _returnvalue
        (:`Is Valid`
          (`KismetSystemLibrary.PrintString` "Healling Station")
          (`/Game/Occam/2_Programming/0_Components/AC_Occam_CharactersManager.RecoverAllCharactersToFull` _returnvalue)
          (`SceneComponent.SetVisibility` (`self.TextRender1`) true false)
          (`KismetSystemLibrary.Delay` 0.4)
          (`SceneComponent.SetVisibility` (`self.TextRender1`) false false))))))

(fn `UserConstructionScript`
  (`parent.UserConstructionScript`)
  (set `self.ObjectGlobalID` "Healing Station"))