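; BP_Occam_WalkingPoint is a named marker actor that marks a walking point in the level, with a flag for cutscene use.
; The construction script shows the point's name on a text render and tints it with a cutscene or general color depending on that flag.
; GetWalkingPointTransfrom returns the scene component's world transform, and the event graph holds no active logic.
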(fn `GetWalkingPointTransfrom`
  (returns (SpawnTransform :type "Transform Structure"))
  (return (`SceneComponent.K2_GetComponentToWorld` (`self.Scene`))))

(fn `UserConstructionScript`
  (locals (Local_CutsceneColor :type "Color Structure" :default (struct :`B` 234 :`R` 255)) (Local_GeneralColor :type "Color Structure" :default (struct :`B` 72 :`G` 255)))
  (bind _textrender (`self.TextRender`))
  (`TextRenderComponent.K2_SetText` (`self.TextRender`) (`KismetTextLibrary.Conv_NameToText` (`self.WalkingPointName`)))
  (if (`self.ForCutscene?`)
    (`TextRenderComponent.SetTextRenderColor` _textrender (`local.Local_CutsceneColor`))
    (else
      (`TextRenderComponent.SetTextRenderColor` _textrender (`local.Local_GeneralColor`)))))