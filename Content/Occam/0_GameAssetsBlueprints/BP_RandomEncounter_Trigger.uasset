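; Trigger actor that switches random encounters on or off as the world player character enters its volumes.
; Two overlap boxes, Box_BattleEnabled and Box_BattleDisabled, set the encounter flag on the Occam game instance, which is cached at BeginPlay.
; While DelayEncounter is set, enabling waits for a delay; BeginPlay clears that flag after its own delay, while disabling is always immediate.
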(event `self.ReceiveBeginPlay`
  (bind _asbp_occam_gi_general (cast `/Game/Occam/2_Blueprints/00_SaveContainers/BP_Occam_GI_General` (`GameplayStatics.GetGameInstance`)))
  (set `self.GameInstanceReference` _asbp_occam_gi_general)
  (`KismetSystemLibrary.Delay` (`self.DelayDuration`))
  (set `self.DelayEncounter` false))

(event `self.Box_BattleEnabled.OnComponentBeginOverlap`
  (params (OverlappedComponent :type "PrimitiveComponent Object Reference") (OtherActor :type "Actor Object Reference") (OtherComp :type "PrimitiveComponent Object Reference") (OtherBodyIndex :type Integer) (bFromSweep :type Boolean) (SweepResult :type "HitResult Structure (by ref)"))
  (cast `/Game/Occam/2_Blueprints/5_GameBaseActors/BP_Occam_Character_Player_World` OtherActor)
  (if (`self.DelayEncounter`)
    (`KismetSystemLibrary.Delay` (`self.DelayDuration`)))
  (if (not (`/Game/Occam/2_Blueprints/00_SaveContainers/BP_Occam_GI_General.RandomEncoutersEnabled` (`self.GameInstanceReference`)))
    (set `/Game/Occam/2_Blueprints/00_SaveContainers/BP_Occam_GI_General.RandomEncoutersEnabled` true (`self.GameInstanceReference`))))

(event `self.Box_BattleDisabled.OnComponentBeginOverlap`
  (params (OverlappedComponent :type "PrimitiveComponent Object Reference") (OtherActor :type "Actor Object Reference") (OtherComp :type "PrimitiveComponent Object Reference") (OtherBodyIndex :type Integer) (bFromSweep :type Boolean) (SweepResult :type "HitResult Structure (by ref)"))
  (cast `/Game/Occam/2_Blueprints/5_GameBaseActors/BP_Occam_Character_Player_World` OtherActor)
  (if (`/Game/Occam/2_Blueprints/00_SaveContainers/BP_Occam_GI_General.RandomEncoutersEnabled` (`self.GameInstanceReference`))
    (set `/Game/Occam/2_Blueprints/00_SaveContainers/BP_Occam_GI_General.RandomEncoutersEnabled` false (`self.GameInstanceReference`))))

(fn `UserConstructionScript`)