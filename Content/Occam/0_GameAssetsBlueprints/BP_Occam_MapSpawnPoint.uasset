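; Map spawn point actor that marks either a save-point spawn or an origin spawn in an Occam level.
; The construction script uses the level name as a data table row, reading save point or map data per SaveSpawn and labeling itself with the entry at MapDataIndex.
; It turns both text renders relative to world north via SetToWorldNorth.
; GetSpawnTransfrom returns the Arrow component's world transform as the spawn transform.
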(fn `GetSpawnTransfrom`
  (returns (SpawnTransform :type "Transform Structure"))
  (return (`SceneComponent.K2_GetComponentToWorld` (`self.Arrow`))))

(fn `UserConstructionScript`
  (locals (Local_W :type "Float (double-precision)" :default 180.0))
  (bind _localmapdataname (`self.LocalMapDataName`))
  (bind _returnvalue (`GameplayStatics.GetCurrentLevelName` true))
  (`KismetSystemLibrary.PrintString` _returnvalue)
  (set `self.LocalMapDataName` (`KismetStringLibrary.Conv_StringToName` _returnvalue))
  (if (`self.SaveSpawn?`)
    (bind _returnvalue_2 (`|GetDataTableRow` "/Game/Occam/2_Programming/1_Datatables/DT_Occam_SavePointData.DT_Occam_SavePointData" _localmapdataname)
      (:`then`
        (`TextRenderComponent.K2_SetText` (`self.TextRender`) (`KismetTextLibrary.Conv_StringToText` (`|GetArrayItem` (`.SavePointHardcodedName_7_D632BBF9447B033CE88B6A8152829E6A` (break `/Game/Occam/2_Programming/2_Structures/Strut_Occam_SavePointData` _returnvalue_2)) (`self.MapDataIndex`))))))
    (else
      (bind _returnvalue_3 (`|GetDataTableRow` "/Game/Occam/2_Programming/1_Datatables/DT_Occam_MapData.DT_Occam_MapData" _localmapdataname)
        (:`then`
          (`TextRenderComponent.K2_SetText` (`self.TextRender`) (`KismetTextLibrary.Conv_StringToText` (`|GetArrayItem` (`.OriginSpawnPoint_15_A0CE083E42694BAF0022C6867E85D3DD` (break `/Game/Occam/2_Programming/2_Structures/Strut_Occam_MapData` _returnvalue_3)) (`self.MapDataIndex`))))))))
  (`/Game/Occam/2_Programming/FL_Occam_Custom.SetToWorldNorth` (`self.TextRender`) (`self.Scene`))
  (`/Game/Occam/2_Programming/FL_Occam_Custom.SetToWorldNorth` (`self.TextRender1`) (`self.Scene`)))