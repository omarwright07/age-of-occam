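; BP_Indoor_Temp is an indoor/outdoor transition actor that switches the player's camera between interior and exterior modes.
; Overlapping its indoor or outdoor trigger box with BP_Occam_Character_Player_World calls ChangeCamera with true or false respectively and prints a debug label.
; Two DoOnce gates re-arm each other, so the switches alternate, and the outdoor gate starts closed until the player first enters indoors.
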(event `self.ReceiveBeginPlay`
  (`parent.ReceiveBeginPlay`))

(event `self.ReceiveActorBeginOverlap`
  (params (OtherActor :type "Actor Object Reference"))
  (`parent.ReceiveActorBeginOverlap` OtherActor))

(event `self.ReceiveTick`
  (params (DeltaSeconds :type "Float (single-precision)"))
  (`parent.ReceiveTick` DeltaSeconds))

(event `self.IndoorTriggerBox.OnComponentBeginOverlap`
  (params (OverlappedComponent :type "PrimitiveComponent Object Reference") (OtherActor :type "Actor Object Reference") (OtherComp :type "PrimitiveComponent Object Reference") (OtherBodyIndex :type Integer) (bFromSweep :type Boolean) (SweepResult :type "HitResult Structure (by ref)"))
  (bind _asbp_occam_character_player_world (cast `/Game/Occam/2_Programming/5_GameBaseActors/BP_Occam_Character_Player_World` OtherActor))
  (`/Engine/EditorBlueprintResources/StandardMacros.DoOnce` false :!label _label
    (:`Completed`
      (`|ExecutionSequence`
        (:`then_0`
          (goto _label_2 :!via `Reset`))
        (:`then_1`
          (`KismetSystemLibrary.PrintString` "Inside")
          (`/Game/Occam/2_Programming/5_GameBaseActors/BP_Occam_Character_Player_World.Change Camera` _asbp_occam_character_player_world true))))))

(event `self.OutdoorTriggerBox.OnComponentBeginOverlap`
  (params (OverlappedComponent :type "PrimitiveComponent Object Reference") (OtherActor :type "Actor Object Reference") (OtherComp :type "PrimitiveComponent Object Reference") (OtherBodyIndex :type Integer) (bFromSweep :type Boolean) (SweepResult :type "HitResult Structure (by ref)"))
  (bind _asbp_occam_character_player_world (cast `/Game/Occam/2_Programming/5_GameBaseActors/BP_Occam_Character_Player_World` OtherActor))
  (`/Engine/EditorBlueprintResources/StandardMacros.DoOnce` true :!label _label_2
    (:`Completed`
      (`|ExecutionSequence`
        (:`then_0`
          (goto _label :!via `Reset`))
        (:`then_1`
          (`KismetSystemLibrary.PrintString` "Outside")
          (`/Game/Occam/2_Programming/5_GameBaseActors/BP_Occam_Character_Player_World.Change Camera` _asbp_occam_character_player_world false))))))

(fn `UserConstructionScript`)