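; BP_LightControl is a water environment Blueprint that passes a light's direction and color to the MPC_Water material parameter collection.
; Its UpdateSunAndMoon event writes the light's forward vector to either the Sun or Moon vector parameters, chosen by the SunOrMoon flag.
; It also copies the light color to Sun Reflection Color in both modes, outside the validity check.
; Nothing in this Blueprint calls the event; BeginPlay, Tick and construction are empty.
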(event `UpdateSunAndMoon`
  (bind _light (`self.Light`))
  (bind _returnvalue (`SceneComponent.K2_GetComponentRotation` _light))
  (bind (_returnvalue_x _returnvalue_y _returnvalue_z) (`KismetMathLibrary.BreakVector` (`KismetMathLibrary.GetForwardVector` _returnvalue)))
  (bind (_returnvalue_x_2 _returnvalue_y_2 _returnvalue_z_2) (`KismetMathLibrary.BreakVector` (`KismetMathLibrary.GetForwardVector` _returnvalue)))
  (bind (_returnvalue_x_3 _returnvalue_y_3 _returnvalue_z_3) (`KismetMathLibrary.BreakVector` (`KismetMathLibrary.GetForwardVector` _returnvalue)))
  (bind (_returnvalue_x_4 _returnvalue_y_4 _returnvalue_z_4) (`KismetMathLibrary.BreakVector` (`KismetMathLibrary.GetForwardVector` _returnvalue)))
  (`|ExecutionSequence`
    (:`then_0`
      (`/Engine/EditorBlueprintResources/StandardMacros.IsValid` _light
        (:`Is Valid`
          (if (`self.Sun_or_Moon`)
            (`KismetMaterialLibrary.SetVectorParameterValue` "/Game/Occam/3_Environment/3_Generic/Water/MPC_Water.MPC_Water" "$$$ Sun Vector" (make `LinearColor` _returnvalue_x_4 _returnvalue_y_4 _returnvalue_z_4 1.0))
            (`KismetMaterialLibrary.SetVectorParameterValue` "/Game/Occam/3_Environment/3_Generic/Water/MPC_Water.MPC_Water" "Sun Vector" (make `LinearColor` _returnvalue_x_2 _returnvalue_y_2 _returnvalue_z_2 1.0))
            (else
              (`KismetMaterialLibrary.SetVectorParameterValue` "/Game/Occam/3_Environment/3_Generic/Water/MPC_Water.MPC_Water" "$$$ Moon Vector" (make `LinearColor` _returnvalue_x _returnvalue_y _returnvalue_z 1.0))
              (`KismetMaterialLibrary.SetVectorParameterValue` "/Game/Occam/3_Environment/3_Generic/Water/MPC_Water.MPC_Water" "Moon Vector" (make `LinearColor` _returnvalue_x_3 _returnvalue_y_3 _returnvalue_z_3 1.0)))))))
    (:`then_1`
      (`KismetMaterialLibrary.SetVectorParameterValue` "/Game/Occam/3_Environment/3_Generic/Water/MPC_Water.MPC_Water" "Sun Reflection Color" (`LightComponentBase.GetLightColor` _light)))))

(fn `UserConstructionScript`)