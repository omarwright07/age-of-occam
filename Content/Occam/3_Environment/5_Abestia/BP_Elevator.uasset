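; Elevator actor that carries a platform between a low position and a configurable ElevatorHeight, with animated wheel parts.
; Overlapping the platform Box or the top and bottom call triggers runs one eased MoveComponentTo, then flips the target height and IsUp flag.
; The construction script raises the top trigger by ElevatorHeight.
; The WaterMovement timeline, played from Tick, counter-rotates the wheel parts independently of platform movement.
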(event `self.ReceiveTick`
  (params (DeltaSeconds :type "Float (single-precision)"))
  (bind (_direction _crotation) (`Timeline|WaterMovement`)
    (:`Update`
      (`SceneComponent.K2_SetRelativeRotation` (`self.WheelPivot`) (`KismetMathLibrary.MakeRotator` 0.0 (- 0.0 _crotation)) false false)
      (`SceneComponent.K2_SetRelativeRotation` (`self.MovePart 7`) (`KismetMathLibrary.MakeRotator` 0.0 (- 0.0 _crotation)) false false)
      (`SceneComponent.K2_SetRelativeRotation` (`self.MovePart 6`) (`KismetMathLibrary.MakeRotator` 0.0 _crotation) false false))))

(event `self.Box.OnComponentBeginOverlap`
  (params (OverlappedComponent :type "PrimitiveComponent Object Reference") (OtherActor :type "Actor Object Reference") (OtherComp :type "PrimitiveComponent Object Reference") (OtherBodyIndex :type Integer) (bFromSweep :type Boolean) (SweepResult :type "HitResult Structure (by ref)"))
  (`KismetSystemLibrary.MoveComponentTo` (`self.Pivot4Platform`) (`KismetMathLibrary.MakeVector` 50.0 50.0 (`KismetMathLibrary.Conv_IntToDouble` (`self.cElevatorTargetZ`))) (struct) true true 5.0 :!label _label)
  (if (== (`self.ElevatorHeight`) (`self.cElevatorTargetZ`))
    (set `self.isUp` false)
    (set `self.cElevatorTargetZ` 50)
    (else
      (set `self.isUp` true)
      (set `self.cElevatorTargetZ` (`self.ElevatorHeight`)))))

(event `self.bottom Trigger.OnComponentBeginOverlap`
  (params (OverlappedComponent :type "PrimitiveComponent Object Reference") (OtherActor :type "Actor Object Reference") (OtherComp :type "PrimitiveComponent Object Reference") (OtherBodyIndex :type Integer) (bFromSweep :type Boolean) (SweepResult :type "HitResult Structure (by ref)"))
  (set `self.cElevatorTargetZ` 50)
  (goto _label))

(event `self.Box.OnComponentEndOverlap`
  (params (OverlappedComponent :type "PrimitiveComponent Object Reference") (OtherActor :type "Actor Object Reference") (OtherComp :type "PrimitiveComponent Object Reference") (OtherBodyIndex :type Integer))
  (if (`self.isUp`)
    (set `self.cElevatorTargetZ` (`self.ElevatorHeight`))
    (else
      (set `self.cElevatorTargetZ` 50))))

(event `self.topTrigger.OnComponentBeginOverlap`
  (params (OverlappedComponent :type "PrimitiveComponent Object Reference") (OtherActor :type "Actor Object Reference") (OtherComp :type "PrimitiveComponent Object Reference") (OtherBodyIndex :type Integer) (bFromSweep :type Boolean) (SweepResult :type "HitResult Structure (by ref)"))
  (set `self.cElevatorTargetZ` (`self.ElevatorHeight`))
  (goto _label))

(fn `UserConstructionScript`
  (bind _elevatorheight (`self.ElevatorHeight`))
  (bind _toptrigger (`self.topTrigger`))
  (bind (_returnvalue_x _returnvalue_y _returnvalue_z) (`KismetMathLibrary.BreakVector` (`SceneComponent.K2_GetComponentLocation` _toptrigger)))
  (set `self.cElevatorTargetZ` _elevatorheight)
  (set `self.isUp` true)
  (`SceneComponent.K2_SetWorldLocation` _toptrigger (`KismetMathLibrary.MakeVector` 0.0 0.0 (+ _returnvalue_z (`KismetMathLibrary.Conv_IntToDouble` _elevatorheight))) false false))