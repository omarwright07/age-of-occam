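; A modular ramp level-building actor that assembles itself from static mesh components in the construction script.
; It loops over the UnitSize array, placing the first piece at the default transform and later pieces along local Y at 100-unit steps tracked by CurrentSize.
; A closing piece follows the last segment, and an empty array yields a single mesh.
; The event graph holds no logic.
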(fn `UserConstructionScript`
  (if (> (`KismetArrayLibrary.Array_Length` (`self.UnitSize`)) 0)
    (for (_ _array_index) (`self.UnitSize`)
      (if (> _array_index 0)
        (`AddComponent|NODE_AddStaticMeshComponent-4` :`RelativeTransform` (`KismetMathLibrary.MakeTransform` (`KismetMathLibrary.MakeVector` 0.0 (`KismetMathLibrary.Conv_IntToDouble` (* (`self.CurrentSize`) 100)))))
        (else
          (`AddComponent|NODE_AddStaticMeshComponent-0`)))
      (`/Engine/EditorBlueprintResources/StandardMacros.IncrementInt` (`self.CurrentSize`)))
    (`AddComponent|NODE_AddStaticMeshComponent-3` :`RelativeTransform` (`KismetMathLibrary.MakeTransform` (`KismetMathLibrary.MakeVector` 0.0 (`KismetMathLibrary.Conv_IntToDouble` (* (`self.CurrentSize`) 100)))))
    (else
      (`AddComponent|NODE_AddStaticMeshComponent-1`))))